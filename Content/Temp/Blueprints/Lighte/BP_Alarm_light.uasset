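; BP_Alarm_light is a rotating alarm beacon light built from a sphere mesh and a spot light.
; Every Tick it yaws both components by a fixed speed scaled by delta seconds, giving a frame-rate-independent spin.
; The construction script and the Radius replication callback are empty.
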(event `self.ReceiveTick`
  (params (DeltaSeconds :type "Float (single-precision)"))
  (bind _output_get (set `self.AlarmRotationSpeed` DeltaSeconds))
  (bind _returnvalue (`KismetMathLibrary.MakeRotator` 0.0 0.0 (* _output_get 220.0)))
  (`SceneComponent.K2_AddRelativeRotation` (`self.Sphere`) _returnvalue false false)
  (`SceneComponent.K2_AddRelativeRotation` (`self.SpotLight`) _returnvalue false false))

(fn `OnRep_Radius`)

(fn `UserConstructionScript`)