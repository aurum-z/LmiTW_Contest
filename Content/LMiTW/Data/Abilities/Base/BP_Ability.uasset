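; BP_Ability is a base ability data asset exposing an ability's info: type, ID, logic, montages and attack parameters.
; Simple getters read from the AbilityInfo struct, while GetAttackInfo returns a separate AttackParams value.
; GetRandomMontage converts the montage collection to an array and returns a random valid entry, printing an error if the pick is invalid.
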(fn `GetAttackInfo`
  (returns (Info :type "/Game/LMiTW/Blueprints/Structures/S_AbilityAttackParams Structure"))
  (return (`self.AttackParams`)))

(fn `GetId`
  (returns (Id :type Integer))
  (return (`.Id_11_07FF995140FB8240BF66389E3970E9E0` (break `/Game/LMiTW/Blueprints/Structures/S_Ability` (`self.GetInfo`)))))

(fn `GetInfo`
  (returns (AbilityInfo :type "/Game/LMiTW/Blueprints/Structures/S_Ability Structure"))
  (return (`self.AbilityInfo`)))

(fn `GetLogic`
  (returns (Logic :type "/Game/LMiTW/Blueprints/AbilityLogic/Base/BP_AbilityBaseLogic Class Reference"))
  (return (`.AbilityLogic_14_CE8A3A9448DBECF019B6D082A082207D` (break `/Game/LMiTW/Blueprints/Structures/S_Ability` (`self.GetInfo`)))))

(fn `GetMontages`
  (returns (Montages :type "Set of AnimMontage Object Reference"))
  (return (`.Montages_7_965B5EEB41C809F675B90D94D4FDA7E8` (break `/Game/LMiTW/Blueprints/Structures/S_Ability` (`self.GetInfo`)))))

(fn `GetRandomMontage`
  (returns (Montage :type "AnimMontage Object Reference"))
  (locals (Local_RandomIndex :type Integer :default 0) (Local_Montages :type "Array of AnimMontage Object Reference"))
  (bind _output (`|GetArrayItem` (`local.Local_Montages`) (`local.Local_RandomIndex`)))
  (bind _result (`BlueprintSetLibrary.Set_ToArray` (`self.GetMontages`)))
  (set `local.Local_Montages` _result)
  (set `local.Local_RandomIndex` (`KismetMathLibrary.RandomIntegerInRange` 0 (- (`KismetArrayLibrary.Array_Length` (`local.Local_Montages`)) 1)))
  (if (`KismetArrayLibrary.Array_IsValidIndex` (`local.Local_Montages`) (`local.Local_RandomIndex`))
    (`/Engine/EditorBlueprintResources/StandardMacros.IsValid` _output
      (:`Is Valid`
        (return _output))
      (:`Is Not Valid`
        _)))
  (`KismetSystemLibrary.PrintString` null "BP_Ability: Montage is not valid!" true true (struct :`R` 1.0 :`G` 0.032086 :`A` 1.0) 1.0)
  (return null))

(fn `GetType`
  (returns (Type :type "/Game/LMiTW/Blueprints/Enums/E_AbilityType Enum"))
  (return (`.Type_2_66056C354E9CA4AD87721899600CF737` (break `/Game/LMiTW/Blueprints/Structures/S_Ability` (`self.GetInfo`)))))