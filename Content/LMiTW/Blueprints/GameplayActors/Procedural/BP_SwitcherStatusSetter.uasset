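; Procedural setup actor that rolls access states for every BP_DoorSlider in the level once BP_Graph finishes its work.
; A looping timer polls the graph, then AllDoorSetState applies the "Easy" DataTable row; other difficulty zones are unwired.
; Each non-button door gets a weighted random state from the row's cumulative thresholds.
; SetState's switch cases are disconnected, so the open, pin-lock and closed writes to doors and control panels never run.
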(event `self.ReceiveBeginPlay`
  (`self.Init`))

(event `E_StatusSet`
  (`|ExecutionSequence`
    (:`then_0`
      ;[1 1 1] Zone 1
      (`self.allDoorSetState` "Easy" "/Game/LMiTW/Blueprints/GameplayActors/Door/BP_DoorSlider.BP_DoorSlider_C"))))

(fn `allDoorSetState`
  (params (DoorStateLevel :type Name) (Door_BP :type "/Game/LMiTW/Blueprints/GameplayActors/Door/BP_DoorSlider Class Reference") (DoorTag :type Name))
  (bind _outactors (`GameplayStatics.GetAllActorsOfClass` "/Game/LMiTW/Blueprints/GameplayActors/Door/BP_DoorSlider.BP_DoorSlider_C"))
  (for (_array_element _array_index) _outactors
    ;[1 1 1] If Door interact with Button
    (bind _doorinteractwithbutton_ (`self.CheckSwitcherSubsidiaryClass` _array_element))
    (if _doorinteractwithbutton_
      (if (`self.drawText?`)
        (`/Game/LMiTW/Blueprints/GameplayActors/Door/BP_MasterDoor.SetAccessStatusToTextRender` _array_element "Button"))
      (else
        ;[1 1 1] If Door interact with Control panel
        (`self.DoorSetState` _array_element _array_index DoorStateLevel Door_BP DoorTag)))))

(fn `CheckDataTablesValues`
  (params (InRow :type "/Game/LMiTW/Blueprints/Structures/S_DoorRangeStatus Structure"))
  (locals (P_1 :type Integer) (P_2 :type Integer) (P_3 :type Integer) (P_4 :type Integer) (P_5 :type Integer) (TAG_1 :type Name) (TAG_2 :type Name) (TAG_3 :type Name) (TAG_4 :type Name) (TAG_5 :type Name) (TAG_6 :type Name) (P_1 :type Integer) (P_2 :type Integer) (P_3 :type Integer) (P_4 :type Integer) (P_5 :type Integer) (TAG_1 :type Name) (TAG_2 :type Name) (TAG_3 :type Name) (TAG_4 :type Name) (TAG_5 :type Name) (TAG_6 :type Name))
  (bind (_p_1 _p_2 _p_3 _p_4 _p_5) (break `/Game/LMiTW/Blueprints/Structures/S_DoorRangeStatus` InRow))
  (bind _p_2_2 (`local.P_2`))
  (bind _p_4_2 (`local.P_4`))
  (bind _p_5_2 (`local.P_5`))
  (bind _p_1_2 (`local.P_1`))
  (bind _p_3_2 (`local.P_3`))
  (bind _p_2_3 (`local.P_2`))
  (bind _p_2_4 (`local.P_2`))
  (set `local.P_1` _p_1)
  (set `local.P_2` _p_2)
  (set `local.P_3` _p_3)
  (set `local.P_4` _p_4)
  (set `local.P_5` _p_5)
  (set `local.TAG_1` "None")
  (set `local.TAG_2` "None")
  (set `local.TAG_3` "None")
  (set `local.TAG_4` "None")
  (set `local.TAG_5` "None")
  (set `local.TAG_6` "None")
  (if (not (and (!= _p_1_2 (`local.P_2`)) (!= _p_1_2 (`local.P_3`)) (!= _p_1_2 (`local.P_4`)) (!= _p_1_2 (`local.P_5`)) (or (!= _p_2_3 _p_3_2) (and (== _p_2_3 0) (== _p_3_2 0))) (or (!= _p_2_4 _p_4_2) (and (== _p_2_4 0) (== _p_4_2 0))) (or (!= _p_2_2 _p_5_2) (and (== _p_2_2 0) (== _p_5_2 0))) false false false))
    (`KismetSystemLibrary.PrintString` (`KismetStringLibrary.Concat_StrStr` (`KismetSystemLibrary.GetObjectName` self) ": CheckDataTable function." "ERR." (`KismetSystemLibrary.GetObjectName` (`self.DT_DoorRangeStatus`)) " have eaqual values") true true (struct :`R` 1.0 :`G` 0.057065 :`A` 1.0) 15.0)
    (return)))

(fn `CheckIsGraphFinishWork`
  (if (`/Game/LMiTW/Blueprints/GameplayActors/Procedural/BP_Graph.FinishWork?` (`self.BP_Graph`))
    (`KismetSystemLibrary.K2_ClearAndInvalidateTimerHandle` (`self.tIsGraphFinishWork`))
    (`self.E_StatusSet`)
    (else
      (`KismetSystemLibrary.PrintString` "BP_DoorStatusSetter wait for graph finish work" false false (struct :`R` 1.0 :`G` 0.215493 :`B` 0.355569 :`A` 1.0) 0.01))))

(fn `CheckSwitcherSubsidiaryClass`
  (params (InBP_Door :type "/Game/LMiTW/Blueprints/GameplayActors/Door/BP_DoorSlider Object Reference"))
  (returns (`DoorInteractWithButton?` :type Boolean))
  ;[1 1 1] Get switcher class
  (if (`KismetSystemLibrary.DoesImplementInterface` InBP_Door "/Game/LMiTW/Blueprints/Interface/BPI_Generator.BPI_Generator_C")
    (bind _subsidiaryclass (message `/Game/LMiTW/Blueprints/Interface/BPI_Generator.WhatSubsidiaryClassOfMasterSwitcher` InBP_Door))
    (if (== _subsidiaryclass "/Game/LMiTW/Blueprints/GameplayActors/Switcher/BP_DoorControlPanel.BP_DoorControlPanel_C")
      (return false)
      (elif (== _subsidiaryclass "/Game/LMiTW/Blueprints/GameplayActors/Switcher/BP_Button.BP_Button_C")
        (return true)))
    (else
      (`KismetSystemLibrary.PrintString` (`KismetStringLibrary.Concat_StrStr` (`KismetSystemLibrary.GetObjectName` self) "CheckSwitcherClass function. ERR.  " (`KismetSystemLibrary.GetObjectName` InBP_Door) "doesn`t implement BPI Generator interface") true true (struct :`R` 1.0 :`B` 0.165275 :`A` 1.0) 20.0))))

(fn `DoorSetState`
  (params (InBP_Door :type "/Game/LMiTW/Blueprints/GameplayActors/Door/BP_DoorSlider Object Reference") (DoorID :type Integer) (DoorStateLevel :type Name) (DoorBP :type "/Game/LMiTW/Blueprints/GameplayActors/Door/BP_DoorSlider Class Reference") (DoorTag :type Name))
  (returns (`Success?` :type Boolean))
  (locals (DoorStateIndex :type Integer) (BP_Door :type "/Game/LMiTW/Blueprints/GameplayActors/Door/BP_DoorSlider Object Reference"))
  (`/Engine/EditorBlueprintResources/StandardMacros.IsValid` InBP_Door
    (:`Is Valid`
      ;[1 1 1] MultiDoor branch
      (set `local.BP_Door` InBP_Door))
    (:`Is Not Valid`
      ;[1 1 1] SoloDoor branch
      (bind (_success_ _bp_door) (`self.findEqualDoorByID` DoorID DoorBP DoorTag))
      (if _success_
        (set `local.BP_Door` _bp_door)
        (else
          (return false)))))
  ;[1 1 1] Get door state from Data table
  (bind _returnvalue (`|GetDataTableRow` (`self.DT_DoorRangeStatus`) DoorStateLevel)
    (:`then`
      (bind (_statetosetout _success__2) (`self.GetStateFromDataTable` _returnvalue))
      (if _success__2
        (`self.setState` (`local.BP_Door`) _statetosetout)
        (return true)))
    (:`RowNotFound`
      (`KismetSystemLibrary.PrintString` "BP_DoorStatusSetter: OneDoorSetState. ERR Row not found" true true (struct :`R` 1.0 :`B` 0.139721 :`A` 1.0) 20.0)
      (return false))))

(fn `findEqualDoorByID`
  (params (DoorID :type Integer) (DoorBP :type "/Game/LMiTW/Blueprints/GameplayActors/Door/BP_DoorSlider Class Reference") (DoorTag :type Name))
  (returns (`Success?` :type Boolean) (BP_Door :type "/Game/LMiTW/Blueprints/GameplayActors/Door/BP_DoorSlider Object Reference"))
  (bind _outactors (`GameplayStatics.GetAllActorsOfClass` DoorBP))
  (for _array_element _outactors
    (bind _asbp_door_slider (cast `/Game/LMiTW/Blueprints/GameplayActors/Door/BP_DoorSlider` _array_element)
      (:`then`
        (if (== (`/Game/LMiTW/Blueprints/GameplayActors/Door/BP_MasterDoor.Id` _asbp_door_slider) DoorID)
          (return true _asbp_door_slider)))
      (:`CastFailed`
        (`KismetSystemLibrary.PrintString` "BP_DoorStatusSetter: findMatchDoorByID function.Cast Fail" true true (struct :`R` 1.0 :`B` 0.217823 :`A` 1.0) 30.0))))
  ;[1 0 0.2203] Comment
  (`KismetSystemLibrary.PrintString` (`KismetStringLibrary.Concat_StrStr` "BP_DoorStatusSetter: findMatchDoorByID function. ERR. Input Door ID out range. Door ID:" (`KismetStringLibrary.Conv_IntToString` DoorID)) true true (struct :`R` 1.0 :`B` 0.217823 :`A` 1.0) 30.0)
  (return false null))

(fn `GetStateFromDataTable`
  (params (DoorRangeStatus :type "/Game/LMiTW/Blueprints/Structures/S_DoorRangeStatus Structure"))
  (returns (StateToSetOut :type "/Game/LMiTW/Blueprints/Enums/E_SwitcherStatusRange Enum") (`Success?` :type Boolean))
  (locals (minRangeOfTable :type Integer :default 1) (maxRangeOfTable :type Integer :default 99) (P_1 :type Integer) (P_2 :type Integer) (P_3 :type Integer) (P_4 :type Integer) (P_5 :type Integer) (SID :type Integer) (TAG_1 :type "/Game/LMiTW/Blueprints/Enums/E_SwitcherStatusRange Enum") (TAG_2 :type "/Game/LMiTW/Blueprints/Enums/E_SwitcherStatusRange Enum") (TAG_3 :type "/Game/LMiTW/Blueprints/Enums/E_SwitcherStatusRange Enum") (TAG_4 :type "/Game/LMiTW/Blueprints/Enums/E_SwitcherStatusRange Enum") (TAG_5 :type "/Game/LMiTW/Blueprints/Enums/E_SwitcherStatusRange Enum") (TAG_6 :type "/Game/LMiTW/Blueprints/Enums/E_SwitcherStatusRange Enum") (bool :type Boolean) (`Debug?` :type Boolean))
  (bind (_p_1 _p_2 _p_3 _p_4 _p_5 _tag_1 _tag_2 _tag_3 _tag_4 _tag_5 _tag_6) (break `/Game/LMiTW/Blueprints/Structures/S_DoorRangeStatus` DoorRangeStatus))
  (bind _tag_1_2 (`local.TAG_1`))
  (bind _tag_2_2 (`local.TAG_2`))
  (bind _tag_3_2 (`local.TAG_3`))
  (bind _tag_4_2 (`local.TAG_4`))
  (bind _debug_ (`local.Debug?`))
  (bind _debug__2 (`local.Debug?`))
  (bind _debug__3 (`local.Debug?`))
  (bind _debug__4 (`local.Debug?`))
  (bind _debug__5 (`local.Debug?`))
  (bind _debug__6 (`local.Debug?`))
  (bind _tag_5_2 (`local.TAG_5`))
  (bind _debug__7 (`local.Debug?`))
  (bind _tag_6_2 (`local.TAG_6`))
  (set `local.P_1` _p_1)
  (set `local.P_2` _p_2)
  (set `local.P_3` _p_3)
  (set `local.P_4` _p_4)
  (set `local.P_5` _p_5)
  (set `local.TAG_1` _tag_1)
  (set `local.TAG_2` _tag_2)
  (set `local.TAG_3` _tag_3)
  (set `local.TAG_4` _tag_4)
  (set `local.TAG_5` _tag_5)
  (set `local.TAG_6` _tag_6)
  (bind _output_get (set `local.SID` (+ (`KismetMathLibrary.RandomInteger` 99) 1)))
  (`KismetSystemLibrary.PrintString` (`KismetStringLibrary.Conv_IntToString` _output_get) _debug__6 _debug__6 (struct :`R` 1.0 :`G` 0.243682 :`A` 1.0) 20.0)
  ;[1 1 1] TAG_1
  (if (`KismetMathLibrary.InRange_IntInt` (`local.SID`) (`local.minRangeOfTable`) (`local.P_1`))
    (`KismetSystemLibrary.PrintString` (`|GetEnumeratorNameAsString` _tag_1_2) _debug__2 _debug__2 (struct :`R` 1.0 :`G` 0.823312 :`A` 1.0))
    (return _tag_1_2 true)
    (else
      ;[1 1 1] TAG_2
      (if (`KismetMathLibrary.InRange_IntInt` (`local.SID`) (`local.P_1`) (`local.P_2`) false)
        (`KismetSystemLibrary.PrintString` (`|GetEnumeratorNameAsString` _tag_2_2) _debug__3 _debug__3 (struct :`R` 1.0 :`G` 0.823312 :`A` 1.0))
        (return _tag_2_2 true)
        (else
          ;[1 1 1] TAG_3
          (if (`KismetMathLibrary.InRange_IntInt` (`local.SID`) (`local.P_2`) (`local.P_3`) false)
            (`KismetSystemLibrary.PrintString` (`|GetEnumeratorNameAsString` _tag_3_2) _debug__4 _debug__4 (struct :`R` 1.0 :`G` 0.823312 :`A` 1.0))
            (return _tag_3_2 true)
            (else
              ;[1 1 1] TAG_4
              (if (`KismetMathLibrary.InRange_IntInt` (`local.SID`) (`local.P_3`) (`local.P_4`) false)
                (`KismetSystemLibrary.PrintString` (`|GetEnumeratorNameAsString` _tag_4_2) _debug__5 _debug__5 (struct :`R` 1.0 :`G` 0.823312 :`A` 1.0))
                (return _tag_4_2 true)
                (else
                  ;[1 1 1] TAG_5
                  (if (`KismetMathLibrary.InRange_IntInt` (`local.SID`) (`local.P_4`) (`local.P_5`) false)
                    (`KismetSystemLibrary.PrintString` (`|GetEnumeratorNameAsString` _tag_5_2) _debug__7 _debug__7 (struct :`R` 1.0 :`G` 0.823312 :`A` 1.0))
                    (return _tag_5_2 true)
                    (else
                      ;[1 1 1] TAG_6
                      (if (`KismetMathLibrary.InRange_IntInt` (`local.SID`) (`local.P_5`) (`local.maxRangeOfTable`) false)
                        (`KismetSystemLibrary.PrintString` (`|GetEnumeratorNameAsString` _tag_6_2) _debug_ _debug_ (struct :`R` 1.0 :`G` 0.823312 :`A` 1.0))
                        (return _tag_6_2 true)
                        (else
                          (`KismetSystemLibrary.PrintString` "BP_DoorStatusSetter: OneDoorSetState function. ERR. SID not in range" true true (struct :`R` 1.0 :`B` 0.217823 :`A` 1.0) 30.0)
                          (return "NewEnumerator0" false))))))))))))))

(fn `Init`
  (if (`self.work?`)
    ;[1 1 1] Check BP_Graph
    (`/Engine/EditorBlueprintResources/StandardMacros.IsValid` (`self.BP_Graph`)
      (:`Is Valid`
        (bind _returnvalue (`KismetSystemLibrary.K2_SetTimer` self "CheckIsGraphFinishWork" 0.01 true))
        (set `self.tIsGraphFinishWork` _returnvalue)
        ;[1 1 1] Comment
        (for _array_element (`self.DoorStateList`)
          (bind _returnvalue_2 (`|GetDataTableRow` (`self.DT_DoorRangeStatus`) _array_element)
            (:`then`
              (`self.CheckDataTablesValues` _returnvalue_2)))))
      (:`Is Not Valid`
        (`KismetSystemLibrary.PrintString` "BP_DoorStatusSetter: ERR. No BP_Graph reference" true true (struct :`R` 1.0 :`G` 0.021536 :`A` 1.0) 20.0)))))

(fn `setState`
  (params (DoorRef :type "/Game/LMiTW/Blueprints/GameplayActors/Door/BP_DoorSlider Object Reference") (StateToSet :type "/Game/LMiTW/Blueprints/Enums/E_SwitcherStatusRange Enum" :default "NewEnumerator0"))
  (returns (`Success?` :type Boolean))
  (locals (BP_Door :type "/Game/LMiTW/Blueprints/GameplayActors/Door/BP_DoorSlider Object Reference"))
  (set `local.BP_Door` DoorRef)
  (switch `/Game/LMiTW/Blueprints/Enums/E_SwitcherStatusRange` StateToSet))

(fn `setStateToDoorControlPanel`
  (params (`isPermanentLocked?` :type Boolean) (accessLevel :type "/Game/LMiTW/Blueprints/Enums/E_AcessLevels Enum" :default "NewEnumerator3") (BP_DoorIn :type "/Game/LMiTW/Blueprints/GameplayActors/Door/BP_DoorSlider Object Reference"))
  (locals (BP_Door :type "/Game/LMiTW/Blueprints/GameplayActors/Door/BP_DoorSlider Object Reference"))
  (bind _bp_door (`local.BP_Door`))
  (bind _bp_door_2 (`local.BP_Door`))
  (set `local.BP_Door` BP_DoorIn)
  (if `isPermanentLocked?`
    ;[1 1 1] Permanent Lock
    (set `/Game/LMiTW/Blueprints/GameplayActors/Door/BP_MasterDoor.IsEnabled` false _bp_door)
    (set `/Game/LMiTW/Blueprints/GameplayActors/Door/BP_MasterDoor.IsAutomaticOpen` true _bp_door)
    (else
      (set `/Game/LMiTW/Blueprints/GameplayActors/Door/BP_MasterDoor.IsEnabled` true _bp_door_2)
      (set `/Game/LMiTW/Blueprints/GameplayActors/Door/BP_MasterDoor.IsAutomaticOpen` true _bp_door_2)
      ;[1 1 1] Set Access Level to switchers
      (for _array_element (`/Game/LMiTW/Blueprints/GameplayActors/Door/BP_MasterDoor.BP_MasterSwitchers` (`local.BP_Door`))
        (set `/Game/LMiTW/Blueprints/GameplayActors/Switcher/BP_MasterSwitcher.AccessLevel` accessLevel _array_element)
        (bind _asbp_door_control_panel (cast `/Game/LMiTW/Blueprints/GameplayActors/Switcher/BP_DoorControlPanel` _array_element))
        (`/Game/LMiTW/Blueprints/GameplayActors/Switcher/BP_DoorControlPanel.UpdateWidgetInfo` _asbp_door_control_panel)))))

(fn `UserConstructionScript`
  (`KismetArrayLibrary.Array_Clear` (`self.DoorStateList`))
  (bind _outrownames (`DataTableFunctionLibrary.GetDataTableRowNames` (`self.DT_DoorRangeStatus`)))
  (for _array_element _outrownames
    (`KismetArrayLibrary.Array_Add` (`self.DoorStateList`) _array_element)))