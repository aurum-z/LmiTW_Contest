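; BP_NoteGenerator fills every BP_Note in the level with text and randomized door pincodes on BeginPlay.
; It looks up each note's title, date, author and body in DTNotes, using the note's text number as row name.
; A bounded search loop replaces each pincode placeholder in the body with a random four-digit code and collects the codes.
; For notes flagged as having a pincode, it passes those codes to the linked door control panel's widget.
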(event `self.ReceiveBeginPlay`
  (bind _outactors (`GameplayStatics.GetAllActorsOfClass` "/Game/LMiTW/Blueprints/GameplayActors/Pickup/BP_Note.BP_Note_C"))
  (for _array_element _outactors
    (bind (_notehavepincode_ _outnote _outcodes) (`self.SetDataToNote` _array_element))
    (`self.TrySetCodeToControlPanel` _notehavepincode_ _outnote _outcodes)))

(fn `ConvertingPinCodeToNumber`
  (params (mainText :type String))
  (returns (finishedText :type String) (OutCodes :type "Array of Text"))
  (locals (startIndex :type Integer) (findedIndex :type Integer) (numberString :type String) (localString :type String) (localCodes :type "Array of Text"))
  (bind _returnvalue (`KismetStringLibrary.FindSubstring` (`local.localString`) "<pincode>" false false (`local.startIndex`)))
  (set `local.startIndex` 0)
  (set `local.localString` mainText)
  (for _ (range 21)
    ;[1 1 1] if don`t find string "<pincode>"
    (if (== _returnvalue -1)
      (return (`local.localString`) (`local.localCodes`))
      (else
        (set `local.findedIndex` _returnvalue)
        (set `local.numberString` (`KismetStringLibrary.Concat_StrStr` (`KismetStringLibrary.Conv_IntToString` (`KismetMathLibrary.RandomIntegerInRange` 0 9)) (`KismetStringLibrary.Conv_IntToString` (`KismetMathLibrary.RandomIntegerInRange` 0 9)) (`KismetStringLibrary.Conv_IntToString` (`KismetMathLibrary.RandomIntegerInRange` 0 9)) (`KismetStringLibrary.Conv_IntToString` (`KismetMathLibrary.RandomIntegerInRange` 0 9))))
        (set `local.localString` (`KismetStringLibrary.Concat_StrStr` (`KismetStringLibrary.GetSubstring` (`local.localString`) 0 (`local.findedIndex`)) (`local.numberString`) (`KismetStringLibrary.GetSubstring` (`local.localString`) (+ (`local.findedIndex`) 9) (`KismetStringLibrary.Len` (`local.localString`)))))
        (`KismetArrayLibrary.Array_Add` (`local.localCodes`) (`KismetTextLibrary.Conv_StringToText` (`local.numberString`)))
        (set `local.startIndex` (+ (`local.findedIndex`) 4))))))

(fn `SetDataToNote`
  (params (InNote :type "/Game/LMiTW/Blueprints/GameplayActors/Pickup/BP_Note Object Reference"))
  (returns (`NoteHavePincode?` :type Boolean) (OutNote :type "/Game/LMiTW/Blueprints/GameplayActors/Pickup/BP_Note Object Reference") (OutCodes :type "Array of Text"))
  (bind _returnvalue (`|GetDataTableRow` (`self.DT_Notes`) (`KismetStringLibrary.Conv_StringToName` (`KismetStringLibrary.Conv_IntToString` (`/Game/LMiTW/Blueprints/GameplayActors/Pickup/BP_Note.NumberOfText` InNote))))
    (:`then`
      (bind (_titleofnode _date _author _maintext) (break `/Game/LMiTW/Blueprints/Structures/S_NoteData` _returnvalue))
      (bind (_finishedtext _outcodes) (`self.ConvertingPinCodeToNumber` _maintext))
      (`/Game/LMiTW/Blueprints/GameplayActors/Pickup/BP_Note.SetNoteData` InNote (make `/Game/LMiTW/Blueprints/Structures/S_NoteData` _titleofnode _date _author _finishedtext))
      (bind _havepincode_ (`/Game/LMiTW/Blueprints/GameplayActors/Pickup/BP_Note.GetHavePinCode` InNote))
      (return _havepincode_ InNote _outcodes))
    (:`RowNotFound`
      (`KismetSystemLibrary.PrintString` (`KismetStringLibrary.Concat_StrStr` "ERR." (`KismetSystemLibrary.GetObjectName` self) " Not found Row") true true (struct :`R` 1.0 :`G` 0.039115 :`A` 1.0)))))

(fn `TrySetCodeToControlPanel`
  (params (`NoteHavePincode?` :type Boolean) (InNote :type "/Game/LMiTW/Blueprints/GameplayActors/Pickup/BP_Note Object Reference") (TrueCodes :type "Array of Text"))
  (if `NoteHavePincode?`
    (bind _doorcontrolpanel (`/Game/LMiTW/Blueprints/GameplayActors/Pickup/BP_Note.GetDoorControlPanel` InNote))
    (`/Game/LMiTW/HUD/GameplayActors/Interactable/WBP_DoorControlPanel.SetTrueCode` (`/Game/LMiTW/Blueprints/GameplayActors/Switcher/BP_DoorControlPanel.Widget` _doorcontrolpanel) TrueCodes)))

(fn `UserConstructionScript`)