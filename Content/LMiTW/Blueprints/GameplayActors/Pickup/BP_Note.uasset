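; BP_Note is an interactable readable note that opens on the interacting actor and closes on the next interaction.
; Interact passes the note data and itself to ENoteOpen, tracks taken and read state, and calls ENoteClose when already open.
; Focus toggles custom depth on the pickup mesh.
; Construction checks the door control panel reference to flag a PIN code, with getters exposing note, panel and interaction info.
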(event `self.ReceiveBeginPlay`
  (`self.Init`))

(event `/Game/LMiTW/Blueprints/Interface/BPI_Interactable.Interact`
  (params (Interactor :type "/Game/LMiTW/Blueprints/Character/BP_LMPlayerCharacter Object Reference") (InputKey :type "Key Structure"))
  ;[1 1 1] Pick up
  (if (`self.PlayerRead?`)
    (`/Game/LMiTW/Blueprints/Character/BP_LMPlayerCharacter.E_NoteClose` Interactor)
    (set `self.PlayerRead?` false)
    (else
      (`self.PickUp` Interactor))))

(event `/Game/LMiTW/Blueprints/Interface/BPI_Interactable.StartFocus`
  ;[1 1 1] Focusing
  (`self.SetRenderCustomDepth` true))

(event `/Game/LMiTW/Blueprints/Interface/BPI_Interactable.StopFocus`
  ;[1 1 1] Focusing
  (`self.SetRenderCustomDepth` false))

(fn `GetDoorControlPanel`
  (returns (DoorControlPanel :type "/Game/LMiTW/Blueprints/GameplayActors/Switcher/BP_DoorControlPanel Object Reference"))
  (return (`self.BP_DoorControlPanel`)))

(fn `GetHavePinCode`
  (returns (`HavePinCode?` :type Boolean))
  (return (`self.HavePinCode?`)))

(fn `GetInteractInfo`
  (returns (Info :type "/Game/LMiTW/Blueprints/Structures/S_InteractionInfo Structure"))
  (return (`self.InteractInfo`)))

(fn `GetNoteData`
  (returns (NoteData :type "/Game/LMiTW/Blueprints/Structures/S_NoteData Structure"))
  (return (`self.NoteData`)))

(fn `GetOrigin`
  (returns (OriginLocation :type "Vector Structure"))
  (return (`KismetSystemLibrary.GetComponentBounds` (`self.PickupMesh`))))

(fn `GetSwitcherInfo`
  (returns (TypeOfSwitcher :type "/Game/LMiTW/Blueprints/Enums/E_SwitcherTYpe Enum") (`Online?` :type Boolean) (`DoorOpen?` :type Boolean) (SwitcherActor :type "/Game/LMiTW/Blueprints/GameplayActors/Switcher/BP_MasterSwitcher Object Reference") (ControlPanelStatus :type "/Game/LMiTW/Blueprints/Enums/E_SwitcherStatusRange Enum"))
  (return "NewEnumerator2" false false null "NewEnumerator0"))

(fn `Init`)

(fn `PickUp`
  (params (Interactor :type "/Game/LMiTW/Blueprints/Character/BP_LMPlayerCharacter Object Reference"))
  (`/Game/LMiTW/Blueprints/Character/BP_LMPlayerCharacter.E_NoteOpen` Interactor (`self.NoteData`) self)
  (set `self.PlayerTookTheNote?` true)
  (set `self.PlayerRead?` true))

(fn `PinCodeCheck`
  (if (not (== (`self.BP_DoorControlPanel`) null))
    (set `self.HavePinCode?` true)))

(fn `PreInit`
  (`self.PinCodeCheck`))

(fn `SetNoteData`
  (params (NoteData :type "/Game/LMiTW/Blueprints/Structures/S_NoteData Structure"))
  (set `self.NoteData` NoteData))

(fn `SetRenderCustomDepth`
  (params (Render :type Boolean))
  (`PrimitiveComponent.SetRenderCustomDepth` (`self.PickupMesh`) Render))

(fn `UserConstructionScript`
  (`self.PreInit`))