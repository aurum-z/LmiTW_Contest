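; Master pickup Blueprint that serves as a base for interactable objects that can be picked up and dropped.
; Pressing F on interact alternates between PickUp and Drop through a FlipFlop; both currently only print debug text.
; Focus events toggle custom depth rendering on the pickup mesh.
; Empty PreInit and Init hooks run at construction and BeginPlay, while getters expose interaction info, mesh origin and fixed switcher info.
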(event `self.ReceiveBeginPlay`
  (`self.Init`))

(event `/Game/LMiTW/Blueprints/Interface/BPI_Interactable.Interact`
  (params (Interactor :type "/Game/LMiTW/Blueprints/Character/BP_LMPlayerCharacter Object Reference") (InputKey :type "Key Structure"))
  ;[1 1 1] Pick up
  (if (== InputKey "F")
    (`/Engine/EditorBlueprintResources/StandardMacros.FlipFlop`
      (:`A`
        (`self.PickUp` Interactor))
      (:`B`
        (`self.Drop` Interactor true)))))

(event `/Game/LMiTW/Blueprints/Interface/BPI_Interactable.StartFocus`
  ;[1 1 1] Focusing
  (`self.SetRenderCustomDepth` true))

(event `/Game/LMiTW/Blueprints/Interface/BPI_Interactable.StopFocus`
  ;[1 1 1] Focusing
  (`self.SetRenderCustomDepth` false))

(fn `Drop`
  (params (Interactor :type "/Game/LMiTW/Blueprints/Character/BP_LMPlayerCharacter Object Reference") (`SetSimulatePhysics?` :type Boolean))
  (`KismetSystemLibrary.PrintString` "drop" true true (struct :`R` 1.0 :`G` 0.116388 :`B` 0.026724 :`A` 1.0)))

(fn `GetInteractInfo`
  (returns (Info :type "/Game/LMiTW/Blueprints/Structures/S_InteractionInfo Structure"))
  (return (`self.InteractInfo`)))

(fn `GetOrigin`
  (returns (OriginLocation :type "Vector Structure"))
  (return (`KismetSystemLibrary.GetComponentBounds` (`self.PickupMesh`))))

(fn `GetSwitcherInfo`
  (returns (TypeOfSwitcher :type "/Game/LMiTW/Blueprints/Enums/E_SwitcherTYpe Enum") (`Online?` :type Boolean) (`DoorOpen?` :type Boolean) (SwitcherActor :type "/Game/LMiTW/Blueprints/GameplayActors/Switcher/BP_MasterSwitcher Object Reference") (ControlPanelStatus :type "/Game/LMiTW/Blueprints/Enums/E_SwitcherStatusRange Enum"))
  (return "NewEnumerator2" false false null "NewEnumerator0"))

(fn `Init`)

(fn `PickUp`
  (params (Interactor :type "/Game/LMiTW/Blueprints/Character/BP_LMPlayerCharacter Object Reference"))
  (`KismetSystemLibrary.PrintString` "pickup" true true (struct :`R` 1.0 :`G` 0.066005 :`A` 1.0)))

(fn `PreInit`)

(fn `SetRenderCustomDepth`
  (params (Render :type Boolean))
  (`PrimitiveComponent.SetRenderCustomDepth` (`self.PickupMesh`) Render))

(fn `UserConstructionScript`
  (`self.PreInit`))