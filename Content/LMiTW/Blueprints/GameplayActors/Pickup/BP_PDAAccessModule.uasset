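; BP_PDAAccessModule is a key card pickup that grants a PDA access level to whoever picks it up.
; The construction script assigns the pickup mesh and sets the interaction prompt info for pressing the interact key.
; Its PickUp override runs the parent logic, passes AccessLevelGranted to the interactor's SetPdaAccessLevel, then removes the actor through a short life span.
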(fn `PickUp`
  (params (Interactor :type "/Game/LMiTW/Blueprints/Character/BP_LMPlayerCharacter Object Reference"))
  (`parent.PickUp` Interactor)
  (`/Game/LMiTW/Blueprints/Character/BP_LMPlayerCharacter.SetPdaAccessLevel` Interactor (`self.AccessLevelGranted`))
  (`self.SetLifeSpan` 0.1))

(fn `UserConstructionScript`
  (`StaticMeshComponent.SetStaticMesh` (`self.PickupMesh`) (`self.Mesh`))
  (set `self.InteractInfo` (make `/Game/LMiTW/Blueprints/Structures/S_InteractionInfo` "Key card" "Press" "F")))