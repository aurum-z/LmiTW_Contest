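; BP_TwoHandedItem is a pickup actor for items carried two-handed, such as doors and batteries.
; Construction sets the mesh from ItemInfo; BeginPlay applies the configured physics state and loads type-specific offset data from a DataTable.
; PickUp asks the interactor through BPI_PlayerInteraction to attach it, recording that interactor as Master on success.
; Dropping clears the in-use state and Master, then sets physics simulation as requested.
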(event `self.ReceiveBeginPlay`
  ;[1 1 1] BeginPlay
  (`parent.ReceiveBeginPlay`)
  (`PrimitiveComponent.SetSimulatePhysics` (`self.PickupMesh`) (`self.simulatePhysicAtBeginPlay`))
  (`ActorComponent.K2_DestroyComponent` (`self.DefaultSceneRoot`))
  (`self.InitTwoHanded`))

(event `self.PickUp`
  (params (Interactor :type "/Game/LMiTW/Blueprints/Character/BP_LMPlayerCharacter Object Reference"))
  (if (and (not (`self.InUse?`)) (`KismetSystemLibrary.DoesImplementInterface` Interactor "/Game/LMiTW/Blueprints/Interface/BPI_PlayerInteraction.BPI_PlayerInteraction_C"))
    (bind _success_ (message `/Game/LMiTW/Blueprints/Interface/BPI_PlayerInteraction.AddTwoHandedItem` Interactor self "None"))
    (if _success_
      (set `self.InUse?` true)
      (set `self.master` Interactor)
      (`/Engine/EditorBlueprintResources/StandardMacros.DoOnce` false))))

(event `E_DropTwoHandedItem`
  (params (`SumulatePhysics?` :type Boolean))
  (set `self.InUse?` false)
  (set `self.master` null)
  (`PrimitiveComponent.SetSimulatePhysics` (`self.PickupMesh`) `SumulatePhysics?`))

(fn `GetItemInfo`
  (returns (ItemInfo :type "/Game/LMiTW/Blueprints/Structures/S_ItemInfo Structure"))
  (return (`self.ItemInfo`)))

(fn `GetTwoHandedItemOffset`
  (returns (TwoHandedItemOffset :type "/Game/LMiTW/Blueprints/Structures/S_TwoHandedItem Structure"))
  (return (`self.S_TwoHandedItemOffset`)))

(fn `InitTwoHanded`
  (switch `/Game/LMiTW/Blueprints/Enums/E_TwoHandedItems` (`.TwoHandedItemType_8_DB7A70274E1565B6104F538F4E4BFD75` (break `/Game/LMiTW/Blueprints/Structures/S_TwoHandedItem` (`self.S_TwoHandedItemOffset`)))
    (:`NewEnumerator0`
      (bind _returnvalue (`|GetDataTableRow` (`self.DT_TypesOfTwoHandedItems`) "Door")
        (:`then`
          (set `self.S_TwoHandedItemOffset` _returnvalue))))
    (:`NewEnumerator1`
      (bind _returnvalue_2 (`|GetDataTableRow` (`self.DT_TypesOfTwoHandedItems`) "Battery")
        (:`then`
          (set `self.S_TwoHandedItemOffset` _returnvalue_2))))))

(fn `PreInitTwoHanded`
  (`StaticMeshComponent.SetStaticMesh` (`self.PickupMesh`) (`.StaticMesh_23_9F5223F84DD7D2895F9C5585A125810E` (break `/Game/LMiTW/Blueprints/Structures/S_ItemInfo` (`self.ItemInfo`)))))

(fn `SetSimulatePhysicAtBeginPlay`
  (params (`Simulate?` :type Boolean))
  (set `self.simulatePhysicAtBeginPlay` `Simulate?`))

(fn `UserConstructionScript`
  (`self.PreInit`)
  (`self.PreInitTwoHanded`))