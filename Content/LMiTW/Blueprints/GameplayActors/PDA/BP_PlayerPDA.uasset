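; BP_PlayerPDA is the player's PDA actor, which stores the access level the PDA currently grants.
; SetAccessLevel only raises the level unless its force flag is set, in which case it overwrites it, and GetAccessLevel returns the stored value.
; On BeginPlay, Init uses the forced path to set a fixed starting enum level.
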(event `self.ReceiveBeginPlay`
  (`self.Init`))

(fn `GetAccessLevel`
  (returns (OutPDA_AccessLevel :type "/Game/LMiTW/Blueprints/Enums/E_AcessLevels Enum"))
  (return (`self.PDA_AccessLevel`)))

(fn `Init`
  (`self.SetAccessLevel` "NewEnumerator3" true))

(fn `SetAccessLevel`
  (params (NewAccessLevel :type "/Game/LMiTW/Blueprints/Enums/E_AcessLevels Enum" :default "NewEnumerator3") (`ForceOverried?` :type Boolean))
  (if `ForceOverried?`
    ;[1 1 1] Use when init
    (set `self.PDA_AccessLevel` NewAccessLevel)
    (else
      ;[1 1 1] If new PDA level more then current PDA level
      (if (> NewAccessLevel (`self.PDA_AccessLevel`))
        (set `self.PDA_AccessLevel` NewAccessLevel)))))

(fn `UserConstructionScript`)