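; Base door Blueprint with configurable meshes and trigger size, leaving animation, interaction and init hooks empty.
; An overlap counter opens it for any actor in None mode, otherwise only AI characters, and optionally closes it when empty.
; Linked switchers or consoles can open and close it in Button mode; Control Panel mode only toggles an auto-open flag.
; Opening and closing notify RemoteControlComponent; access checks and delayed closing are unfinished.
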(event `E_Close_Door`
  ;[1 0 0] Delete this when we have procedural generator
  (`self.CloseDoor` null))

(event `self.ReceiveBeginPlay`
  ;[1 1 1] Init
  (`self.Init`))

(event `/Game/LMiTW/Blueprints/Interface/BPI_Generator.SetSwitcherReferencesToDoor`
  (params (SelfActor :type "Actor Object Reference"))
  ;[1 1 1] Create switcher references in BP_Door
  (`self.AddSwitcherReference` SelfActor))

(event `self.ActivationVolumeBox.OnComponentBeginOverlap`
  (params (OverlappedComponent :type "PrimitiveComponent Object Reference") (OtherActor :type "Actor Object Reference") (OtherComp :type "PrimitiveComponent Object Reference") (OtherBodyIndex :type Integer) (bFromSweep :type Boolean) (SweepResult :type "HitResult Structure (by ref)"))
  ;[1 1 1] Open / close
  (`/Engine/EditorBlueprintResources/StandardMacros.IncrementInt` (`self.AmountOfHumansInTriggerBox`)
    (:`  `
      (if (`|EnumEquality` (`self.DoorMode`) "NewEnumerator0")
        (`self.OpenDoor` null :!label _label)
        (elif (`KismetSystemLibrary.DoesImplementInterface` OtherActor "/Game/LMiTW/Blueprints/Interface/BPI_AICharacter.BPI_AICharacter_C")
          (goto _label))))))

(event `self.ActivationVolumeBox.OnComponentEndOverlap`
  (params (OverlappedComponent :type "PrimitiveComponent Object Reference") (OtherActor :type "Actor Object Reference") (OtherComp :type "PrimitiveComponent Object Reference") (OtherBodyIndex :type Integer))
  ;[1 1 1] Open / close
  (bind _result (`/Engine/EditorBlueprintResources/StandardMacros.DecrementInt` (`self.AmountOfHumansInTriggerBox`))
    (:`  `
      (if (and (== _result 0) (`self.IsAutomaticClose`))
        (`self.CloseDoor` null)))))

(event `PlayOpeningAnimation`
  ;[1 1 1] Open / close
  ;;[0.6146 1 0.6667] Animation
)

(event `PlayClosingAnimation`
  ;[1 1 1] Open / close
  ;;[0.6146 1 0.6667] Animation
)

(event `/Game/LMiTW/Blueprints/Interface/BPI_RemoteControl.ActivateControlledActor`
  ;[1 1 1] Open / close
  ;;[0.5395 1 0.5982] Indirect access (via console or switcher) - if connected
  (`self.IndirectAccessActivate`))

(event `/Game/LMiTW/Blueprints/Interface/BPI_RemoteControl.DeactivateControlledActor`
  ;[1 1 1] Open / close
  ;;[0.5395 1 0.5982] Indirect access (via console or switcher) - if connected
  (`self.IndirectAccessDeactivate`))

(event `/Game/LMiTW/Blueprints/Interface/BPI_Interactable.Interact`
  (params (Interactor :type "/Game/LMiTW/Blueprints/Character/BP_LMPlayerCharacter Object Reference") (InputKey :type "Key Structure"))
  ;[0.5833 1 0.6396] Interact
)

(fn `AddSwitcherReference`
  (params (Actor :type "Actor Object Reference"))
  (bind _asbp_master_switcher (cast `/Game/LMiTW/Blueprints/GameplayActors/Switcher/BP_MasterSwitcher` Actor))
  (`KismetArrayLibrary.Array_Add` (`self.BP_MasterSwitchers`) _asbp_master_switcher))

(fn `CheckPlayerAccessLevel`
  (returns (`Access Granted` :type Boolean))
  ;[1 1 1] TODO
  (message `/Game/LMiTW/Blueprints/Interface/BPI_PlayerInteraction.GetAccessLevel` self)
  (return true))

(fn `CloseDoor`
  (params (Instigator :type "Actor Object Reference"))
  (`self.OnDoorClosed` Instigator)
  (`/Game/LMiTW/Blueprints/Components/BP_RemoteControlComponent.OnControlledActorDeactivated` (`self.RemoteControlComponent`))
  (`self.PlayClosingAnimation`)
  (`self.TryDeactivateTimerToCloseDoor`))

(fn `GetAutomaticClose`
  (returns (`CanClose?` :type Boolean))
  (return (`self.IsAutomaticClose`)))

(fn `GetInteractInfo`
  (returns (Info :type "/Game/LMiTW/Blueprints/Structures/S_InteractionInfo Structure"))
  (return))

(fn `GetIsEnable`
  (returns (`IsEnable?` :type Boolean))
  (return (`self.IsEnabled`)))

(fn `GetRemoteControlComponent`
  (returns (Component :type "/Game/LMiTW/Blueprints/Components/BP_RemoteControlComponent Object Reference"))
  (return (`self.RemoteControlComponent`)))

(fn `IndirectAccessActivate`
  (switch `/Game/LMiTW/Blueprints/Enums/E_DoorIndirectControlMode` (`self.DoorMode`)
    (:`NewEnumerator1`
      ;[1 1 1] Delete this?
      (`self.SetDisableAutomaticOpen`)
      (`self.OpenDoor` null))
    (:`NewEnumerator2`
      (`self.SetDisableAutomaticOpen`))))

(fn `IndirectAccessDeactivate`
  (`self.SetEnableAutomaticOpen`)
  (switch `/Game/LMiTW/Blueprints/Enums/E_DoorIndirectControlMode` (`self.DoorMode`)
    (:`NewEnumerator1`
      (`self.CloseDoor` null))))

(fn `Init`)

(fn `OpenDoor`
  (params (Instigator :type "Actor Object Reference"))
  (`self.OnDoorOpened` Instigator)
  (`/Game/LMiTW/Blueprints/Components/BP_RemoteControlComponent.OnControlledActorActivated` (`self.RemoteControlComponent`))
  (`self.PlayOpeningAnimation`))

(fn `PreInit`
  (`self.SetActivationBoxExtents`)
  (`self.SetDoorMesh`))

(fn `SetAccessStatusToTextRender`
  (params (InText :type Text))
  (`TextRenderComponent.K2_SetText` (`self.TextRender`) InText))

(fn `SetActivationBoxExtents`
  (`BoxComponent.SetBoxExtent` (`self.ActivationVolumeBox`) (`self.ActivationBoxExtent`) true))

(fn `SetAutomaticClose`
  (params (`CanClose?` :type Boolean))
  (set `self.IsAutomaticClose` `CanClose?`))

(fn `SetDisableAutomaticOpen`
  (set `self.IsAutomaticOpen` false))

(fn `SetDoorMesh`
  (`StaticMeshComponent.SetStaticMesh` (`self.Door`) (`self.DoorMesh`))
  (`StaticMeshComponent.SetStaticMesh` (`self.DoorFrame`) (`self.DoorFrameMesh`)))

(fn `setDoorMode`
  (params (InDoorMode :type "/Game/LMiTW/Blueprints/Enums/E_DoorIndirectControlMode Enum" :default "NewEnumerator0"))
  (set `self.DoorMode` InDoorMode))

(fn `SetEnableAutomaticOpen`
  (set `self.IsAutomaticOpen` true))

(fn `SetIsEnable`
  (params (`IsEnable?` :type Boolean))
  (set `self.IsEnabled` `IsEnable?`))

(fn `SetRenderCustomDepth`
  (params (Render :type Boolean))
  (`PrimitiveComponent.SetRenderCustomDepth` (`self.Door`) Render))

(fn `TryActivateTimerToCloseDoor`
  (if (<= (`self.AmountOfHumansInTriggerBox`) 0)
    (bind _returnvalue (`KismetSystemLibrary.K2_SetTimer` self "CloseDoor" (`self.TimeForCloseIfNobodyInTrigger`)))
    (set `self.DoorCloseForNobodyTimer` _returnvalue)))

(fn `TryDeactivateTimerToCloseDoor`
  (bind _doorclosefornobodytimer (`self.DoorCloseForNobodyTimer`))
  (if (`KismetSystemLibrary.K2_IsValidTimerHandle` _doorclosefornobodytimer)
    (`KismetSystemLibrary.K2_ClearAndInvalidateTimerHandle` _doorclosefornobodytimer)))

(fn `UserConstructionScript`
  (`self.PreInit`))

(fn `WhatSubsidiaryClassOfMasterSwitcher`
  (returns (SubsidiaryClass :type "/Game/LMiTW/Blueprints/GameplayActors/Switcher/BP_MasterSwitcher Class Reference"))
  (return null))