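; Interactable welding tool item that a character picks up with the F key.
; Pickup registers the tool on the interactor through SetWelding, then hides the welder meshes and disables the Box collision.
; The invisible actor snaps to the interactor's spine_02 socket with a fixed local offset and rotation, then flags itself as owned.
; Focus events and Init are empty.
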(event `/Game/LMiTW/Blueprints/Interface/BPI_Interactable.Interact`
  (params (Interactor :type "/Game/LMiTW/Blueprints/Character/BP_LMPlayerCharacter Object Reference") (InputKey :type "Key Structure"))
  (if (== InputKey "F")
    (`self.Pick Up` Interactor)))

(event `/Game/LMiTW/Blueprints/Interface/BPI_Interactable.StopFocus`)

(event `/Game/LMiTW/Blueprints/Interface/BPI_Interactable.StartFocus`)

(fn `ChangeMeshVisibility`
  (params (`Visible?` :type Boolean))
  (`SceneComponent.SetVisibility` (`self.Space_welder_Bottle_001`) `Visible?` false)
  (`SceneComponent.SetVisibility` (`self.Space_welder_Corps`) `Visible?` false)
  (`SceneComponent.SetVisibility` (`self.Space_welder_Nose`) `Visible?` false)
  (`SceneComponent.SetVisibility` (`self.Space_welder_Protection`) `Visible?` false)
  (`SceneComponent.SetVisibility` (`self.Space_welder_Protection_bar`) `Visible?` false)
  (`SceneComponent.SetVisibility` (`self.Space_welder_Bottle_002`) `Visible?` false))

(fn `DisableMeshCollision`
  (`PrimitiveComponent.SetCollisionEnabled` (`self.Box`) "NoCollision"))

(fn `Init`)

(fn `Pick Up`
  (params (Interactor :type "/Game/LMiTW/Blueprints/Character/BP_LMPlayerCharacter Object Reference"))
  (`/Game/LMiTW/Blueprints/Character/BP_LMPlayerCharacter.SetWelding` Interactor self)
  (`self.ChangeMeshVisibility` false)
  (`self.K2_AttachToActor` self Interactor "spine_02" "SnapToTarget" "SnapToTarget" "KeepWorld" true)
  ;[1 1 1] Add transform to Character Vector
  (`self.K2_AddActorLocalOffset` self (60.0 30.0 20.0) false false)
  (`self.K2_AddActorLocalRotation` self (struct :`Yaw` -90.0) false false)
  (`self.DisableMeshCollision`)
  (set `self.HaveOwner?` true))

(fn `UserConstructionScript`
  (`parent.UserConstructionScript`))