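; Wild instrument item actor that a character picks up by interacting with the F key.
; Pickup registers it with the interactor through SetWelding, hides its static mesh, snaps it onto that actor at world scale and disables the mesh's collision.
; The focus events and Init are empty, and construction only calls the parent.
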(event `/Game/LMiTW/Blueprints/Interface/BPI_Interactable.Interact`
  (params (Interactor :type "/Game/LMiTW/Blueprints/Character/BP_LMPlayerCharacter Object Reference") (InputKey :type "Key Structure"))
  (if (== InputKey "F")
    (`self.Pick Up` Interactor)))

(event `/Game/LMiTW/Blueprints/Interface/BPI_Interactable.StopFocus`)

(event `/Game/LMiTW/Blueprints/Interface/BPI_Interactable.StartFocus`)

(fn `Init`)

(fn `Pick Up`
  (params (Interactor :type "/Game/LMiTW/Blueprints/Character/BP_LMPlayerCharacter Object Reference"))
  (`/Game/LMiTW/Blueprints/Character/BP_LMPlayerCharacter.SetWelding` Interactor self)
  (`SceneComponent.SetVisibility` (`self.StaticMesh`) false false)
  (`self.K2_AttachToActor` self Interactor "None" "SnapToTarget" "SnapToTarget" "KeepWorld" true)
  (`PrimitiveComponent.SetCollisionEnabled` (`self.StaticMesh`) "NoCollision"))

(fn `UserConstructionScript`
  (`parent.UserConstructionScript`))