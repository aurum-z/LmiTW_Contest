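; Interactable generator that accepts a carried two-handed Battery and powers linked actors.
; Interacting drops the battery into the socket, marks it in use and slides it in by timeline; completion powers actors, updates the capsule widget and moves a pointer platform.
; Power is sent through BPI_PowerSupply, with extra refresh for door control panels, and is also set at BeginPlay from the installed flag.
; Focus toggles custom-depth rendering on the mesh.
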(event `self.ReceiveBeginPlay`
  (`self.SetPowerStatusForSlaveActors` (`self.HaveItemInstalled?`))
  ;[1 1 1] Animations play rate
  (`TimelineComponent.SetPlayRate` (`self.PointerPlatformOffsetTimeline`) (/ 1.0 (`self.PointerAnimationTime`)))
  (`TimelineComponent.SetPlayRate` (`self.ItemMoveInSocketTimeline`) (/ 1.0 (`self.ItemAnimationTime`)))
  (bind _aswbp_capsule (cast `/Game/LMiTW/HUD/GameplayActors/Interactable/WBP_Capsule` (`WidgetComponent.GetWidget` (`self.Widget`)))
    (:`then`
      (set `self.WBP_Capsule` _aswbp_capsule)
      (set `self.SuccessInit` true))
    (:`CastFailed`
      (set `self.SuccessInit` false))))

(event `/Game/LMiTW/Blueprints/Interface/BPI_Interactable.Interact`
  (params (Interactor :type "/Game/LMiTW/Blueprints/Character/BP_LMPlayerCharacter Object Reference") (InputKey :type "Key Structure"))
  (bind (_haveitem_ _iteminfo _actor) (`/Game/LMiTW/Blueprints/Character/BP_LMPlayerCharacter.GetTwoHandedItem` Interactor))
  (if _haveitem_
    (if (`KismetTextLibrary.EqualEqual_TextText` "Battery" (`.Name_2_C87A6EC948CB0F82780F01BD265E0887` (break `/Game/LMiTW/Blueprints/Structures/S_ItemInfo` _iteminfo)))
      (`/Game/LMiTW/Blueprints/Character/BP_LMPlayerCharacter.TryDropTwoHandedItem` Interactor)
      (set `self.HaveItemInstalled?` true)
      (bind _output_get (set `self.Item` _actor))
      ;[1 0.06105 0.3653] resolve what to use - bottom or top?
      (`SceneComponent.K2_SetWorldLocation` (`/Game/LMiTW/Blueprints/GameplayActors/Pickup/BP_MasterPickup.PickupMesh` _output_get) (`SceneComponent.K2_GetComponentLocation` (`self.SocketPlace`)) false false)
      (`SceneComponent.K2_SetWorldRotation` (`/Game/LMiTW/Blueprints/GameplayActors/Pickup/BP_MasterPickup.PickupMesh` _output_get) (`SceneComponent.K2_GetComponentRotation` (`self.SocketPlace`)) false false)
      (set `/Game/LMiTW/Blueprints/GameplayActors/Pickup/BP_TwoHandedItem.master` self _actor)
      (set `/Game/LMiTW/Blueprints/GameplayActors/Pickup/BP_TwoHandedItem.InUse?` true _actor)
      (`self.Event Move Meshes`)
      (bind _interactcomponent (message `/Game/LMiTW/Blueprints/Interface/BPI_PlayerController.GetPlayerInteractComponent` (`GameplayStatics.GetPlayerController` 0)))
      ;[1 1 1] Fake drop for UI character in interaction component
      (`/Game/LMiTW/Blueprints/Components/BP_PlayerInteractionComponent.StartProcessOfDroppingTwoHandedItem` _interactcomponent)
      (`/Game/LMiTW/Blueprints/Components/BP_PlayerInteractionComponent.EndProcessWithTwoHandedItem` _interactcomponent false))))

(event `/Game/LMiTW/Blueprints/Interface/BPI_Interactable.StartFocus`
  (`self.SetRenderCustomDepth` true))

(event `/Game/LMiTW/Blueprints/Interface/BPI_Interactable.StopFocus`
  (`self.SetRenderCustomDepth` false))

(event `Event Move Meshes`
  ;[1 1 1] Item animation
  (bind (_direction _offset) (`Timeline|ItemMoveInSocketTimeline` :!via `PlayFromStart`)
    (:`Update`
      (`SceneComponent.K2_AddLocalOffset` (`/Game/LMiTW/Blueprints/GameplayActors/Pickup/BP_MasterPickup.PickupMesh` (`self.Item`)) (* (`self.ItemAnimationDirectionAndSpeed`) (* _offset (`GameplayStatics.GetWorldDeltaSeconds`))) false false))
    (:`Finished`
      ;[1 1 1] Power status ON
      (`self.SetPowerStatusForSlaveActors` (`self.HaveItemInstalled?`))
      (`/Game/LMiTW/HUD/GameplayActors/Interactable/WBP_Capsule.Event Finish Work` (`self.WBP_Capsule`) false)
      ;[1 1 1] Pointer animation
      (bind (_direction_2 _offset_2) (`Timeline|PointerPlatformOffsetTimeline` :!via `PlayFromStart`)
        (:`Update`
          (`SceneComponent.K2_AddLocalOffset` (`self.MovePlatform`) (* (`self.PointerAnimationDirectionAndSpeed`) (* _offset_2 (`GameplayStatics.GetWorldDeltaSeconds`))) false false))))))

(fn `ApplyItem`)

(fn `GetInteractInfo`
  (returns (Info :type "/Game/LMiTW/Blueprints/Structures/S_InteractionInfo Structure"))
  (return (`self.InteractInfo`)))

(fn `GetOrigin`
  (returns (OriginLocation :type "Vector Structure"))
  (return (`KismetSystemLibrary.GetComponentBounds` (`self.OutlinePointForScan`))))

(fn `GetSwitcherInfo`
  (returns (TypeOfSwitcher :type "/Game/LMiTW/Blueprints/Enums/E_SwitcherTYpe Enum") (`Online?` :type Boolean) (`DoorOpen?` :type Boolean) (SwitcherActor :type "/Game/LMiTW/Blueprints/GameplayActors/Switcher/BP_MasterSwitcher Object Reference") (ControlPanelStatus :type "/Game/LMiTW/Blueprints/Enums/E_SwitcherStatusRange Enum"))
  (return "NewEnumerator2" false false null "NewEnumerator0"))

(fn `SetPowerStatusForSlaveActors`
  (params (`PowerOn?` :type Boolean))
  (if `PowerOn?`
    ;[1 1 1] If item installed, power turn on
    (`|ExecutionSequence`
      (:`then_0`
        (for _array_element (`self.ListOfInfluencePowerActors`)
          (if (`KismetSystemLibrary.DoesImplementInterface` _array_element "/Game/LMiTW/Blueprints/Interface/BPI_PowerSupply.BPI_PowerSupply_C")
            (message `/Game/LMiTW/Blueprints/Interface/BPI_PowerSupply.TurnOnPower` _array_element)
            (bind _asbp_door_control_panel (cast `/Game/LMiTW/Blueprints/GameplayActors/Switcher/BP_DoorControlPanel` _array_element))
            ;[1 0 0.1525] Delete this bicycle by make 1 function for Control panel
            (`/Game/LMiTW/Blueprints/GameplayActors/Switcher/BP_DoorControlPanel.UpdateWidgetInfo` _asbp_door_control_panel false)
            (bind _outstatus (`/Game/LMiTW/Blueprints/GameplayActors/Switcher/BP_DoorControlPanel.GetStatus` _asbp_door_control_panel))
            (`/Game/LMiTW/Blueprints/GameplayActors/Switcher/BP_DoorControlPanel.SetStatus` _asbp_door_control_panel _outstatus)
            (else
              (`KismetSystemLibrary.PrintString` "ERR. BP_Generator. Referencead actor have no BPI_PowerSupply" true true (struct :`R` 1.0 :`G` 0.180672 :`A` 1.0) 10.0))))))
    (else
      ;[1 1 1] if item not installed, power turn off
      (for _array_element_2 (`self.ListOfInfluencePowerActors`)
        (if (`KismetSystemLibrary.DoesImplementInterface` _array_element_2 "/Game/LMiTW/Blueprints/Interface/BPI_PowerSupply.BPI_PowerSupply_C")
          (message `/Game/LMiTW/Blueprints/Interface/BPI_PowerSupply.TurnOffPower` _array_element_2)
          (bind _asbp_door_control_panel_2 (cast `/Game/LMiTW/Blueprints/GameplayActors/Switcher/BP_DoorControlPanel` _array_element_2))
          (`/Game/LMiTW/Blueprints/GameplayActors/Switcher/BP_DoorControlPanel.UpdateWidgetInfo` _asbp_door_control_panel_2 false)
          (bind _outstatus_2 (`/Game/LMiTW/Blueprints/GameplayActors/Switcher/BP_DoorControlPanel.GetStatus` _asbp_door_control_panel_2))
          (`/Game/LMiTW/Blueprints/GameplayActors/Switcher/BP_DoorControlPanel.SetStatus` _asbp_door_control_panel_2 _outstatus_2)
          (else
            (`KismetSystemLibrary.PrintString` "ERR. BP_Generator. Referencead actor have no BPI_PowerSupply" true true (struct :`R` 1.0 :`G` 0.180672 :`A` 1.0) 10.0)))))))

(fn `SetRenderCustomDepth`
  (params (Render :type Boolean))
  (`PrimitiveComponent.SetRenderCustomDepth` (`self.MeshGenerator`) Render))

(fn `UserConstructionScript`
  (`StaticMeshComponent.SetStaticMesh` (`self.MeshGenerator`) (`.StaticMesh_23_9F5223F84DD7D2895F9C5585A125810E` (break `/Game/LMiTW/Blueprints/Structures/S_ItemInfo` (`self.ItemInfo`)))))