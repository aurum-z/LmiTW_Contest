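; Interactable quest actor with a static mesh that toggles custom depth rendering as it gains or loses focus, typically for a highlight.
; Focus events route through a shared SetRenderCustomDepth helper, while Interact is an empty stub.
; Getters expose the InteractInfo, the mesh's bounds origin and a fixed default switcher state (type, online, door, control panel).
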(event `/Game/LMiTW/Blueprints/Interface/BPI_Interactable.Interact`
  (params (Interactor :type "/Game/LMiTW/Blueprints/Character/BP_LMPlayerCharacter Object Reference") (InputKey :type "Key Structure")))

(event `/Game/LMiTW/Blueprints/Interface/BPI_Interactable.StartFocus`
  (`self.SetRenderCustomDepth` true))

(event `/Game/LMiTW/Blueprints/Interface/BPI_Interactable.StopFocus`
  (`self.SetRenderCustomDepth` false))

(fn `GetInteractInfo`
  (returns (Info :type "/Game/LMiTW/Blueprints/Structures/S_InteractionInfo Structure"))
  (return (`self.InteractInfo`)))

(fn `GetOrigin`
  (returns (OriginLocation :type "Vector Structure"))
  (return (`KismetSystemLibrary.GetComponentBounds` (`self.StaticMesh`))))

(fn `GetSwitcherInfo`
  (returns (TypeOfSwitcher :type "/Game/LMiTW/Blueprints/Enums/E_SwitcherTYpe Enum") (`Online?` :type Boolean) (`DoorOpen?` :type Boolean) (SwitcherActor :type "/Game/LMiTW/Blueprints/GameplayActors/Switcher/BP_MasterSwitcher Object Reference") (ControlPanelStatus :type "/Game/LMiTW/Blueprints/Enums/E_SwitcherStatusRange Enum"))
  (return "NewEnumerator2" false false null "NewEnumerator0"))

(fn `SetRenderCustomDepth`
  (params (Render :type Boolean))
  (`PrimitiveComponent.SetRenderCustomDepth` (`self.StaticMesh`) Render))

(fn `UserConstructionScript`)