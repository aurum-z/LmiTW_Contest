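; Box-trigger hazard zone that harms the player with Fire or Electricity, or drives a post-process blur for Smoke.
; On BeginPlay, a looping timer polls until the player character exists, then caches it and precomputes per-tick damage from max health or blur steps.
; Player capsule overlaps start and stop the damage timer, or swap between timers that step the post-process blend weight on enter and exit.
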(event `self.ReceiveBeginPlay`
  (`self.CreateTimerAskCharacter`))

(event `self.Box.OnComponentBeginOverlap`
  (params (OverlappedComponent :type "PrimitiveComponent Object Reference") (OtherActor :type "Actor Object Reference") (OtherComp :type "PrimitiveComponent Object Reference") (OtherBodyIndex :type Integer) (bFromSweep :type Boolean) (SweepResult :type "HitResult Structure (by ref)"))
  ;[1 1 1] Box Collision
  (`self.TryActivateEffect` OtherActor OtherComp))

(event `self.Box.OnComponentEndOverlap`
  (params (OverlappedComponent :type "PrimitiveComponent Object Reference") (OtherActor :type "Actor Object Reference") (OtherComp :type "PrimitiveComponent Object Reference") (OtherBodyIndex :type Integer))
  ;[1 1 1] Box Collision
  (`self.TryDeactivateEffect` OtherActor OtherComp))

(fn `ActivateAddBlurTimerAndDeactivateAnotherT`
  (`KismetSystemLibrary.K2_ClearAndInvalidateTimerHandle` (`self.TimerSubtractionBlur`))
  (bind _returnvalue (`KismetSystemLibrary.K2_SetTimer` null "AddBlur" (`self.CallFrequinceForBlur`) true))
  (set `self.TimerAddBlur` _returnvalue))

(fn `ActivateDamageTimer`
  (bind _returnvalue (`KismetSystemLibrary.K2_SetTimer` null "DamagePlayerCharacter" (`self.CallFrequinceForHealthDamage`) true))
  (set `self.TimerForDamageCharacter` _returnvalue))

(fn `ActivateSubtractionBlurTimerAndDeactivateAnotherT`
  (`KismetSystemLibrary.K2_ClearAndInvalidateTimerHandle` (`self.TimerAddBlur`))
  (bind _returnvalue (`KismetSystemLibrary.K2_SetTimer` null "SubtractionBlur" (`self.CallFrequinceForBlur`) true))
  (set `self.TimerSubtractionBlur` _returnvalue))

(fn `AddBlur`
  (bind _returnvalue (+ (`self.CurrentBlur`) (`self.AmountOfBlurToAdd`)))
  (set `self.CurrentBlur` _returnvalue)
  (if (>= _returnvalue 0.95)
    ;[1 1 1] End work process
    (set `self.CurrentBlur` 1.0)
    (set `PostProcessComponent.BlendWeight` (`self.AmountOfBlurToAdd`) (`self.PostProcess`))
    (`KismetSystemLibrary.K2_ClearAndInvalidateTimerHandle` (`self.TimerAddBlur`))
    (else
      (set `PostProcessComponent.BlendWeight` (- 1.0 (`self.CurrentBlur`)) (`self.PostProcess`)))))

(fn `AskCharacterAndDestroyTimer`
  (returns (CharacterMaxHealth :type "Float (double-precision)") (`Success?` :type Boolean))
  (bind _outactors (`GameplayStatics.GetAllActorsOfClass` "/Game/LMiTW/Blueprints/Character/BP_LMPlayerCharacter.BP_LMPlayerCharacter_C"))
  (bind _output (`|GetArrayItem` _outactors))
  (`/Engine/EditorBlueprintResources/StandardMacros.IsValid` _output
    (:`Is Valid`
      (`KismetSystemLibrary.K2_ClearAndInvalidateTimerHandle` (`self.TimerForCharacterAsk`))
      (bind _output_get (set `self.BP_PlayerCharacter` _output))
      (set `self.CharacterCapsuleCollision` (`Character.CapsuleComponent` _output_get))
      (bind _maxhealth (`/Game/LMiTW/Blueprints/Character/BP_LMPlayerCharacter.GetMaxHealth` _output_get))
      (return _maxhealth true))
    (:`Is Not Valid`
      (return -1.1 false))))

(fn `CalculateAmountOfBlur`
  (`|ExecutionSequence`
    (:`then_0`
      (set `self.AmountOfBlurToAdd` (* (`self.BlurPercentAddPerSecond`) (`self.CallFrequinceForBlur`) 0.01)))
    (:`then_1`
      (set `self.AmountOfBlurToSubtract` (* (`self.BlurPercentSubtractPerSecond`) (`self.CallFrequinceForBlur`) 0.01)))))

(fn `CalculateHealthToSubstract`
  (params (CharacterMaxHealth :type "Float (double-precision)"))
  (switch `/Game/LMiTW/Blueprints/Enums/E_EnvironmentZones` (`self.Effect`)
    (:`NewEnumerator1`
      (set `self.AmountOfHealthForCharacterDamage` (* (/ CharacterMaxHealth 100.0) (`self.FirePercentDamagePerSecond`) (`self.CallFrequinceForHealthDamage`))))
    (:`NewEnumerator2`
      (set `self.AmountOfHealthForCharacterDamage` (* (/ CharacterMaxHealth 100.0) (`self.ElectricityPercentDamagePerSecond`) (`self.CallFrequinceForHealthDamage`))))))

(fn `CreateMesh`
  (`AddComponent|NODE_AddStaticMeshComponent-0` :`RelativeTransform` (`SceneComponent.K2_GetComponentToWorld` (`self.DefaultSceneRoot`))))

(fn `CreateTimerAskCharacter`
  (bind _returnvalue (`KismetSystemLibrary.K2_SetTimer` null "Preparation" (`KismetMathLibrary.RandomFloatInRange` 0.5 0.6) true))
  (set `self.TimerForCharacterAsk` _returnvalue))

(fn `DamagePlayerCharacter`
  (`GameplayStatics.ApplyDamage` (`self.BP_PlayerCharacter`) (`self.AmountOfHealthForCharacterDamage`)))

(fn `DeactivateDamageTimer`
  (`KismetSystemLibrary.K2_ClearAndInvalidateTimerHandle` (`self.TimerForDamageCharacter`)))

(fn `GetCharacterMaxHealth`
  (returns (maxHealth :type "Float (double-precision)"))
  (return 0.0))

(fn `GetPlayerCharacter`
  (returns (PlayerCharacter :type "/Game/LMiTW/Blueprints/Character/BP_LMPlayerCharacter Object Reference"))
  (return (`self.BP_PlayerCharacter`)))

(fn `IsPlayerCharacter?`
  (params (Actor :type "Actor Object Reference") (ActorComponent :type "ActorComponent Object Reference"))
  (returns (`IsPlayerCharacter?` :type Boolean))
  (bind _bp_playercharacter (`self.BP_PlayerCharacter`))
  (`/Engine/EditorBlueprintResources/StandardMacros.IsValid` _bp_playercharacter
    (:`Is Valid`
      (return (and (== _bp_playercharacter Actor) (== ActorComponent (`self.CharacterCapsuleCollision`)))))))

(fn `PreInit`
  (`BoxComponent.SetBoxExtent` (`self.Box`) (`self.BoxExtent`) true)
  (set `PostProcessComponent.BlendWeight` 0.0 (`self.PostProcess`))
  (`SceneComponent.K2_SetRelativeTransform` (`self.ParticleSystem`) (`self.ParticleSystemTransform`) false false))

(fn `Preparation`
  ;[1 1 1] Destroy "Character Ask timer" if success
  (bind (_charactermaxhealth _success_) (`self.AskCharacterAndDestroyTimer`))
  (if _success_
    (switch `/Game/LMiTW/Blueprints/Enums/E_EnvironmentZones` (`self.Effect`)
      (:`NewEnumerator1`
        (`self.CalculateHealthToSubstract` _charactermaxhealth :!label _label))
      (:`NewEnumerator2`
        (goto _label))
      (:`NewEnumerator3`
        (`self.CalculateAmountOfBlur`)))))

(fn `SetEffect`
  (params (Effect :type "/Game/LMiTW/Blueprints/Enums/E_EnvironmentZones Enum" :default "NewEnumerator0"))
  (set `self.Effect` Effect))

(fn `SubtractionBlur`
  (bind _returnvalue (- (`self.CurrentBlur`) (`self.AmountOfBlurToSubtract`)))
  (set `self.CurrentBlur` _returnvalue)
  (if (<= _returnvalue 0.55)
    ;[1 1 1] End work process
    (bind _output_get (set `self.CurrentBlur` 0.0))
    (set `PostProcessComponent.BlendWeight` _output_get (`self.PostProcess`))
    (`KismetSystemLibrary.K2_ClearAndInvalidateTimerHandle` (`self.TimerSubtractionBlur`))
    (else
      (set `PostProcessComponent.BlendWeight` (- 1.0 (`self.CurrentBlur`)) (`self.PostProcess`)))))

(fn `TryActivateEffect`
  (params (Actor :type "Actor Object Reference") (ActorComponent :type "ActorComponent Object Reference"))
  (bind _isplayercharacter_ (`self.IsPlayerCharacter?` Actor ActorComponent))
  (if _isplayercharacter_
    (switch `/Game/LMiTW/Blueprints/Enums/E_EnvironmentZones` (`self.Effect`)
      (:`NewEnumerator1`
        (`self.ActivateDamageTimer` :!label _label))
      (:`NewEnumerator2`
        (goto _label))
      (:`NewEnumerator3`
        (`self.ActivateAddBlurTimerAndDeactivateAnotherT`)))))

(fn `TryDeactivateEffect`
  (params (Actor :type "Actor Object Reference") (ActorComponent :type "ActorComponent Object Reference"))
  (bind _isplayercharacter_ (`self.IsPlayerCharacter?` Actor ActorComponent))
  (if _isplayercharacter_
    (switch `/Game/LMiTW/Blueprints/Enums/E_EnvironmentZones` (`self.Effect`)
      (:`NewEnumerator1`
        (`self.DeactivateDamageTimer` :!label _label))
      (:`NewEnumerator2`
        (goto _label))
      (:`NewEnumerator3`
        (`self.ActivateSubtractionBlurTimerAndDeactivateAnotherT`)))))

(fn `UserConstructionScript`
  (`self.PreInit`))