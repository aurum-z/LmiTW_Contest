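; Electricity hazard zone that, with freezing enabled, intermittently locks the player's movement and mouse input.
; Box overlaps track the player's presence in freezing mode, or defer to the parent effect otherwise.
; A Freeze timeline drives the pulse, with two cross-resetting DoOnce nodes toggling audio, particles and the freeze only at threshold crossings.
; Leaving the zone releases the player immediately.
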(event `self.ReceiveBeginPlay`
  (`parent.ReceiveBeginPlay`)
  (if (`self.freezingEffectActive?`)
    (switch `int` (`self.FreezingTimeLineNumber`)
      (:`Default`
        ;[1 1 1] Add new time line with function "Update Freezing Status", if u want use 1 more time lines
        (bind (_direction _freezeactive_) (`Timeline|Freeze` :!via `PlayFromStart` :!label _label)
          (:`Update`
            (`self.UpdateFreezingStatus` _freezeactive_))))
      (:`0`
        (goto _label :!via `PlayFromStart`)))))

(event `self.Box.OnComponentBeginOverlap`
  (params (OverlappedComponent :type "PrimitiveComponent Object Reference") (OtherActor :type "Actor Object Reference") (OtherComp :type "PrimitiveComponent Object Reference") (OtherBodyIndex :type Integer) (bFromSweep :type Boolean) (SweepResult :type "HitResult Structure (by ref)"))
  (`self.TryActivateEffect` OtherActor OtherComp))

(event `self.Box.OnComponentEndOverlap`
  (params (OverlappedComponent :type "PrimitiveComponent Object Reference") (OtherActor :type "Actor Object Reference") (OtherComp :type "PrimitiveComponent Object Reference") (OtherBodyIndex :type Integer))
  (`self.TryDeactivateEffect` OtherActor OtherComp))

(fn `TryActivateEffect`
  (params (Actor :type "Actor Object Reference") (ActorComponent :type "ActorComponent Object Reference"))
  (if (`self.freezingEffectActive?`)
    (`self.TryActivateFreezing` Actor ActorComponent)
    (else
      (`parent.TryActivateEffect` Actor ActorComponent))))

(fn `TryActivateFreezing`
  (params (Actor :type "Actor Object Reference") (ActorComponent :type "ActorComponent Object Reference"))
  (bind _isplayercharacter_ (`self.IsPlayerCharacter?` Actor ActorComponent))
  (if _isplayercharacter_
    (set `self.playerInZone?` true)))

(fn `TryDeactivateEffect`
  (params (Actor :type "Actor Object Reference") (ActorComponent :type "ActorComponent Object Reference"))
  (if (`self.freezingEffectActive?`)
    (`self.TryDeactivateFreezing` Actor ActorComponent)
    (else
      (`parent.TryDeactivateEffect` Actor ActorComponent))))

(fn `TryDeactivateFreezing`
  (params (Actor :type "Actor Object Reference") (ActorComponent :type "ActorComponent Object Reference"))
  (bind _isplayercharacter_ (`self.IsPlayerCharacter?` Actor ActorComponent))
  (if _isplayercharacter_
    (set `self.playerInZone?` false)
    (bind _playercharacter (`self.GetPlayerCharacter`))
    (message `/Game/LMiTW/Blueprints/Interface/BPI_Movement.FreezingMoveAndMouse` _playercharacter false false)))

(fn `UpdateFreezingStatus`
  (params (`FreezeActive?` :type "Float (double-precision)"))
  (if (> `FreezeActive?` 0.9)
    (`/Engine/EditorBlueprintResources/StandardMacros.DoOnce` false :!label _label
      (:`Completed`
        (`|ExecutionSequence`
          (:`then_0`
            (`AudioComponent.SetVolumeMultiplier` (`self.Audio`) 1.0)
            (`SceneComponent.SetVisibility` (`self.ParticleSystem`) true false)
            (if (`self.playerInZone?`)
              ;[1 1 1] Freeze
              (set `self.freezePlayer` true)
              (bind _playercharacter (`self.GetPlayerCharacter`))
              (message `/Game/LMiTW/Blueprints/Interface/BPI_Movement.FreezingMoveAndMouse` _playercharacter true true)))
          (:`then_1`
            (goto _label_2 :!via `Reset`)))))
    (else
      (`/Engine/EditorBlueprintResources/StandardMacros.DoOnce` false :!label _label_2
        (:`Completed`
          (`|ExecutionSequence`
            (:`then_0`
              (`AudioComponent.SetVolumeMultiplier` (`self.Audio`) 0.0)
              (`SceneComponent.SetVisibility` (`self.ParticleSystem`) false false)
              (if (`self.playerInZone?`)
                ;[1 1 1] No effect
                (set `self.freezePlayer` false)
                (bind _playercharacter_2 (`self.GetPlayerCharacter`))
                (message `/Game/LMiTW/Blueprints/Interface/BPI_Movement.FreezingMoveAndMouse` _playercharacter_2 false false)))
            (:`then_1`
              (goto _label :!via `Reset`))))))))

(fn `UserConstructionScript`
  (`parent.UserConstructionScript`)
  (`self.SetEffect` "NewEnumerator2"))