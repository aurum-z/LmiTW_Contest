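; Box volume actor that marks an area without oxygen, activating an overlapping actor's BP_PlayerOxygenComponent on entry and deactivating it on exit.
; PreInit applies the configured box extent, and Init sets collision from the IsHasOxygen flag.
; SetOxygenStatus toggles the volume between query-only and no collision, so it only triggers while oxygen is absent.
; Indirect control events drive that status: activation removes oxygen, deactivation restores it.
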(event `self.Volume.OnComponentBeginOverlap`
  (params (OverlappedComponent :type "PrimitiveComponent Object Reference") (OtherActor :type "Actor Object Reference") (OtherComp :type "PrimitiveComponent Object Reference") (OtherBodyIndex :type Integer) (bFromSweep :type Boolean) (SweepResult :type "HitResult Structure (by ref)"))
  ;[0.5833 1 0.6396] Overlap handling
  (`/Game/LMiTW/Blueprints/Components/BP_PlayerOxygenComponent.ActivateOxygenComponent` (`self.GetComponentByClass` OtherActor "/Game/LMiTW/Blueprints/Components/BP_PlayerOxygenComponent.BP_PlayerOxygenComponent_C")))

(event `self.Volume.OnComponentEndOverlap`
  (params (OverlappedComponent :type "PrimitiveComponent Object Reference") (OtherActor :type "Actor Object Reference") (OtherComp :type "PrimitiveComponent Object Reference") (OtherBodyIndex :type Integer))
  ;[0.5833 1 0.6396] Overlap handling
  (`/Game/LMiTW/Blueprints/Components/BP_PlayerOxygenComponent.DeactivateOxygenComponent` (`self.GetComponentByClass` OtherActor "/Game/LMiTW/Blueprints/Components/BP_PlayerOxygenComponent.BP_PlayerOxygenComponent_C")))

(event `/Game/LMiTW/Blueprints/Interface/BPI_RemoteControl.ActivateControlledActor`
  ;[0.5833 1 0.6396] IndirectControl
  (`self.SetOxygenStatus` false))

(event `/Game/LMiTW/Blueprints/Interface/BPI_RemoteControl.DeactivateControlledActor`
  ;[0.5833 1 0.6396] IndirectControl
  (`self.SetOxygenStatus` true))

(fn `DisableVolume`
  (`PrimitiveComponent.SetCollisionEnabled` (`self.Volume`) "NoCollision"))

(fn `EnableVolume`
  (`PrimitiveComponent.SetCollisionEnabled` (`self.Volume`) "QueryOnly"))

(fn `Init`
  (if (`self.IsHasOxygen`)
    (`self.DisableVolume`)
    (else
      (`self.EnableVolume`))))

(fn `PreInit`
  (`self.SetVolumeExtent` (`self.VolumeExtent`)))

(fn `SetOxygenStatus`
  (params (HasOxygen :type Boolean))
  (bind _output_get (set `self.IsHasOxygen` HasOxygen))
  (if _output_get
    (`self.DisableVolume`)
    (else
      (`self.EnableVolume`))))

(fn `SetVolumeExtent`
  (params (NewExtent :type "Vector Structure" :default (100.0 100.0 100.0)))
  (`BoxComponent.SetBoxExtent` (`self.Volume`) NewExtent true))

(fn `UserConstructionScript`)