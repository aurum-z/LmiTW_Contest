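; Master switcher that a player interacts with (F) to toggle a remotely controlled actor, such as a door, when the interactor's access level is high enough.
; On BeginPlay it binds to the controlled actor's remote control component to mirror its active state, warning if no actor is assigned.
; A separate event registers the switcher with a BP_MasterDoor after a BPI_Generator interface check.
; Focus toggles custom depth on the mesh for outlining.
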(event `self.ReceiveBeginPlay`
  ;[1 1 1] Init
  (`self.Init`))

(event `Event_AddSwitcherToDoorBP`
  ;[1 1 1] Add self reference to controlled door
  (`self.AddSwitcherToDoorBP`))

(event `/Game/LMiTW/Blueprints/Interface/BPI_Interactable.Interact`
  (params (Interactor :type "/Game/LMiTW/Blueprints/Character/BP_LMPlayerCharacter Object Reference") (InputKey :type "Key Structure"))
  ;[1 1 1] Interaction
  (if (== InputKey "F")
    (bind _haveaccess (`self.CheckAccessLevel` Interactor))
    (if _haveaccess
      (`self.TryActivateRemoteActor`))))

(event `/Game/LMiTW/Blueprints/Interface/BPI_Interactable.StartFocus`
  ;[1 1 1] Outline postroccess visibility
  (`self.SetRenderCustomDepth` true))

(event `/Game/LMiTW/Blueprints/Interface/BPI_Interactable.StopFocus`
  ;[1 1 1] Outline postroccess visibility
  (`self.SetRenderCustomDepth` false))

(event `RemoteControlActorActivated`
  (`self.SetControlledActorState` true))

(event `RemoteControlActorDeactivated`
  (`self.SetControlledActorState` false))

(fn `AddSwitcherToDoorBP`
  (bind _returnvalue (`KismetSystemLibrary.Conv_InterfaceToObject` (`self.ControlledActor`)))
  (if (`KismetSystemLibrary.DoesImplementInterface` _returnvalue "/Game/LMiTW/Blueprints/Interface/BPI_Generator.BPI_Generator_C")
    (bind _asbp_master_door (cast `/Game/LMiTW/Blueprints/GameplayActors/Door/BP_MasterDoor` _returnvalue)
      (:`then`
        (message `/Game/LMiTW/Blueprints/Interface/BPI_Generator.SetSwitcherReferencesToDoor` _asbp_master_door self))
      (:`CastFailed`
        (`KismetSystemLibrary.PrintString` (`KismetStringLibrary.Concat_StrStr` (`KismetSystemLibrary.GetObjectName` self) "AddSwitcherToDoorBP function. ERR. Controlled Actor doesn`t cast") true true (struct :`R` 1.0 :`G` 0.060741 :`A` 1.0) 15.0)))
    (else
      (`KismetSystemLibrary.PrintString` (`KismetStringLibrary.Concat_StrStr` (`KismetSystemLibrary.GetObjectName` self) "AddSwitcherToDoorBP function. ERR. Controlled Actor doesn`t have interface") true true (struct :`R` 1.0 :`G` 0.060741 :`A` 1.0) 15.0))))

(fn `BindRemoteControlEvents`
  (locals (Local_RemoteControlComponent :type "/Game/LMiTW/Blueprints/Components/BP_RemoteControlComponent Object Reference"))
  (bind _controlledactor (`self.ControlledActor`))
  (`/Engine/EditorBlueprintResources/StandardMacros.IsValid` (`KismetSystemLibrary.Conv_InterfaceToObject` _controlledactor)
    (:`Is Valid`
      (bind _component (`/Game/LMiTW/Blueprints/Interface/BPI_RemoteControl.GetRemoteControlComponent` _controlledactor))
      (bind _output_get (set `local.Local_RemoteControlComponent` _component))
      (`/Engine/EditorBlueprintResources/StandardMacros.IsValid` _output_get
        (:`Is Valid`
          (add `/Game/LMiTW/Blueprints/Components/BP_RemoteControlComponent.OnControlledActorActivated` (`local.Local_RemoteControlComponent`) (`|CreateDelegate` :!event `RemoteControlActorActivated`))
          (add `/Game/LMiTW/Blueprints/Components/BP_RemoteControlComponent.OnControlledActorDeactivated` (`local.Local_RemoteControlComponent`) (`|CreateDelegate` :!event `RemoteControlActorDeactivated`)))))
    (:`Is Not Valid`
      (`KismetSystemLibrary.PrintString` (`KismetStringLibrary.Concat_StrStr` "Warning. " (`KismetSystemLibrary.GetObjectName` self) " have no controlled actor. delete this actor from scene") true true (struct :`R` 1.0 :`G` 0.570476 :`A` 1.0) 10.0))))

(fn `CheckAccessLevel`
  (params (Interactor :type "Actor Object Reference"))
  (returns (HaveAccess :type Boolean))
  (bind _access_level (message `/Game/LMiTW/Blueprints/Interface/BPI_PlayerInteraction.GetAccessLevel` Interactor))
  (return (>= _access_level (`self.AccessLevel`))))

(fn `GetInteractInfo`
  (returns (Info :type "/Game/LMiTW/Blueprints/Structures/S_InteractionInfo Structure"))
  (return (`self.InteractInfo`)))

(fn `Init`
  (`self.BindRemoteControlEvents`))

(fn `SetControlledActorState`
  (params (IsActive :type Boolean))
  (set `self.ControlledActorIsActive` IsActive)
  (return))

(fn `SetRenderCustomDepth`
  (params (Render :type Boolean))
  (`PrimitiveComponent.SetRenderCustomDepth` (`self.SwitcherMesh`) Render))

(fn `TryActivateRemoteActor`
  (set `self.IsActivated` (not (`self.IsActivated`)))
  (if (`self.IsActivated`)
    (`/Game/LMiTW/Blueprints/Interface/BPI_RemoteControl.ActivateControlledActor` (`self.ControlledActor`))
    (else
      (`/Game/LMiTW/Blueprints/Interface/BPI_RemoteControl.DeactivateControlledActor` (`self.ControlledActor`)))))

(fn `UserConstructionScript`)