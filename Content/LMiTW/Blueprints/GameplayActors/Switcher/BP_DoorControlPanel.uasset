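; Door control panel switcher whose Status configures its linked door, access level, indicator light color and 3D screen widget.
; F opens directly when Unlocked, checks the interactor's access level, or for pin codes moves camera and input to the panel until Q/Escape.
; Power events toggle interaction and refresh the widget.
; Status None also disables the slider door's nav link; several pin-code pieces are marked temporary until a planned move to the PDA.
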(event `self.ReceiveBeginPlay`
  (`self.Init`)
  (`self.SetStatus` (`self.Status`))
  (`|ExecutionSequence`
    (:`then_0`
      (`self.TryDestroyNavLink`))
    (:`then_1`
      ;[1 0.04116 0.071] delete in future, when pincode move to PDA
      (set `/Game/LMiTW/HUD/GameplayActors/Interactable/WBP_DoorControlPanel.ParentActor` self (`self.Widget`))
      (switch `/Game/LMiTW/Blueprints/Enums/E_SwitcherStatusRange` (`self.Status`)
        (:`NewEnumerator5`
          _)
        (:`NewEnumerator7`
          _)
        (:`NewEnumerator9`
          _))
      (`KismetSystemLibrary.Delay` 5.0)
      (if (== (`self.BP_Note`) null)
        (`KismetSystemLibrary.PrintString` (`KismetStringLibrary.Concat_StrStr` "ERR." (`KismetSystemLibrary.GetObjectName` self) ".  BP_Note variable have no refereance") true true (struct :`R` 1.0 :`B` 0.013939 :`A` 1.0) 10.0)))))

(event `/Game/LMiTW/Blueprints/Interface/BPI_Interactable.Interact`
  (params (Interactor :type "/Game/LMiTW/Blueprints/Character/BP_LMPlayerCharacter Object Reference") (InputKey :type "Key Structure"))
  ;[1 1 1] Interact
  (if (and (`self.IsOnline`) (== InputKey "F"))
    (switch `/Game/LMiTW/Blueprints/Enums/E_SwitcherStatusRange` (`self.Status`)
      (:`NewEnumerator11`
        ;[1 1 1] Unlocked
        (`self.TryActivateRemoteActor`))
      (:`NewEnumerator1`
        ;[1 1 1] Access level
        (bind _haveaccess (`self.CheckAccessLevel` Interactor :!label _label))
        (if _haveaccess
          (`self.TryActivateRemoteActor`)
          (else
            (`KismetSystemLibrary.PrintString` "PDA Have no access"))))
      (:`NewEnumerator2`
        (goto _label))
      (:`NewEnumerator3`
        (goto _label))
      (:`NewEnumerator5`
        ;[1 1 1] Send PDA or player message to start mini game
        (`/Game/LMiTW/Blueprints/Character/BP_LMPlayerCharacter.E_SetNewCameraAndRedirectInput` Interactor self (`self.Arrow`) :!label _label_2)
        ;[1 0 0.1046] Delete in future
        (set `self.User` Interactor)
        (set `self.UserController` (`Pawn.GetController` Interactor))
        (`/Game/LMiTW/Blueprints/Character/BP_LMPlayerCharacter.SetInteractObjectLockMovement` (`self.User`) true))
      (:`NewEnumerator7`
        (goto _label_2))
      (:`NewEnumerator9`
        (goto _label_2)))))

(event `E_InteractExit`
  (params (inputKey :type "Key Structure" :default "None"))
  ;[1 1 1] Exit
  (if (and (`self.IsOnline`) (or (== inputKey "Q") (== inputKey "Escape")))
    (`/Engine/EditorBlueprintResources/StandardMacros.IsValid` (`self.User`)
      (:`Is Valid`
        (`/Game/LMiTW/Blueprints/Character/BP_LMPlayerCharacter.E_SetNewCameraAndRedirectInput` (`self.User`) self (`self.Arrow`))
        ;[1 0 0.1046] Delete in future
        (`/Game/LMiTW/Blueprints/Character/BP_LMPlayerCharacter.SetInteractObjectLockMovement` (`self.User`) false)
        (set `self.User` null)
        (set `self.UserController` null)))))

(event `/Game/LMiTW/Blueprints/Interface/BPI_PowerSupply.TurnOffPower`
  ;[1 1 1] PowerSupply
  (set `self.IsOnline` false)
  (`self.UpdateWidgetInfo` false :!label _label_3))

(event `/Game/LMiTW/Blueprints/Interface/BPI_PowerSupply.TurnOnPower`
  ;[1 1 1] PowerSupply
  (set `self.IsOnline` true)
  (goto _label_3))

(fn `GetInteractInfo`
  (returns (Info :type "/Game/LMiTW/Blueprints/Structures/S_InteractionInfo Structure"))
  (return (`self.InteractInfo`)))

(fn `GetStatus`
  (returns (outStatus :type "/Game/LMiTW/Blueprints/Enums/E_SwitcherStatusRange Enum"))
  (return (`self.Status`)))

(fn `Init`
  (`parent.Init`)
  (bind _returnvalue (`|CreateWidget` (`self.WidgetClass`)))
  (bind _output_get (set `self.Widget` _returnvalue))
  (`WidgetComponent.SetWidget` (`self.3dWidget`) _output_get)
  (`self.UpdateWidgetInfo` false))

(fn `SetAccessLevel`
  (params (InAccessLevel :type "/Game/LMiTW/Blueprints/Enums/E_AcessLevels Enum" :default "NewEnumerator3"))
  (set `self.AccessLevel` InAccessLevel))

(fn `SetControlledActorState`
  (params (IsActive :type Boolean))
  (`parent.SetControlledActorState` IsActive)
  (set `self.IsActivated` IsActive)
  (`self.UpdateWidgetInfo` false))

(fn `SetLightIndicatorStatus`
  (params (SwitcherStatus :type "/Game/LMiTW/Blueprints/Enums/E_SwitcherStatusRange Enum" :default "NewEnumerator0"))
  (switch `/Game/LMiTW/Blueprints/Enums/E_SwitcherStatusRange` SwitcherStatus
    (:`NewEnumerator0`
      ;[1 1 1] Red
      (`PrimitiveComponent.SetMaterial` (`self.LightIndicator`) 2 "/Game/LMiTW/Assets/ModSciInteriors/Materials/Lights/MI_Base_Light_Red.MI_Base_Light_Red" :!label _label))
    (:`NewEnumerator12`
      (goto _label))
    (:`NewEnumerator13`
      ;[1 1 1] Green
      (`PrimitiveComponent.SetMaterial` (`self.LightIndicator`) 2 "/Game/LMiTW/Assets/ModSciInteriors/Materials/Lights/MI_Base_Light_Green.MI_Base_Light_Green" :!label _label_2))
    (:`NewEnumerator16`
      (goto _label_2))
    (:`NewEnumerator11`
      (goto _label_2))
    (:`NewEnumerator1`
      ;[1 1 1] Yellow
      (`PrimitiveComponent.SetMaterial` (`self.LightIndicator`) 2 "/Game/LMiTW/Assets/ModSciInteriors/Materials/Lights/MI_Base_Light_yellow.MI_Base_Light_yellow" :!label _label_3))
    (:`NewEnumerator2`
      (goto _label_3))
    (:`NewEnumerator3`
      (goto _label_3))
    (:`NewEnumerator5`
      (goto _label_3))
    (:`NewEnumerator7`
      (goto _label_3))
    (:`NewEnumerator9`
      (goto _label_3))))

(fn `SetStatus`
  (params (InStatus :type "/Game/LMiTW/Blueprints/Enums/E_SwitcherStatusRange Enum" :default "NewEnumerator0"))
  (bind _output_get (set `self.Status` InStatus))
  (switch `/Game/LMiTW/Blueprints/Enums/E_SwitcherStatusRange` _output_get
    (:`NewEnumerator0`
      ;[1 0 0] None
      (bind _asbp_master_door (cast `/Game/LMiTW/Blueprints/GameplayActors/Door/BP_MasterDoor` (`self.ControlledActor`)))
      (`self.SetAccessLevel` "NewEnumerator3")
      (`/Game/LMiTW/Blueprints/GameplayActors/Door/BP_MasterDoor.SetIsEnable` _asbp_master_door false)
      (`/Game/LMiTW/Blueprints/GameplayActors/Door/BP_MasterDoor.SetAutomaticClose` _asbp_master_door false)
      (`/Game/LMiTW/Blueprints/GameplayActors/Door/BP_MasterDoor.SetDisableAutomaticOpen` _asbp_master_door)
      (`/Game/LMiTW/Blueprints/GameplayActors/Door/BP_MasterDoor.E_Close_Door` _asbp_master_door)
      (set `/Game/LMiTW/Blueprints/GameplayActors/Door/BP_MasterDoor.DoorMode` "NewEnumerator1" _asbp_master_door))
    (:`NewEnumerator12`
      ;[1 1 1] Blocked
      (`self.SetAccessLevel` "NewEnumerator3")
      (bind _asbp_master_door_2 (cast `/Game/LMiTW/Blueprints/GameplayActors/Door/BP_MasterDoor` (`self.ControlledActor`)))
      (`/Game/LMiTW/Blueprints/GameplayActors/Door/BP_MasterDoor.SetIsEnable` _asbp_master_door_2 false)
      ;[1 0 0] Comment
      (`/Game/LMiTW/Blueprints/GameplayActors/Door/BP_MasterDoor.E_Close_Door` _asbp_master_door_2)
      (set `/Game/LMiTW/Blueprints/GameplayActors/Door/BP_MasterDoor.DoorMode` "NewEnumerator1" _asbp_master_door_2))
    (:`NewEnumerator13`
      ;[1 1 1] Bypassed
      (`self.SetAccessLevel` "NewEnumerator3")
      (bind _asbp_master_door_3 (cast `/Game/LMiTW/Blueprints/GameplayActors/Door/BP_MasterDoor` (`self.ControlledActor`)))
      ;;[1 0.08657 0] Comment
      (`/Game/LMiTW/Blueprints/GameplayActors/Door/BP_MasterDoor.E_Close_Door` _asbp_master_door_3)
      (message `/Game/LMiTW/Blueprints/Interface/BPI_Interactable.Interact` _asbp_master_door_3 null "None")
      (`/Game/LMiTW/Blueprints/GameplayActors/Door/BP_MasterDoor.SetAutomaticClose` _asbp_master_door_3 false)
      (`/Game/LMiTW/Blueprints/GameplayActors/Door/BP_MasterDoor.SetIsEnable` _asbp_master_door_3 false)
      ;[1 0 0] Comment
      (set `/Game/LMiTW/Blueprints/GameplayActors/Door/BP_MasterDoor.DoorMode` "NewEnumerator0" _asbp_master_door_3))
    (:`NewEnumerator16`
      ;[1 1 1] Automatic
      (`self.SetAccessLevel` "NewEnumerator3")
      (bind _asbp_master_door_4 (cast `/Game/LMiTW/Blueprints/GameplayActors/Door/BP_MasterDoor` (`self.ControlledActor`)))
      (set `/Game/LMiTW/Blueprints/GameplayActors/Door/BP_MasterDoor.DoorMode` "NewEnumerator0" _asbp_master_door_4)
      (`/Game/LMiTW/Blueprints/GameplayActors/Door/BP_MasterDoor.SetEnableAutomaticOpen` _asbp_master_door_4)
      ;;[1 0 0] Comment
      (`/Game/LMiTW/Blueprints/GameplayActors/Door/BP_MasterDoor.SetAutomaticClose` _asbp_master_door_4 true)
      (`/Game/LMiTW/Blueprints/GameplayActors/Door/BP_MasterDoor.E_Close_Door` _asbp_master_door_4))
    (:`NewEnumerator11`
      ;[1 1 1] Unlock
      (`self.SetAccessLevel` "NewEnumerator3")
      (bind _asbp_master_door_5 (cast `/Game/LMiTW/Blueprints/GameplayActors/Door/BP_MasterDoor` (`self.ControlledActor`) :!label _label))
      (`/Game/LMiTW/Blueprints/GameplayActors/Door/BP_MasterDoor.SetDisableAutomaticOpen` _asbp_master_door_5)
      ;[1 0 0.0781] Comment
      (`/Game/LMiTW/Blueprints/GameplayActors/Door/BP_MasterDoor.SetIsEnable` _asbp_master_door_5 true)
      (`/Game/LMiTW/Blueprints/GameplayActors/Door/BP_MasterDoor.E_Close_Door` _asbp_master_door_5)
      (set `/Game/LMiTW/Blueprints/GameplayActors/Door/BP_MasterDoor.DoorMode` "NewEnumerator1" _asbp_master_door_5))
    (:`NewEnumerator1`
      ;[1 1 1] Access levels
      (`self.SetAccessLevel` "NewEnumerator0")
      (goto _label))
    (:`NewEnumerator2`
      (`self.SetAccessLevel` "NewEnumerator1")
      (goto _label))
    (:`NewEnumerator3`
      (`self.SetAccessLevel` "NewEnumerator2")
      (goto _label))
    (:`NewEnumerator5`
      ;[1 1 1] PinCode
      (`self.SetAccessLevel` "NewEnumerator3" :!label _label_2))
    (:`NewEnumerator7`
      (goto _label_2))
    (:`NewEnumerator9`
      (goto _label_2)))
  ;[1 1 1] Change light indicator
  (if (`self.IsOnline`)
    (`self.SetLightIndicatorStatus` (`self.Status`))
    (else
      (`self.SetLightIndicatorStatus` "NewEnumerator0"))))

(fn `TryDestroyNavLink`
  (bind _returnvalue (`KismetSystemLibrary.Conv_InterfaceToObject` (`self.ControlledActor`)))
  (bind _outstatus (`self.GetStatus`))
  (switch `/Game/LMiTW/Blueprints/Enums/E_SwitcherStatusRange` _outstatus
    (:`NewEnumerator0`
      ;[1 1 1] Off proxy on the door if Status "None"
      (`/Engine/EditorBlueprintResources/StandardMacros.IsValid` _returnvalue
        (:`Is Valid`
          (bind _asbp_door_slider (cast `/Game/LMiTW/Blueprints/GameplayActors/Door/BP_DoorSlider` _returnvalue))
          (bind _navlink (`/Game/LMiTW/Blueprints/GameplayActors/Door/BP_DoorSlider.NavLink` _asbp_door_slider))
          (`/Engine/EditorBlueprintResources/StandardMacros.IsValid` _navlink
            (:`Is Valid`
              (`ActorComponent.Deactivate` _navlink)
              (`KismetArrayLibrary.Array_Clear` (`NavLinkComponent.Links` _navlink)))))))))

(fn `UpdateWidgetInfo`
  (params (`PlayerInteractReactionActive?` :type Boolean))
  (bind _outstatus (`self.GetStatus`))
  (`/Game/LMiTW/HUD/GameplayActors/Interactable/WBP_DoorControlPanel.UpdateInfo` (`self.Widget`) (make `/Game/LMiTW/Blueprints/Structures/S_DoorPanelInfo` (`self.IsOnline`) (`self.AccessLevel`) _outstatus (`self.IsActivated`))))

(fn `UserConstructionScript`
  (`parent.UserConstructionScript`)
  ;[1 1 1] Try Destroy Nav link if status "None"
  (`self.TryDestroyNavLink`)
  (`self.SetLightIndicatorStatus` (`self.Status`)))