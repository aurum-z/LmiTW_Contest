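; BP_ButtonCapsuleEscape is an interactable button that registers the player's escape through a capsule once the capsule has power.
; TurnonPower flags the capsule as energized and the button as activated, then refreshes its widget info.
; Interact requires power and an interactor of exactly the BP_LMPlayerCharacter class, then sets PlayerEscape through a DoOnce so it fires only once.
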(event `self.ReceiveBeginPlay`
  (`parent.ReceiveBeginPlay`))

(event `/Game/LMiTW/Blueprints/Interface/BPI_PowerSupply.TurnOnPower`
  (set `self.CapsuleHaveEnergy?` true)
  (set `self.IsActivated` true)
  (`self.UpdateWidgetInfo`))

(event `/Game/LMiTW/Blueprints/Interface/BPI_Interactable.Interact`
  (params (Interactor :type "/Game/LMiTW/Blueprints/Character/BP_LMPlayerCharacter Object Reference") (InputKey :type "Key Structure"))
  (if (and (`self.CapsuleHaveEnergy?`) (== (`GameplayStatics.GetObjectClass` Interactor) "/Game/LMiTW/Blueprints/Character/BP_LMPlayerCharacter.BP_LMPlayerCharacter_C"))
    (`/Engine/EditorBlueprintResources/StandardMacros.DoOnce` false
      (:`Completed`
        (set `self.PlayerEscape` true)))))

(fn `UserConstructionScript`
  (`parent.UserConstructionScript`))