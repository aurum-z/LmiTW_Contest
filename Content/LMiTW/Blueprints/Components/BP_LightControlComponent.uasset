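; BP_LightControlComponent is an actor component that makes the hallway lights of a BP_CorridorStraght corridor flicker at random.
; On BeginPlay, if enabled and the corridor's flicker is active, it gathers the owner's BP_main_hallway_light child actors.
; A looping timer at the corridor's update frequency makes one coin-flip roll and passes it with the corridor's high and low intensities to every light, switching them in unison.
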(event `self.ReceiveBeginPlay`
  (bind _successinit_ (`self.Init`))
  (if _successinit_
    (`KismetSystemLibrary.K2_SetTimerDelegate` (delegate `CustomEvent_0`) (`/Game/LMiTW/Blueprints/Drafts/BP_CorridorStraght.frequencyOfUpdate` (`self.ParentActor`)) true)))

(event `CustomEvent_0`
  (bind _returnvalue (`KismetMathLibrary.RandomIntegerInRange` 0 9))
  (bind _parentactor (`self.ParentActor`))
  (set `self.randInt` _returnvalue)
  (bind _output_get (set `self.EnableLight` (> _returnvalue 4)))
  (for _array_element (`self.RectLightComponents`)
    (`/Game/LMiTW/Blueprints/Lighte/BP_main_hallway_light.E_ChangeLight` _array_element _output_get (`/Game/LMiTW/Blueprints/Drafts/BP_CorridorStraght.HighIntensity` _parentactor) (`/Game/LMiTW/Blueprints/Drafts/BP_CorridorStraght.LowIntensity` _parentactor))))

(fn `Init`
  (returns (`SuccessInit?` :type Boolean))
  (bind _returnvalue (`self.GetOwner`))
  (bind _rectlightcomponents (`self.RectLightComponents`))
  (bind _asbp_corridor_straght (cast `/Game/LMiTW/Blueprints/Drafts/BP_CorridorStraght` _returnvalue))
  (bind _output_get (set `self.ParentActor` _asbp_corridor_straght))
  (if (and (`self.EnableWork?`) (`/Game/LMiTW/Blueprints/Drafts/BP_CorridorStraght.flickerActive?` _output_get))
    (for _array_element (`Actor.GetAllChildActors` _returnvalue true)
      (bind _asbp_main_hallway_light (cast `/Game/LMiTW/Blueprints/Lighte/BP_main_hallway_light` _array_element))
      (`KismetArrayLibrary.Array_Add` _rectlightcomponents _asbp_main_hallway_light))
    (if (`KismetArrayLibrary.Array_IsValidIndex` _rectlightcomponents)
      (return true)
      (else
        (return false)))
    (else
      (return false))))