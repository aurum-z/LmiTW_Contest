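; Player inventory component that keeps items in a fixed-size slot array, with adding, removing, swapping, splitting, dropping and using.
; Stackable items top up matching partial stacks, and any remainder takes an empty slot, marked by a no-item ID.
; Dropping spawns a pickup at a fixed offset from the owner; using spawns the item's usable-class actor and removes consumables.
; Successful changes broadcast the item array through an inventory-updated event.
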(event `self.ReceiveBeginPlay`
  (`KismetSystemLibrary.Delay` 0.1)
  (`self.Init`))

(fn `AddItem`
  (params (NewItemInfo :type "/Game/LMiTW/Blueprints/Structures/S_ItemInfo Structure"))
  (returns (Success :type Boolean))
  (locals (Local_NewItemInfo :type "/Game/LMiTW/Blueprints/Structures/S_ItemInfo Structure"))
  (set `local.Local_NewItemInfo` NewItemInfo)
  (if (`self.HaveEmptySlots`)
    (bind (_success _slotindex) (`self.SearchFreeSlot`))
    (if _success
      (`KismetArrayLibrary.Array_Set` (`self.Items`) _slotindex (`local.Local_NewItemInfo`))
      (`/Engine/EditorBlueprintResources/StandardMacros.IncrementInt` (`self.UsedSlots`)
        (:`  `
          (return true)))
      (else
        _)))
  (return false))

(fn `AddStackableItem`
  (params (NewItemInfo :type "/Game/LMiTW/Blueprints/Structures/S_ItemInfo Structure"))
  (returns (Success :type Boolean))
  (locals (Local_NewItemInfo :type "/Game/LMiTW/Blueprints/Structures/S_ItemInfo Structure") (Local_Count :type Integer) (Local_Id :type Integer) (Local_CurrentElementInfo :type "/Game/LMiTW/Blueprints/Structures/S_ItemInfo Structure") (Local_Index :type Integer) (Local_CountRemaining :type Integer))
  (bind ((`Count_17_D19A6EBD41C242C28CC0F39910C423A9` _count) (`StackSize_22_A0B76A20497498BC51DB029EFCFB634F` _stacksize)) (break `/Game/LMiTW/Blueprints/Structures/S_ItemInfo` NewItemInfo))
  (bind _local_currentelementinfo (`local.Local_CurrentElementInfo`))
  (bind ((`Id_26_B8349D294FC6345E116DB081DF9569FA` _id) (`Count_17_D19A6EBD41C242C28CC0F39910C423A9` _count_2)) (break `/Game/LMiTW/Blueprints/Structures/S_ItemInfo` (`local.Local_NewItemInfo`)))
  (set `local.Local_NewItemInfo` NewItemInfo)
  (if (!= _count _stacksize)
    (set `local.Local_Id` _id)
    (set `local.Local_Count` _count_2)
    (bind _success (`self.HaveItemByID` (`local.Local_Id`)))
    (if _success
      (for (_array_element _array_index) (`self.Items`)
        (set `local.Local_Index` _array_index)
        (if (> (`local.Local_Count`) 0)
          (set `local.Local_CurrentElementInfo` _array_element)
          (if (`self.ValidateStack` (`local.Local_CurrentElementInfo`) (`local.Local_Id`))
            (if (<= (`self.GetCountRemaining` (`local.Local_Count`) (`local.Local_CurrentElementInfo`)) 0)
              ;[1 1 1] No overflow
              (set `local.Local_Count` (`self.GetSummCount` (`local.Local_Count`) (`local.Local_CurrentElementInfo`)))
              (bind _structout (setmembers `/Game/LMiTW/Blueprints/Structures/S_ItemInfo` :`StructRef` (`local.Local_CurrentElementInfo`) :`Count` (`local.Local_Count`)))
              (`KismetArrayLibrary.Array_Set` (`self.Items`) (`local.Local_Index`) _structout)
              (return true)
              (else
                ;[1 1 1] Overflow  - fill current item stack and set remaining count
                (set `local.Local_Count` (`self.GetCountRemaining` (`local.Local_Count`) (`local.Local_CurrentElementInfo`)))
                (bind _structout_2 (setmembers `/Game/LMiTW/Blueprints/Structures/S_ItemInfo` :`StructRef` _local_currentelementinfo :`Count` (`.StackSize_22_A0B76A20497498BC51DB029EFCFB634F` (break `/Game/LMiTW/Blueprints/Structures/S_ItemInfo` _local_currentelementinfo))))
                (`KismetArrayLibrary.Array_Set` (`self.Items`) (`local.Local_Index`) _structout_2))))))
      (if (> (`local.Local_Count`) 0)
        ;[1 1 1] We have some count remaining - lets create a new item stack!
        (bind _structout_3 (setmembers `/Game/LMiTW/Blueprints/Structures/S_ItemInfo` :`StructRef` (`local.Local_NewItemInfo`) :`Count` (`local.Local_Count`)))
        (bind _success_2 (`self.AddItem` _structout_3))
        (return _success_2))
      (else
        ;[1 1 1] Player don't have this item, create new item stack
        (bind _success_3 (`self.AddItem` (`local.Local_NewItemInfo`)))
        (return _success_3)))
    (else
      ;[1 1 1] Already full stack - add new item stack
      (bind _success_4 (`self.AddItem` (`local.Local_NewItemInfo`)))
      (return _success_4))))

(fn `DropItem`
  (params (Index :type Integer))
  (returns (Success :type Boolean))
  (locals (Local_Index :type Integer))
  (set `local.Local_Index` Index)
  (if (`self.IsValidIndex` (`local.Local_Index`))
    (bind _successs (`self.SpawnDroppedItem` (`self.GetItem` (`local.Local_Index`))))
    (if _successs
      (bind _success (`self.TryRemoveItem` (`local.Local_Index`)))
      (return _success)
      (else
        (return false)))
    (else
      (return false))))

(fn `GetCountRemaining`
  (params (AdditionalCount :type Integer) (Item :type "/Game/LMiTW/Blueprints/Structures/S_ItemInfo Structure (by ref)"))
  (returns (ReturnValue :type Integer))
  (return (- (`self.GetSummCount` AdditionalCount Item) (`.StackSize_22_A0B76A20497498BC51DB029EFCFB634F` (break `/Game/LMiTW/Blueprints/Structures/S_ItemInfo` Item)))))

(fn `GetItem`
  (params (SlotIndex :type Integer))
  (returns (ItemInfo :type "/Game/LMiTW/Blueprints/Structures/S_ItemInfo Structure"))
  (locals (Local_Index :type Integer))
  (set `local.Local_Index` SlotIndex)
  (if (`self.IsValidIndex` (`local.Local_Index`))
    (return (`|GetArrayItem` (`self.Items`) (`local.Local_Index`)))
    (else
      (return))))

(fn `GetSummCount`
  (params (AdditionalCount :type Integer) (S_ItemInfo :type "/Game/LMiTW/Blueprints/Structures/S_ItemInfo Structure (by ref)"))
  (returns (Summ :type Integer))
  (return (+ AdditionalCount (`.Count_17_D19A6EBD41C242C28CC0F39910C423A9` (break `/Game/LMiTW/Blueprints/Structures/S_ItemInfo` S_ItemInfo)))))

(fn `HaveEmptySlots`
  (returns (Success :type Boolean))
  (return (< (`self.UsedSlots`) (`self.MaxSlots`))))

(fn `HaveItemByID`
  (params (Id :type Integer))
  (returns (Success :type Boolean))
  (locals (Local_Id :type Integer) (Local_ItemIndex :type Integer :default -1))
  (set `local.Local_Id` Id)
  (for (_array_element _array_index) (`self.Items`)
    (if (== (`local.Local_Id`) (`.Id_26_B8349D294FC6345E116DB081DF9569FA` (break `/Game/LMiTW/Blueprints/Structures/S_ItemInfo` _array_element)))
      (set `local.Local_ItemIndex` _array_index)
      (break)))
  (if (!= (`local.Local_ItemIndex`) -1)
    (return true)
    (else
      (return false))))

(fn `Init`
  (`self.UpdateStorageSize`)
  (`self.UpdateInventory`))

(fn `IsValidIndex`
  (params (Index :type Integer))
  (returns (IsValid :type Boolean))
  (if (<= Index (- (`KismetArrayLibrary.Array_Length` (`self.Items`)) 1))
    (return true)
    (else
      (return false))))

(fn `RemoveItem`
  (params (ItemIndex :type Integer))
  (returns (Success :type Boolean))
  (locals (Local_Index :type Integer))
  (set `local.Local_Index` ItemIndex)
  (if (`self.IsValidIndex` (`local.Local_Index`))
    (`KismetArrayLibrary.Array_Set` (`self.Items`) (`local.Local_Index`))
    (`/Engine/EditorBlueprintResources/StandardMacros.DecrementInt` (`self.UsedSlots`)
      (:`  `
        (return true)))
    (else
      (return false))))

(fn `SearchFreeSlot`
  (returns (Success :type Boolean) (SlotIndex :type Integer))
  (locals (Local_Success :type Boolean) (Local_Index :type Integer :default -1))
  (for (_array_element _array_index) (`self.Items`)
    (if (== (`.Id_26_B8349D294FC6345E116DB081DF9569FA` (break `/Game/LMiTW/Blueprints/Structures/S_ItemInfo` _array_element)) (`self.NO_ITEM_ID`))
      (set `local.Local_Success` true)
      (set `local.Local_Index` _array_index)
      (break)))
  (return (`local.Local_Success`) (`local.Local_Index`)))

(fn `SpawnDroppedItem`
  (params (ItemInfo :type "/Game/LMiTW/Blueprints/Structures/S_ItemInfo Structure"))
  (returns (Successs :type Boolean))
  (bind ((`Id_26_B8349D294FC6345E116DB081DF9569FA` _id) (`Count_17_D19A6EBD41C242C28CC0F39910C423A9` _count)) (break `/Game/LMiTW/Blueprints/Structures/S_ItemInfo` ItemInfo))
  (bind _returnvalue (`|SpawnActorFromClass` "/Game/LMiTW/Blueprints/GameplayActors/Pickup/BP_DefaultPickup.BP_DefaultPickup_C" (`KismetMathLibrary.MakeTransform` (+ (`Actor.K2_GetActorLocation` (`self.GetOwner`)) (200.0 0.0 -100.0))) "AlwaysSpawn" "OverrideRootScale" null _id _count (struct) null))
  (`/Engine/EditorBlueprintResources/StandardMacros.IsValid` _returnvalue
    (:`Is Valid`
      (return true))
    (:`Is Not Valid`
      (return false))))

(fn `SwapItems`
  (params (FirstIndex :type Integer) (SecondIndex :type Integer))
  (returns (Success :type Boolean))
  (`KismetArrayLibrary.Array_Swap` (`self.Items`) FirstIndex SecondIndex)
  (`self.UpdateInventory`)
  (return true))

(fn `TryAddItem`
  (params (ItemInfo :type "/Game/LMiTW/Blueprints/Structures/S_ItemInfo Structure"))
  (returns (Success :type Boolean))
  (if (`.Stackable_14_31B9986A4FF3E6346627B2966AB841C5` (break `/Game/LMiTW/Blueprints/Structures/S_ItemInfo` ItemInfo))
    (bind _success (`self.AddStackableItem` ItemInfo))
    (if _success
      _
      (else
        (return false)))
    (else
      (bind _success_2 (`self.AddItem` ItemInfo))
      (if _success_2
        _
        (else
          (return false)))))
  (`self.UpdateInventory`)
  (return true))

(fn `TryDropItem`
  (params (SlotIndex :type Integer))
  (returns (Success :type Boolean))
  (bind _success (`self.DropItem` SlotIndex))
  (return _success))

(fn `TryRemoveItem`
  (params (ItemIndex :type Integer))
  (returns (Success :type Boolean))
  (bind _success (`self.RemoveItem` ItemIndex))
  (if _success
    (`self.UpdateInventory`)
    (return true)
    (else
      (return false))))

(fn `TrySplitItems`
  (params (`Slot index` :type Integer) (NewStackValue :type Integer))
  (returns (Success :type Boolean))
  (locals (Local_CountInNewStack :type Integer :default 0) (Local_Index :type Integer) (Local_CountInOldStack :type Integer) (Local_CurrentCount :type Integer) (Local_NewStackValue :type Integer))
  (set `local.Local_Index` `Slot index`)
  (set `local.Local_CountInNewStack` NewStackValue)
  (if (`self.ValidateSplitOperation` (`local.Local_Index`) (`local.Local_CountInNewStack`))
    (set `local.Local_CurrentCount` (`.Count_17_D19A6EBD41C242C28CC0F39910C423A9` (break `/Game/LMiTW/Blueprints/Structures/S_ItemInfo` (`self.GetItem` (`local.Local_Index`)))))
    (bind _output_get (set `local.Local_CountInOldStack` (- (`local.Local_CurrentCount`) (`local.Local_CountInNewStack`))))
    (setmembers `/Game/LMiTW/Blueprints/Structures/S_ItemInfo` :`StructRef` (`|GetArrayItem` (`self.Items`) (`local.Local_Index`)) :`Count` _output_get) ; Count in the old stack
    (bind _structout (setmembers `/Game/LMiTW/Blueprints/Structures/S_ItemInfo` :`StructRef` (`self.GetItem` (`local.Local_Index`)) :`Count` (`local.Local_CountInNewStack`))) ; Count in the new stack
    (bind _success (`self.AddItem` _structout))
    (`self.UpdateInventory`)
    (return _success)
    (else
      (return false) ; Not valid operation! Returning.
    )))

(fn `TryUseItem`
  (params (SlotIndex :type Integer))
  (returns (Success :type Boolean))
  (locals (Local_SlotIndex :type Integer))
  (set `local.Local_SlotIndex` SlotIndex)
  (if (`self.IsValidIndex` (`local.Local_SlotIndex`))
    (`self.ItemTypeIsEqual` (`local.Local_SlotIndex`) "NewEnumerator1" ; We can't use item if it is not valid or not usable!
      (:`true`
        ;[0.5833 1 0.6396] Valid item
        (bind _success (`self.UseItem` (`local.Local_SlotIndex`)))
        (if _success
          (if (`.Consumable_28_8AF25E9746A40113FB9A53A16848E951` (break `/Game/LMiTW/Blueprints/Structures/S_ItemInfo` (`self.GetItem` (`local.Local_SlotIndex`))))
            (bind _success_2 (`self.TryRemoveItem` (`local.Local_SlotIndex`)))
            (return _success_2)
            (else
              (return true)))
          (else
            (return false))))
      (:`false`
        _)))
  ;[0.5833 1 0.6396] Not valid item
  (return false))

(fn `UpdateInventory`
  (`self.OnInventoryUpdated` (`self.Items`)))

(fn `UpdateStorageSize`
  (`KismetArrayLibrary.Array_Resize` (`self.Items`) (`self.MaxSlots`)))

(fn `UseItem`
  (params (SlotIndex :type Integer))
  (returns (Success :type Boolean))
  (locals (LocalIndex :type Integer))
  (set `local.LocalIndex` SlotIndex)
  (`|SpawnActorFromClass` (`.UsableClass_31_35745ADD4A3F8111EB16AD8C5E4F04B4` (break `/Game/LMiTW/Blueprints/Structures/S_ItemInfo` (`self.GetItem` (`local.LocalIndex`)))) (`/Game/LMiTW/Blueprints/FunctionLibrary/LMFunctionLibrary.GetZeroSpawnTransform`) "AlwaysSpawn" "OverrideRootScale" null (`self.GetOwner`) null)
  (return true))

(fn `ValidateSplitOperation`
  (params (LocalIndex :type Integer) (Count :type Integer))
  (returns (ReturnValue :type Boolean))
  (locals (LocalItemIndex :type Integer))
  (set `local.LocalItemIndex` LocalIndex)
  (return (and (`self.IsValidIndex` (`local.LocalItemIndex`)) (`self.HaveEmptySlots`) (> (`.Count_17_D19A6EBD41C242C28CC0F39910C423A9` (break `/Game/LMiTW/Blueprints/Structures/S_ItemInfo` (`self.GetItem` (`local.LocalItemIndex`)))) 1) (!= (`.Count_17_D19A6EBD41C242C28CC0F39910C423A9` (break `/Game/LMiTW/Blueprints/Structures/S_ItemInfo` (`self.GetItem` (`local.LocalItemIndex`)))) Count))))

(fn `ValidateStack`
  (params (S_ItemInfo :type "/Game/LMiTW/Blueprints/Structures/S_ItemInfo Structure (by ref)") (Id :type Integer))
  (returns (IsValid :type Boolean))
  (bind ((`Id_26_B8349D294FC6345E116DB081DF9569FA` _id) (`Count_17_D19A6EBD41C242C28CC0F39910C423A9` _count) (`StackSize_22_A0B76A20497498BC51DB029EFCFB634F` _stacksize)) (break `/Game/LMiTW/Blueprints/Structures/S_ItemInfo` S_ItemInfo))
  (bind _returnvalue (and (!= _count _stacksize) (== Id _id)))
  (if _returnvalue
    (return _returnvalue)))