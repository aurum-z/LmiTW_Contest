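; Player component that tracks an oxygen supply, starting at maximum on BeginPlay.
; Activation starts a looping timer that drains oxygen by a set rate at a set interval, and deactivation clears it.
; Each change is clamped, broadcast through a change dispatcher and printed as debug text, with a separate event fired when oxygen reaches zero.
; Activation and deactivation also broadcast a status change.
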(event `self.ReceiveBeginPlay`
  ;[1 1 1] Init
  (`self.Init`))

(fn `ActivateOxygenComponent`
  (bind _returnvalue (`KismetSystemLibrary.K2_SetTimer` self "DrainOxygen" (`self.OxygenDrainingInterval`) true))
  (set `self.OxygenTimerHandle` _returnvalue)
  (`self.OnOxygenComponentStatusChanged` true))

(fn `ChangeOxygenCurrentCount`
  (params (Value :type "Float (double-precision)"))
  (set `self.CurrentOxygenCount` (`KismetMathLibrary.FClamp` (+ (`self.CurrentOxygenCount`) Value) 0.0 (`self.MaxOxygenCount`)))
  (`self.UpdateOxygenValue`)
  (if (<= (`self.CurrentOxygenCount`) 0.0)
    (`self.OxygenIsOut`)))

(fn `DeactivateOxygenComponent`
  (`KismetSystemLibrary.K2_ClearAndInvalidateTimerHandle` (`self.OxygenTimerHandle`))
  (`self.OnOxygenComponentStatusChanged` false))

(fn `DrainOxygen`
  (`self.ChangeOxygenCurrentCount` (* (`self.OxygenDrainingRate`) -1.0)))

(fn `Init`
  (set `self.PlayerCharacter` (`self.GetOwner`))
  (set `self.CurrentOxygenCount` (`self.MaxOxygenCount`)))

(fn `OxygenIsOut`
  (`self.OnOxygenIsOut`))

(fn `UpdateOxygenValue`
  (`self.OnOxygenCountChanged` (`self.CurrentOxygenCount`) (`self.MaxOxygenCount`))
  (`KismetSystemLibrary.PrintString` (`KismetStringLibrary.Concat_StrStr` "Oxygen: " (`KismetStringLibrary.Conv_DoubleToString` (`self.CurrentOxygenCount`)))))