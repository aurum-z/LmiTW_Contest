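; Player interaction component that finds what the first-person camera looks at and routes interact input to it.
; A looping timer line-traces for BPI_Interactable targets, updating the cursor tooltip and toggling the PDA menu for door panels and access modules.
; Left mouse uses the cutting tool or shows PDA parameters.
; Other keys send InteractMessage or run timed, hold-to-complete take/drop of two-handed items with a progress bar, cancelled on release.
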(event `self.ReceiveTick`
  (params (DeltaSeconds :type "Float (single-precision)"))
  ;[1 1 1] Debug
  (`KismetSystemLibrary.PrintString` (`KismetStringLibrary.Concat_StrStr` "LineTraceInteract: " (`KismetSystemLibrary.GetDisplayName` (`self.LinetraceInteractionTarget`))) true true (struct :`G` 0.66 :`B` 1.0 :`A` 1.0) 0.0)
  (`KismetSystemLibrary.PrintString` (`KismetStringLibrary.Concat_StrStr` "InteractTarget: " (`KismetSystemLibrary.GetDisplayName` (`self.InteractionTarget`))) true true (struct :`G` 0.66 :`B` 1.0 :`A` 1.0) 0.0))

(event `self.ReceiveBeginPlay`
  ;[1 1 1] Init
  (`self.InitOwner`)
  (`self.StartTracing`))

(event `Event On Linetrace Target UI Changed`
  (`self.ShowCursorTooltip`))

(event `Event Pressed Interact`
  (params (InputKey :type "Key Structure" :default "None"))
  (bind _debug2_handeditem (`self.Debug2_HandedItem`))
  (bind _debug2_handeditem_2 (`self.Debug2_HandedItem`))
  (bind _debug2_handeditem_3 (`self.Debug2_HandedItem`))
  (bind _debug2_handeditem_4 (`self.Debug2_HandedItem`))
  (bind _debug2_handeditem_5 (`self.Debug2_HandedItem`))
  ;[1 1 1] Calls when player pressed the key for interaction
  (if (== InputKey "LeftMouseButton")
    (`self.WeldInstrumentLogic`
      (:`TryUseCuttingInstrument`
        (message `/Game/LMiTW/Blueprints/Interface/BPI_Interactable.Interact` (`self.InteractionTarget`) (`self.OwnerPlayerCharacter`) InputKey :!label _label))
      (:`ShowParametersPDA`
        (`/Game/LMiTW/Blueprints/Character/BP_LMPlayerCharacter.Event Show Character Parameters in PDA` (`self.OwnerPlayerCharacter`))))
    (else
      (`self.TwoHandedItemLogic` InputKey
        (:`TryTake2 HandedItem`
          ;;[1 1 1 0.5] debug
          (`KismetSystemLibrary.PrintString` "Try take 2 handed item" _debug2_handeditem_5 _debug2_handeditem_5 (`self.DebugColor`) (`self.MessageDebugDuration`))
          (`self.StartProcessOfTakingTwoHandedItem`))
        (:`CharacterCantInteractWith2 HandedItem`
          (`KismetSystemLibrary.PrintString` "Character cant interact with 2 handed item" _debug2_handeditem_2 _debug2_handeditem_2 (`self.DebugColor`) (`self.MessageDebugDuration`)))
        (:`InteractionTargetIsNot2 HandedItem`
          (`KismetSystemLibrary.PrintString` "Interaction target Is not 2 handed Item. Continue interact to item" _debug2_handeditem_3 _debug2_handeditem_3 (`self.DebugColor`) (`self.MessageDebugDuration`))
          (goto _label))
        (:`HaveNo2 HandedItem`
          (`KismetSystemLibrary.PrintString` "Character have no 2 handed item. Continue interact to item" _debug2_handeditem _debug2_handeditem (`self.DebugColor`) (`self.MessageDebugDuration`))
          (goto _label))
        (:`TryDrop2 HandedItem`
          (`KismetSystemLibrary.PrintString` "Try drop 2 handed item" _debug2_handeditem_4 _debug2_handeditem_4 (`self.DebugColor`) (`self.MessageDebugDuration`))
          (`self.StartProcessOfDroppingTwoHandedItem`)
          ;;[1 0 0] delete this sheeeeet
          (`self.ShowCursorTooltip`))))))

(event `Event Interact With Two Handed Item`
  (params (ActorWithWichToInteract :type "Actor Object Reference"))
  ;[1 1 1] Calls when player pressed the key for interaction
  ;;[1 1 1] Drop / Take 2 handed item. Flip flop system
  (message `/Game/LMiTW/Blueprints/Interface/BPI_Interactable.Interact` ActorWithWichToInteract (`self.OwnerPlayerCharacter`) "F"))

(event `Event Released Interact`
  (params (InputKey :type "Key Structure" :default "None"))
  ;[1 1 1] Calls when player released the key of interaction
  (if (not (== InputKey "LeftMouseButton"))
    (`self.TrySkipProcessOfTakingTwoHandedItemIfCharacterHasNotIt`)))

(fn `AddProgressWithTwoHandedItem`
  (bind _currentinteractitemprogresspercent (`self.CurrentInteractItemProgressPercent`))
  (switch `/Game/LMiTW/Blueprints/Enums/Items/E_InteractionComponentItemStatus` (`self.InteractionComponentStatus`)
    (:`NewEnumerator1`
      (set `self.CurrentInteractItemProgressPercent` (+ (`self.CurrentInteractItemProgressPercent`) (/ (`self.InteractProgressAddPecentPerCall`) (`self.CurrentInteractItemProcessTakeTime`)))))
    (:`NewEnumerator2`
      (set `self.CurrentInteractItemProgressPercent` (+ (`self.CurrentInteractItemProgressPercent`) (/ (`self.InteractProgressAddPecentPerCall`) (`self.CurrentInteractItemProcessDropTime`))))))
  (`/Game/LMiTW/HUD/GameOverlay/WBP_GameOverlay.Update Progress Bar Of Long Process` (`/Game/LMiTW/Blueprints/FunctionLibrary/LMFunctionLibrary.GetGameOverlay`) _currentinteractitemprogresspercent)
  (if (>= _currentinteractitemprogresspercent 100.0)
    (`self.EndProcessWithTwoHandedItem` false)))

(fn `CanCharacterTakeTwoHandedItemByMovementMode`
  (returns (`Can?` :type Boolean))
  (bind _ownerplayercharacter (`self.OwnerPlayerCharacter`))
  (bind _returnvalue (`Actor.GetComponentByClass` _ownerplayercharacter "/Game/LMiTW/Blueprints/Components/BP_PlayerControlMovementComponent.BP_PlayerControlMovementComponent_C"))
  (`/Engine/EditorBlueprintResources/StandardMacros.IsValid` _returnvalue
    (:`Is Valid`
      (bind (_cantake _successwork_) (`/Game/LMiTW/Blueprints/Components/BP_PlayerControlMovementComponent.CanCharacterTakeTwoHandedItem` _returnvalue (`GameplayStatics.GetObjectClass` _ownerplayercharacter)))
      (if (and _cantake _successwork_)
        (return true)
        (else
          (return false))))
    (:`Is Not Valid`
      (return false))))

(fn `ClearTarget`
  (bind _linetraceinteractiontarget (`self.LinetraceInteractionTarget`)
    (:`then`
      (if (`self.IsTraceDebugMode`)
        (`KismetSystemLibrary.PrintString` "ClearTarget()" true true (struct :`R` 0.324843 :`G` 1.0 :`B` 0.416074 :`A` 1.0))))
    (:`else`
      _))
  (`self.HideCursorTooltip`)
  (set `self.LinetraceInteractionTarget` null))

(fn `EndProcessWithTwoHandedItem`
  (params (SkipProcess :type Boolean))
  (bind _interactioncomponentstatus (`self.InteractionComponentStatus`))
  (set `self.CurrentInteractItemProgressPercent` 0.0)
  (`/Game/LMiTW/HUD/GameOverlay/WBP_GameOverlay.Update Progress Bar Of Long Process` (`/Game/LMiTW/Blueprints/FunctionLibrary/LMFunctionLibrary.GetGameOverlay`) 0.0)
  (`KismetSystemLibrary.K2_ClearAndInvalidateTimerHandle` (`self.TimerAddInteractProgress`))
  (if SkipProcess
    (switch `/Game/LMiTW/Blueprints/Enums/Items/E_InteractionComponentItemStatus` _interactioncomponentstatus
      (:`NewEnumerator1`
        (set `self.InteractionComponentStatus` "NewEnumerator0")
        (set `self.ProcessActor` null)
        ;[1 1 1 0.5] for bug, when player 1st time didn`t push full progress bar and then press F when look in sky
        (set `self.InteractionTarget` null))
      (:`NewEnumerator2`
        (set `self.InteractionComponentStatus` "NewEnumerator3")))
    (else
      ;[1 1 1] When proccess of take/drop done
      (switch `/Game/LMiTW/Blueprints/Enums/Items/E_InteractionComponentItemStatus` _interactioncomponentstatus
        (:`NewEnumerator1`
          (`self.Event Interact With Two Handed Item` (`self.InteractionTarget`))
          (set `self.InteractionComponentStatus` "NewEnumerator3"))
        (:`NewEnumerator2`
          (bind (_haveitem_ _iteminfo _actor) (`/Game/LMiTW/Blueprints/Character/BP_LMPlayerCharacter.GetTwoHandedItem` (`self.OwnerPlayerCharacter`)))
          (`self.Event Interact With Two Handed Item` _actor)
          (set `self.InteractionTarget` (`self.LinetraceInteractionTarget`))
          (set `self.InteractionComponentStatus` "NewEnumerator0")
          (set `self.ProcessActor` null)
          (`self.ShowCursorTooltip`))))))

(fn `GetInteractionTarget`
  (returns (InteractionTarget :type "Actor Object Reference"))
  (return (`self.InteractionTarget`)))

(fn `GetTraceParams`
  (returns (Start :type "Vector Structure") (End :type "Vector Structure"))
  (bind _camerafirstperson (`/Game/LMiTW/Blueprints/Character/BP_LMPlayerCharacter.CameraFirstPerson` (`self.OwnerPlayerCharacter`)))
  (bind _returnvalue (`SceneComponent.K2_GetComponentLocation` _camerafirstperson))
  (return _returnvalue (+ _returnvalue (* (`SceneComponent.GetForwardVector` _camerafirstperson) (`self.TraceDistance`)))))

(fn `HaveInteractionText`
  (params (S_InteractionInfo :type "/Game/LMiTW/Blueprints/Structures/S_InteractionInfo Structure (by ref)"))
  (returns (ReturnValue :type Boolean))
  (return (`KismetTextLibrary.NotEqual_TextText` (`.NameOfObject_13_2CA896B84EC61FBC1CBB7C9044E1313A` (break `/Game/LMiTW/Blueprints/Structures/S_InteractionInfo` S_InteractionInfo)) "")))

(fn `HideCursorTooltip`
  (`/Game/LMiTW/HUD/GameOverlay/WBP_GameOverlay.HideCursorTooltip` (`/Game/LMiTW/Blueprints/FunctionLibrary/LMFunctionLibrary.GetGameOverlay`)))

(fn `InitOwner`
  (bind _asbp_lmplayer_character (cast `/Game/LMiTW/Blueprints/Character/BP_LMPlayerCharacter` (`self.GetOwner`)))
  (set `self.OwnerPlayerCharacter` _asbp_lmplayer_character))

(fn `SetTarget`
  (params (NewTarget :type "Actor Object Reference"))
  (bind _output_get (set `self.LinetraceInteractionTarget` NewTarget))
  (switch `/Game/LMiTW/Blueprints/Enums/Items/E_InteractionComponentItemStatus` (`self.InteractionComponentStatus`)
    (:`NewEnumerator0`
      (set `self.InteractionTarget` _output_get))
    (:`NewEnumerator3`
      (bind _asbp_master_switcher (cast `/Game/LMiTW/Blueprints/GameplayActors/Switcher/BP_MasterSwitcher` _output_get)
        (:`then`
          (set `self.InteractionTarget` _asbp_master_switcher))
        (:`CastFailed`
          (set `self.InteractionTarget` (`self.ProcessActor`))))))
  (`self.ShowCursorTooltip`)
  (if (`self.IsTraceDebugMode`)
    (`KismetSystemLibrary.PrintString` "SetTarget()" true true (struct :`R` 0.324843 :`G` 1.0 :`B` 0.416074 :`A` 1.0))))

(fn `ShowCursorTooltip`
  (bind _info (message `/Game/LMiTW/Blueprints/Interface/BPI_Interactable.GetInteractInfo` (`self.InteractionTarget`)))
  (if (`self.HaveInteractionText` _info)
    (`/Game/LMiTW/HUD/GameOverlay/WBP_GameOverlay.ShowCursorTooltip` (`/Game/LMiTW/Blueprints/FunctionLibrary/LMFunctionLibrary.GetGameOverlay`) _info)))

(fn `StartProcessOfDroppingTwoHandedItem`
  (set `self.InteractionComponentStatus` "NewEnumerator2")
  (bind _returnvalue (`KismetSystemLibrary.K2_SetTimer` null "AddProgressWithTwoHandedItem" 0.01 true))
  (set `self.TimerAddInteractProgress` _returnvalue))

(fn `StartProcessOfTakingTwoHandedItem`
  (set `self.InteractionComponentStatus` "NewEnumerator1")
  (bind _returnvalue (`KismetSystemLibrary.K2_SetTimer` null "AddProgressWithTwoHandedItem" 0.01 true))
  (set `self.TimerAddInteractProgress` _returnvalue)
  (bind _output_get (set `self.InteractionTarget` (`self.LinetraceInteractionTarget`)))
  (bind _output_get_2 (set `self.ProcessActor` _output_get))
  ;[1 1 1] Set max drop and take time for current item
  (bind _info (message `/Game/LMiTW/Blueprints/Interface/BPI_Interactable.GetInteractInfo` _output_get_2))
  (bind (_nameofobject _playerinteractionaction _iteminteractionaction _keyforinteractaction _longprocessinteractactor_ _longprocesstaketime _longprocessdroptime) (break `/Game/LMiTW/Blueprints/Structures/S_InteractionInfo` _info))
  (set `self.CurrentInteractItemProcessTakeTime` _longprocesstaketime)
  (set `self.CurrentInteractItemProcessDropTime` _longprocessdroptime))

(fn `StartTracing`
  (bind _returnvalue (`KismetSystemLibrary.K2_SetTimer` null "TraceForInteract" (`self.TraceInterval`) true))
  (set `self.InteractionTimer` _returnvalue))

(fn `StopTracing`
  (`KismetSystemLibrary.K2_ClearAndInvalidateTimerHandle` (`self.InteractionTimer`))
  (`self.ClearTarget`))

(fn `TraceForInteract`
  (locals (L_PotentialTarget :type "Actor Object Reference"))
  (bind (_start _end) (`self.GetTraceParams`))
  (bind _l_potentialtarget (`local.L_PotentialTarget`))
  (bind _processactor (`self.ProcessActor`))
  (bind _l_potentialtarget_2 (`local.L_PotentialTarget`))
  (bind _l_potentialtarget_3 (`local.L_PotentialTarget`))
  (bind (_outhit _returnvalue) (`KismetSystemLibrary.LineTraceSingle` _start _end "TraceTypeQuery3" false (`|MakeArray` (`ChildActorComponent.ChildActor` (`/Game/LMiTW/Blueprints/Character/BP_LMPlayerCharacter.BP_PlayerPDA` (`self.OwnerPlayerCharacter`)))) (select `bool` (`self.IsTraceDebugMode`) :`true` "ForDuration" :!type "EDrawDebugTrace Enum") true (struct :`R` 1.0 :`G` 0.94821 :`B` 0.113053 :`A` 1.0) (struct :`G` 1.0 :`A` 1.0) (`self.DebugLineDuration`)))
  (if _returnvalue
    ;[1 1 1] If different actors
    (bind _output_get (set `local.L_PotentialTarget` (`.HitActor` (`GameplayStatics.BreakHitResult` _outhit))))
    (if (!= _output_get (`self.LinetraceInteractionTarget`))
      (bind _success (`self.ValidateTarget` (`local.L_PotentialTarget`)))
      (if (or _success (`KismetSystemLibrary.IsValid` (`self.ProcessActor`)))
        (`self.SetTarget` (`local.L_PotentialTarget`))
        ;[1 1 1] Comment
        (cast `/Game/LMiTW/Blueprints/GameplayActors/Switcher/BP_DoorControlPanel` _l_potentialtarget_3
          (:`then`
            _)
          (:`CastFailed`
            (cast `/Game/LMiTW/Blueprints/GameplayActors/Pickup/BP_PDAAccessModule` _l_potentialtarget_3)))
        (if (not (`/Game/LMiTW/Blueprints/Character/BP_LMPlayerCharacter.CharacterShowPDA?` (`self.OwnerPlayerCharacter`)))
          (`/Game/LMiTW/Blueprints/Character/BP_LMPlayerCharacter.Event Show Interact Menu in PDA` (`self.OwnerPlayerCharacter`) false))
        (else
          (`self.ClearTarget`)
          (cast `/Game/LMiTW/Blueprints/GameplayActors/Switcher/BP_DoorControlPanel` _l_potentialtarget
            (:`then`
              _)
            (:`CastFailed`
              (cast `/Game/LMiTW/Blueprints/GameplayActors/Pickup/BP_PDAAccessModule` _l_potentialtarget)))
          (if (`/Game/LMiTW/Blueprints/Character/BP_LMPlayerCharacter.CharacterShowPDA?` (`self.OwnerPlayerCharacter`))
            (`/Game/LMiTW/Blueprints/Character/BP_LMPlayerCharacter.Event Show Interact Menu in PDA` (`self.OwnerPlayerCharacter`) false))))
      (else
        (`/Engine/EditorBlueprintResources/StandardMacros.IsValid` (`self.ProcessActor`)
          (:`Is Not Valid`
            ;[1 1 1] Comment
            (cast `/Game/LMiTW/Blueprints/GameplayActors/Switcher/BP_DoorControlPanel` _l_potentialtarget_2
              (:`then`
                _)
              (:`CastFailed`
                (cast `/Game/LMiTW/Blueprints/GameplayActors/Pickup/BP_PDAAccessModule` _l_potentialtarget_2)))
            (if (not (`/Game/LMiTW/Blueprints/Character/BP_LMPlayerCharacter.CharacterShowPDA?` (`self.OwnerPlayerCharacter`)))
              (`/Game/LMiTW/Blueprints/Character/BP_LMPlayerCharacter.Event Show Interact Menu in PDA` (`self.OwnerPlayerCharacter`) false))))))
    (else
      (`/Engine/EditorBlueprintResources/StandardMacros.IsValid` _processactor
        (:`Is Valid`
          (`self.SetTarget` _processactor))
        (:`Is Not Valid`
          (`self.ClearTarget`) ; Not hit - clearing target!
          ;[1 1 1] Comment
          (bind _bp_pda (`/Game/LMiTW/Blueprints/Character/BP_LMPlayerCharacter.GetPDA` (`self.OwnerPlayerCharacter`)))
          (bind _mainmenu (`/Game/LMiTW/Blueprints/GameplayActors/PDA/BP_PlayerPDA.GetCurrentMenuPDA` _bp_pda))
          (if (and (`|EnumEquality` _mainmenu "NewEnumerator1") (`/Game/LMiTW/Blueprints/Character/BP_LMPlayerCharacter.CharacterShowPDA?` (`self.OwnerPlayerCharacter`)))
            (`/Game/LMiTW/Blueprints/Character/BP_LMPlayerCharacter.Event Show Interact Menu in PDA` (`self.OwnerPlayerCharacter`) false)))))))

(fn `TrySkipProcessOfTakingTwoHandedItemIfCharacterHasNotIt`
  (`/Game/LMiTW/Blueprints/Character/BP_LMPlayerCharacter.GetTwoHandedItem` (`self.OwnerPlayerCharacter`))
  (`self.EndProcessWithTwoHandedItem` true))

(fn `ValidateTarget`
  (params (Target :type "Actor Object Reference"))
  (returns (Success :type Boolean))
  (if (`KismetSystemLibrary.DoesImplementInterface` Target "/Game/LMiTW/Blueprints/Interface/BPI_Interactable.BPI_Interactable_C")
    (return true)
    (else
      (return false))))