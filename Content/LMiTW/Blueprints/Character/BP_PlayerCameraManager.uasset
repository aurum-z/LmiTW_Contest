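; BP_PlayerCameraManager is a player camera manager that lets other code temporarily restrict or restore the camera's yaw and pitch view limits.
; Its construction script runs PreInit, which caches the default min and max view angles.
; SetCameraViewAnglesConstraint then either applies new limits or restores those cached defaults, independently for yaw and pitch via separate flags.
; The event graph holds only disabled placeholder events.
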(fn `PreInit`
  (`|ExecutionSequence`
    (:`then_0`
      ;[1 1 1] Save camera default rotation constraints
      (set `self.viewYawMinDefault` (`self.ViewYawMin`))
      (set `self.viewYawMaxDefault` (`self.ViewYawMax`))
      (set `self.viewPitchMinDefault` (`self.ViewPitchMin`))
      (set `self.viewPitchMaxDefault` (`self.ViewPitchMax`)))))

(fn `Set CameraViewAnglesConstraint`
  (params (NewYawMin :type "Float (double-precision)") (NewYawMax :type "Float (double-precision)") (`SetNewYaw?` :type Boolean) (NewPitchMin :type "Float (double-precision)") (NewPitchMax :type "Float (double-precision)") (`SetNewPitch?` :type Boolean))
  (`|ExecutionSequence`
    (:`then_0`
      (if `SetNewYaw?`
        (set `self.ViewYawMin` NewYawMin)
        (set `self.ViewYawMax` NewYawMax)
        (else
          ;[1 1 1] Set default Yaw
          (set `self.ViewYawMin` (`self.viewYawMinDefault`))
          (set `self.ViewYawMax` (`self.viewYawMaxDefault`)))))
    (:`then_1`
      (if `SetNewPitch?`
        (set `self.ViewPitchMin` NewPitchMin)
        (set `self.ViewPitchMax` NewPitchMax)
        (else
          ;[1 1 1] Set default Pitch
          (set `self.ViewPitchMin` (`self.viewPitchMinDefault`))
          (set `self.ViewPitchMax` (`self.viewPitchMaxDefault`)))))))

(fn `UserConstructionScript`
  (`self.PreInit`))