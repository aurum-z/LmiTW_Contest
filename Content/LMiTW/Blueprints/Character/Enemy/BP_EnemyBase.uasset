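; Base enemy character that exposes presets, start settings and mode, stage, patrol and attack commands, relaying to its AI controller through messages.
; Stage selects a movement preset from the AI preset, and mode picks the walk speed from it.
; Attacks play a random montage while a constructed logic object runs the ability, then notify the controller after a delay.
; It turns toward targets in Combat or Suspect, and traces surfaces for footstep audio.
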(event `self.ReceiveBeginPlay`
  (bind ((`StartStage_2_AEB004124BEDD3290AA323BFB5DEFCBC` _startstage) (`AIMovementForStages_16_F9D8130046A605957E9D899D85D7B7E1` _aimovementforstages)) (break `/Game/LMiTW/Blueprints/Structures/SAI_Preset` (`/Game/LMiTW/Data/AIPresets/BP_AIPresetBase.Preset` (`self.Preset`))))
  (`self.UpdateMovement` (`BlueprintMapLibrary.Map_Find` _aimovementforstages _startstage)))

(event `StartAttack`
  (params (Ability :type "/Game/LMiTW/Data/Abilities/Base/BP_Ability Object Reference"))
  (set `self.IsAttacking` true)
  (`|PlayMontage` (`self.Mesh`) (`/Game/LMiTW/Data/Abilities/Base/BP_Ability.GetRandomMontage` Ability)
    (:`then`
      (`self.ProcessAbility` Ability))
    (:`OnCompleted`
      (`self.EndAttack` :!label _label))
    (:`OnInterrupted`
      (goto _label))))

(event `EndAttack`
  (`KismetSystemLibrary.Delay` (`.IntervalBetweenAttacks_26_2ABDAA244BC9A3EB166CA4BF61F5A9D4` (break `/Game/LMiTW/Blueprints/Structures/SAI_Preset` (`/Game/LMiTW/Data/AIPresets/BP_AIPresetBase.Preset` (`self.Preset`)))))
  (set `self.IsAttacking` false)
  (message `/Game/LMiTW/Blueprints/Interface/BPI_AIController.AttackEnd` (`self.GetController`)))

(event `self.ReceiveTick`
  (params (DeltaSeconds :type "Float (single-precision)"))
  (`self.LookAtTarget` DeltaSeconds))

(event `/Game/LMiTW/Blueprints/Interface/BPI_CharSoundInterface.FootstepNotify`
  (bind _returnvalue (`self.K2_GetActorLocation`))
  (bind _footsteps (`self.FootSteps`))
  (bind _outhit (`KismetSystemLibrary.LineTraceSingle` :`Start` _returnvalue :`End` (+ _returnvalue (* (`KismetMathLibrary.Cross_VectorVector` (`self.GetActorRightVector`) (`self.GetActorForwardVector`)) 200.0)) :`TraceChannel` "TraceTypeQuery1" :`DrawDebugType` "Persistent"))
  (bind (_bblockinghit _binitialoverlap _time _distance _location _impactpoint _normal _impactnormal _physmat) (`GameplayStatics.BreakHitResult` _outhit))
  (if _bblockinghit
    (`AudioComponent.Play` _footsteps 0.0)
    (`AudioComponent.SetBoolParameter` _footsteps "step_play" true)
    (`AudioComponent.SetBoolParameter` _footsteps "rattle_play" true)
    (`AudioComponent.SetBoolParameter` _footsteps "IsMale" true)
    (`AudioComponent.SetFloatParameter` _footsteps "step_volume" 0.1)
    (`AudioComponent.SetFloatParameter` _footsteps "rattle_volume" 1.0)
    (`AudioComponent.SetIntParameter` _footsteps "floor" (`KismetArrayLibrary.Array_Find` (`self.Surfaces`) _physmat))))

(fn `GetAcceptableDistance`
  (returns (Distance :type "Float (double-precision)"))
  (return (`self.AcceptableDistanceToPlayer`)))

(fn `GetAIPreset`
  (returns (Preset :type "/Game/LMiTW/Blueprints/Structures/SAI_Preset Structure"))
  (return (`/Game/LMiTW/Data/AIPresets/BP_AIPresetBase.Preset` (`self.Preset`))))

(fn `GetInspectingRadius`
  (returns (Radius :type "Float (double-precision)"))
  (return (`self.GetMaxInspectingRadius`)))

(fn `GetMaxInspectingRadius`
  (returns (Radius :type "Float (double-precision)"))
  (return (`self.InspectingMaxRadius`)))

(fn `GetStartMode`
  (returns (Mode :type "/Game/LMiTW/Blueprints/Enums/E_AIMode Enum"))
  (return (`self.StartAIMode`)))

(fn `GetStartSensesSetup`
  (returns (Setup :type "/Game/LMiTW/Blueprints/Structures/S_AISensesSetup Structure"))
  (return (`self.StartSensesSetup`)))

(fn `GetStartStage`
  (returns (Stage :type "/Game/LMiTW/Blueprints/Enums/E_AIStages Enum"))
  (return (`self.StartAIStage`)))

(fn `LookAtTarget`
  (params (DeltaTime :type "Float (double-precision)"))
  (bind _returnvalue (`self.K2_GetActorRotation`))
  (bind _currentaimode (`self.CurrentAIMode`))
  (if (and (not (`self.IsAttacking`)) (or (`|EnumEquality` _currentaimode "NewEnumerator2") (`|EnumEquality` _currentaimode "NewEnumerator5")))
    (bind _target (message `/Game/LMiTW/Blueprints/Interface/BPI_AIController.GetTarget` (`self.GetController`)))
    (`self.K2_SetActorRotation` (`KismetMathLibrary.MakeRotator` (.roll _returnvalue) (.pitch (`KismetMathLibrary.RInterpTo` _returnvalue (`KismetMathLibrary.FindLookAtRotation` (`self.K2_GetActorLocation`) (`self.K2_GetActorLocation` _target)) DeltaTime 20.0)) (.yaw (`KismetMathLibrary.RInterpTo` _returnvalue (`KismetMathLibrary.FindLookAtRotation` (`self.K2_GetActorLocation`) (`self.K2_GetActorLocation` _target)) DeltaTime 20.0))))))

(fn `ProcessAbility`
  (params (Ability :type "/Game/LMiTW/Data/Abilities/Base/BP_Ability Object Reference"))
  (bind _target (message `/Game/LMiTW/Blueprints/Interface/BPI_AIController.GetTarget` (`self.GetController`)))
  (bind _returnvalue (`|GenericCreateObject` (`/Game/LMiTW/Data/Abilities/Base/BP_Ability.GetLogic` Ability) self self _target Ability))
  (`/Game/LMiTW/Blueprints/AbilityLogic/Base/BP_AbilityBaseLogic.StartAbility` _returnvalue))

(fn `ProcessAttack`
  (params (Ability :type "/Game/LMiTW/Data/Abilities/Base/BP_Ability Object Reference"))
  (returns (Success :type Boolean))
  (`self.StartAttack` Ability)
  (return true))

(fn `SetCurrentMode`
  (params (Mode :type "/Game/LMiTW/Blueprints/Enums/E_AIMode Enum" :default "NewEnumerator0"))
  (set `self.CurrentAIMode` Mode)
  (`self.UpdateMovementSpeedByMode`))

(fn `SetCustomPatrolPath`
  (params (PathPoints :type "Array of Vector Structure (by ref)"))
  (message `/Game/LMiTW/Blueprints/Interface/BPI_AIController.NewCustomPatrolPath` (`self.GetController`) PathPoints))

(fn `SetMode`
  (params (NewMode :type "/Game/LMiTW/Blueprints/Enums/E_AIMode Enum" :default "NewEnumerator0"))
  (returns (Success :type Boolean))
  (`self.SetCurrentMode` NewMode)
  (return true))

(fn `SetNewCustomPatrolPath`
  (params (PathPoints :type "Array of Vector Structure (by ref)"))
  (returns (Success :type Boolean))
  (`self.SetCustomPatrolPath` PathPoints)
  (return true))

(fn `SetStage`
  (params (Stage :type "/Game/LMiTW/Blueprints/Enums/E_AIStages Enum" :default "NewEnumerator0"))
  (returns (Success :type Boolean))
  (bind _success (message `/Game/LMiTW/Blueprints/Interface/BPI_AIController.SetAIStage` (`self.GetController`) Stage))
  (`self.UpdateMovement` (`BlueprintMapLibrary.Map_Find` (`.AIMovementForStages_16_F9D8130046A605957E9D899D85D7B7E1` (break `/Game/LMiTW/Blueprints/Structures/SAI_Preset` (`/Game/LMiTW/Data/AIPresets/BP_AIPresetBase.Preset` (`self.Preset`)))) Stage))
  (return _success))

(fn `UpdateMovement`
  (params (Preset :type "/Game/LMiTW/Blueprints/Structures/S_AIMovementPreset Structure (by ref)"))
  (set `self.CurrentMovementPreset` Preset)
  (`self.UpdateMovementSpeedByMode`))

(fn `UpdateMovementSpeedByMode`
  (bind (_patrolspeed _ispectspeed _combatspeed) (break `/Game/LMiTW/Blueprints/Structures/S_AIMovementPreset` (`self.CurrentMovementPreset`)))
  (set `CharacterMovementComponent.MaxWalkSpeed` (select `/Game/LMiTW/Blueprints/Enums/E_AIMode` (`self.CurrentAIMode`) :`NewEnumerator0` _patrolspeed :`NewEnumerator1` _patrolspeed :`NewEnumerator2` _combatspeed :`NewEnumerator3` _patrolspeed :`NewEnumerator5` _ispectspeed :`NewEnumerator6` _ispectspeed) (`self.CharacterMovement`)))

(fn `UserConstructionScript`
  (`parent.UserConstructionScript`))