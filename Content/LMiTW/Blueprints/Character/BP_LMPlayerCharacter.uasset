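; Player character for LMiTW with switchable first/third-person cameras, health with win and death end screens, notes, and carried two-handed items.
; Input flags feed a movement component; an interaction component handles object use.
; Door keypads take over the camera through timer-driven timeline easing, while notes lock movement and look.
; It also creates start-story and temporary graphics-option widgets, smooths the first-person camera, and stores PDA access level and welding tool.
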(event `Key|Q`
  (params (Key :type "Key Structure"))
  (bind _lastinteractobject (`self.LastInteractObject`))
  ;[1 0.1719 0.1719] Temporary
  (:`Pressed`
    (bind _asbp_door_control_panel (cast `/Game/LMiTW/Blueprints/GameplayActors/Switcher/BP_DoorControlPanel` _lastinteractobject :!label _label)
      (:`then`
        (`/Game/LMiTW/Blueprints/GameplayActors/Switcher/BP_DoorControlPanel.E_InteractExit` _asbp_door_control_panel (stale `Key|Escape` Key)))
      (:`CastFailed`
        (cast `/Game/LMiTW/Blueprints/GameplayActors/Pickup/BP_Note` _lastinteractobject)
        (`self.E_NoteClose`)))))

(event `self.ReceiveBeginPlay`
  ;[1 1 1] BeginPlay
  ;[1 1 1] SetDefaultCamera
  (`ActorComponent.SetActive` (`self.CameraFirstPerson`) true false)
  (`ActorComponent.SetActive` (`self.CameraThirdPerson`) false false)
  (`|ExecutionSequence`
    (:`then_0`
      (bind _asbp_lmplayer_controller_game (cast `/Game/LMiTW/Blueprints/Controller/BP_LMPlayerControllerGame` (`self.GetController`)))
      (`/Game/LMiTW/Blueprints/Controller/BP_LMPlayerControllerGame.SetPlayerInputMode` _asbp_lmplayer_controller_game "NewEnumerator1")
      ;[1 1 1] Widgets
      (`self.InitTemporaryOptionWidget`)
      (`self.InitStartStoryWidget`)
      (`GameplayStatics.SetGamePaused` true)
      ;[1 1 1] Note widget
      (bind _returnvalue (`|CreateWidget` "/Game/LMiTW/HUD/PDA/WBP_Note.WBP_Note_C"))
      (`WidgetComponent.SetWidget` (`self.TemporaryWidgetNote`) _returnvalue))
    (:`then_1`)))

(event `Key|Escape`
  (params (Key :type "Key Structure"))
  ;[1 0.1719 0.1719] Temporary
  (:`Pressed`
    (goto _label)))

(event `Key|V`
  (params (Key :type "Key Structure"))
  ;[0.5306 0.3012 1] Swtich view camera
  (:`Pressed`
    (`/Engine/EditorBlueprintResources/StandardMacros.FlipFlop`
      (:`A`
        (`ActorComponent.SetActive` (`self.CameraThirdPerson`) true false)
        (`ActorComponent.SetActive` (`self.CameraFirstPerson`) false false))
      (:`B`
        (`ActorComponent.SetActive` (`self.CameraFirstPerson`) true false)
        (`ActorComponent.SetActive` (`self.CameraThirdPerson`) false false)))))

(event `self.ReceiveTick`
  (params (DeltaSeconds :type "Float (single-precision)"))
  ;[1 1 1] Event Tick
  (`/Engine/EditorBlueprintResources/StandardMacros.IsValid` (`self.LastInteractObject`)
    (:`Is Not Valid`
      (`self.CameraTransformSmoothing`))))

(event `Key|F`
  (params (Key :type "Key Structure"))
  ;[0.6823 0.3646 1] Заглушки
  (:`Pressed`
    (`/Game/LMiTW/Blueprints/Components/BP_PlayerInteractionComponent.Interact` (`self.BP_PlayerInteractionComponent`) Key)))

(event `Key|One`
  (params (Key :type "Key Structure"))
  ;[1 1 1] Graphic Levels
  (:`Pressed`
    (`/Game/LMiTW/HUD/GameOverlay/WBP_TemporaryGraphicOption.E_SetNewGraphicsLevel` (`self.Temporary_WBP_Option`) 1)
    (`self.SetGraphicsLevel` 1)))

(event `Key|LeftMouseButton`
  (params (Key :type "Key Structure"))
  ;[0.6823 0.3646 1] Заглушки
  (:`Pressed`
    (`/Game/LMiTW/Blueprints/Components/BP_PlayerInteractionComponent.Interact` (`self.BP_PlayerInteractionComponent`) Key)
    (`WidgetInteractionComponent.PressPointerKey` (`self.WidgetInteraction`) "LeftMouseButton"))
  (:`Released`
    (`WidgetInteractionComponent.ReleasePointerKey` (`self.WidgetInteraction`) "LeftMouseButton")))

(event `Key|Two`
  (params (Key :type "Key Structure"))
  ;[1 1 1] Graphic Levels
  (:`Pressed`
    (`/Game/LMiTW/HUD/GameOverlay/WBP_TemporaryGraphicOption.E_SetNewGraphicsLevel` (`self.Temporary_WBP_Option`) 2)
    (`self.SetGraphicsLevel` 2)))

(event `Key|Three`
  (params (Key :type "Key Structure"))
  ;[1 1 1] Graphic Levels
  (:`Pressed`
    (`/Game/LMiTW/HUD/GameOverlay/WBP_TemporaryGraphicOption.E_SetNewGraphicsLevel` (`self.Temporary_WBP_Option`) 3)
    (`self.SetGraphicsLevel` 3)))

(event `Key|I`
  (params (Key :type "Key Structure"))
  ;[0.6823 0.3646 1] Заглушки
)

(event `InputAxis|Move Forward`
  (params (AxisValue :type "Float (single-precision)"))
  ;[1 1 1] Movement
  (message `/Game/LMiTW/Blueprints/Interface/BPI_Movement.PlayerInput` (`self.BP_PlayerControlMovementComponent`) AxisValue (stale `InputAxis|Move Right` AxisValue) (`self.PressKeyCrouch?`) (`self.PressKeyRun?`) (`self.PressKeyCrowl?`) (`self.PressKeyAntiGravityMode?`) (`self.HaveTwoHandedItem?`) (not (`self.CanMove`))))

(event `InputAxis|Move Right`
  (params (AxisValue :type "Float (single-precision)"))
  ;[1 1 1] Movement
)

(event `E_TrueGameEnd`
  ;[1 1 1] End game
  (`/Engine/EditorBlueprintResources/StandardMacros.DoOnce` false
    (:`Completed`
      (set `self.InteractObjectLockMovement?` true)
      (bind _asbp_lmplayer_controller_game (cast `/Game/LMiTW/Blueprints/Controller/BP_LMPlayerControllerGame` (`self.GetController`)))
      (`/Game/LMiTW/Blueprints/Controller/BP_LMPlayerControllerGame.SetPlayerInputMode` _asbp_lmplayer_controller_game "NewEnumerator1")
      (`KismetSystemLibrary.Delay` 3.0)
      (`Widget.RemoveFromParent` (`self.Temporary_WBP_Option`))
      (bind _returnvalue (`|CreateWidget` "/Game/LMiTW/HUD/GameOverlay/WBP_EndGameMain.WBP_EndGameMain_C"))
      (bind _output_get (set `self.WBP_EndGame` _returnvalue))
      (`WidgetSwitcher.SetActiveWidgetIndex` (`/Game/LMiTW/HUD/GameOverlay/WBP_EndGameMain.WidgetSwitcher_End` _output_get) 1)
      (`UserWidget.AddToViewport` _output_get 0))))

(event `InputAxis|Turn`
  (params (AxisValue :type "Float (single-precision)"))
  ;[1 1 1] Mouse
  (if (`self.mouseLock`)
    (`self.AddControllerYawInput` 0.0)
    (else
      (bind _output_get (set `self.YawDirection` AxisValue))
      (`self.AddControllerYawInput` _output_get))))

(event `E_SetNewCameraAndRedirectInput`
  (params (ActorWithCamera :type "Actor Object Reference") (CameraPlace :type "SceneComponent Object Reference"))
  (bind _timertocontrolpanel (`self.timerToControlPanel`))
  (bind _timertocharacter (`self.timerToCharacter`))
  ;[1 1 1] temporary functional for interaction with control panel by pin code
  (cast `/Game/LMiTW/Blueprints/GameplayActors/Switcher/BP_DoorControlPanel` ActorWithCamera)
  (`/Engine/EditorBlueprintResources/StandardMacros.FlipFlop`
    (:`A`
      (`SceneComponent.K2_SetRelativeTransform` (`self.ArrowReturnTransformForCamera`) (`KismetMathLibrary.MakeTransform` (`SceneComponent.RelativeLocation` (`self.CameraFirstPerson`)) (`SceneComponent.RelativeRotation` (`self.CameraFirstPerson`))) false false)
      (if (`KismetSystemLibrary.K2_IsValidTimerHandle` _timertocharacter)
        (`KismetSystemLibrary.K2_ClearAndInvalidateTimerHandle` _timertocharacter))
      ;;[1 1 1] UI input activate
      (bind _returnvalue (`KismetSystemLibrary.K2_SetTimerDelegate` (delegate `CustomEvent_0`) 0.001 true))
      (set `self.timerToControlPanel` _returnvalue)
      (set `CameraComponent.bUsePawnControlRotation` false (`self.CameraFirstPerson`))
      (`TimelineComponent.SetNewTime` (`self.TimelineSoftChangeCameraTransformOnPanel`) (`self.alpha`))
      (set `self.LastInteractObject` ActorWithCamera)
      (`TimelineComponent.Stop` (`self.TimelineSoftChangeCameraTransformOnCharacter`))
      (message `/Game/LMiTW/Blueprints/Interface/BPI_PlayerController.SetPlayerInputMode` (`self.GetController`) "NewEnumerator1")
      (set `self.mouseLock` true))
    (:`B`
      (if (`KismetSystemLibrary.K2_IsValidTimerHandle` _timertocontrolpanel)
        (`KismetSystemLibrary.K2_ClearAndInvalidateTimerHandle` _timertocontrolpanel))
      ;;[1 1 1] Enable Character Input
      (bind _returnvalue_2 (`KismetSystemLibrary.K2_SetTimerDelegate` (delegate `CustomEvent_1`) 0.001 true))
      (set `self.timerToCharacter` _returnvalue_2)
      (`TimelineComponent.SetNewTime` (`self.TimelineSoftChangeCameraTransformOnCharacter`) (- 1.0 (`self.alpha`)))
      (`TimelineComponent.Stop` (`self.TimelineSoftChangeCameraTransformOnPanel`)))))

(event `InputAxis|LookUp`
  (params (AxisValue :type "Float (single-precision)"))
  ;[1 1 1] Mouse
  (if (`self.mouseLock`)
    (`self.AddControllerPitchInput` 0.0)
    (else
      (bind _output_get (set `self.PitchDirection` AxisValue))
      (`self.AddControllerPitchInput` _output_get))))

(event `Key|LeftControl`
  (params (Key :type "Key Structure"))
  ;[1 1 1] crouch
  (:`Pressed`
    (set `self.PressKeyCrouch?` true :!label _label_2))
  (:`Released`
    (set `self.PressKeyCrouch?` false :!label _label_3)))

(event `Key|K`
  (params (Key :type "Key Structure"))
  ;[0.56 0.4432 1] antigravityMode
  (:`Released`
    (set `self.PressKeyAntiGravityMode?` false)))

(event `Key|C`
  (params (Key :type "Key Structure"))
  ;[1 1 1] crouch
  (:`Pressed`
    (goto _label_2))
  (:`Released`
    (goto _label_3)))

(event `self.ReceiveAnyDamage`
  (params (Damage :type "Float (single-precision)") (DamageType :type "DamageType Object Reference") (InstigatedBy :type "Controller Object Reference") (DamageCauser :type "Actor Object Reference"))
  (bind _returnvalue (- (`self.health`) Damage))
  ;[1 1 1] End game
  (set `self.health` _returnvalue)
  ;;[1 1 1] any damage
  (if (<= _returnvalue 0.0)
    (`/Engine/EditorBlueprintResources/StandardMacros.DoOnce` false
      (:`Completed`
        (set `self.InteractObjectLockMovement?` true)
        (bind _asbp_lmplayer_controller_game (cast `/Game/LMiTW/Blueprints/Controller/BP_LMPlayerControllerGame` (`self.GetController`)))
        (`/Game/LMiTW/Blueprints/Controller/BP_LMPlayerControllerGame.SetPlayerInputMode` _asbp_lmplayer_controller_game "NewEnumerator1")
        (`Widget.RemoveFromParent` (`self.Temporary_WBP_Option`))
        (bind _returnvalue_2 (`|CreateWidget` "/Game/LMiTW/HUD/GameOverlay/WBP_EndGameMain.WBP_EndGameMain_C"))
        (bind _output_get (set `self.WBP_EndGame` _returnvalue_2))
        (`WidgetSwitcher.SetActiveWidgetIndex` (`/Game/LMiTW/HUD/GameOverlay/WBP_EndGameMain.WidgetSwitcher_End` _output_get) 0)
        (`UserWidget.AddToViewport` _output_get 0)))
    (else
      (`GameplayStatics.PlaySound2D` "/Game/LMiTW/Assets/Audio/FootstepSound/Sounds/WaveFiles/Jump_Voice_Mono/Male/jump_voice_end_2.jump_voice_end_2" 1.0 1.0 0.0 null null))))

(event `Key|I`
  (params (Key :type "Key Structure"))
  ;[0.5262 0.4169 1] PDA
)

(event `CustomEvent_0`
  ;[1 1 1] temporary functional for interaction with control panel by pin code
  (bind (_direction _timeofcamerachange) (`Timeline|TimelineSoftChangeCameraTransformOnPanel`)
    (:`Update`
      (set `self.alpha` _timeofcamerachange)
      (`SceneComponent.K2_SetWorldTransform` (`self.CameraFirstPerson`) (`KismetMathLibrary.MakeTransform` (`|EaseFunction` "ExpoIn" _timeofcamerachange (`SceneComponent.K2_GetComponentLocation` (`self.CameraFirstPerson`)) (`SceneComponent.K2_GetComponentLocation` (stale `E_SetNewCameraAndRedirectInput` CameraPlace))) (`|EaseFunction` "ExpoIn" _timeofcamerachange (`SceneComponent.K2_GetComponentRotation` (`self.CameraFirstPerson`)) (`SceneComponent.K2_GetComponentRotation` (stale `E_SetNewCameraAndRedirectInput` CameraPlace)) false)) false false))
    (:`Finished`
      (`KismetSystemLibrary.K2_ClearAndInvalidateTimerHandle` (`self.timerToControlPanel`)))))

(event `Key|LeftShift`
  (params (Key :type "Key Structure"))
  ;[1 1 1] run
  (:`Pressed`
    (set `self.PressKeyRun?` true))
  (:`Released`
    (set `self.PressKeyRun?` false)))

(event `Key|G`
  (params (Key :type "Key Structure"))
  ;[1 1 1] Drop two handed item
  (:`Pressed`
    (`self.DropTwoHandedItem` true)))

(event `Key|Z`
  (params (Key :type "Key Structure"))
  ;[1 1 1] crowl
)

(event `CustomEvent_1`
  (bind _camerafirstperson (`self.CameraFirstPerson`))
  (bind _arrowreturntransformforcamera (`self.ArrowReturnTransformForCamera`))
  ;[1 1 1] temporary functional for interaction with control panel by pin code
  (bind (_direction _timeofcamerachange) (`Timeline|TimelineSoftChangeCameraTransformOnCharacter`)
    (:`Update`
      (set `self.alpha` (- 1.0 _timeofcamerachange))
      (`SceneComponent.K2_SetWorldTransform` (`self.CameraFirstPerson`) (`KismetMathLibrary.MakeTransform` (`|EaseFunction` "ExpoIn" _timeofcamerachange (`SceneComponent.K2_GetComponentLocation` _camerafirstperson) (`SceneComponent.K2_GetComponentLocation` _arrowreturntransformforcamera)) (`|EaseFunction` "ExpoIn" _timeofcamerachange (`SceneComponent.K2_GetComponentRotation` _camerafirstperson) (`SceneComponent.K2_GetComponentRotation` _arrowreturntransformforcamera) false)) false false))
    (:`Finished`
      (`KismetSystemLibrary.K2_ClearAndInvalidateTimerHandle` (`self.timerToCharacter`))
      (message `/Game/LMiTW/Blueprints/Interface/BPI_PlayerController.SetPlayerInputMode` (`self.GetController`) "NewEnumerator2")
      (set `self.LastInteractObject` null)
      (set `CameraComponent.bUsePawnControlRotation` true (`self.CameraFirstPerson`))
      (set `self.mouseLock` false))))

(event `E_NoteClose`
  ;[1 1 1] E_NoteClose
  (set `self.LastInteractObject` null)
  (`SceneComponent.SetVisibility` (`self.TemporaryWidgetNote`) false false)
  (`self.SetInteractObjectLockMovement` false)
  (set `self.mouseLock` false)
  (`/Game/LMiTW/Blueprints/Components/BP_PlayerInteractionComponent.StartTracing` (`self.BP_PlayerInteractionComponent`))
  (bind _gameoverlaywidget (message `/Game/LMiTW/Blueprints/Interface/BPI_PlayerController.GetGameOverlay` (`self.GetController`)))
  (`/Game/LMiTW/HUD/GameOverlay/WBP_GameOverlay.ShowCursor` _gameoverlaywidget))

(event `E_NoteOpen`
  (params (NoteData :type "/Game/LMiTW/Blueprints/Structures/S_NoteData Structure") (Note :type "Actor Object Reference"))
  ;[1 1 1] E_NoteOpen
  (set `self.LastInteractObject` Note)
  (`SceneComponent.SetVisibility` (`self.TemporaryWidgetNote`) true false)
  (bind _aswbp_note (cast `/Game/LMiTW/HUD/PDA/WBP_Note` (`WidgetComponent.GetWidget` (`self.TemporaryWidgetNote`))))
  (`/Game/LMiTW/HUD/PDA/WBP_Note.SetNoteDataAndUpdateUI` _aswbp_note NoteData)
  (`self.SetInteractObjectLockMovement` true)
  (set `self.mouseLock` true)
  (`/Game/LMiTW/Blueprints/Components/BP_PlayerInteractionComponent.StopTracing` (`self.BP_PlayerInteractionComponent`))
  (bind _gameoverlaywidget (message `/Game/LMiTW/Blueprints/Interface/BPI_PlayerController.GetGameOverlay` (`self.GetController`)))
  (`/Game/LMiTW/HUD/GameOverlay/WBP_GameOverlay.HideCursor` _gameoverlaywidget))

(event `Key|One`
  (params (Key :type "Key Structure")))

(event `Key|Two`
  (params (Key :type "Key Structure")))

(event `Key|Three`
  (params (Key :type "Key Structure")))

(event `Key|Four`
  (params (Key :type "Key Structure")))

(fn `AddTwoHandedItem`
  (params (`BP TwoHandedItem` :type "/Game/LMiTW/Blueprints/GameplayActors/Pickup/BP_TwoHandedItem Object Reference") (SocketNameToAttach :type Name))
  (returns (`Success?` :type Boolean))
  (bind _pickupmesh (`/Game/LMiTW/Blueprints/GameplayActors/Pickup/BP_MasterPickup.PickupMesh` `BP TwoHandedItem`))
  (if (`self.HaveTwoHandedItem?`)
    (return false)
    (else
      (set `self.HaveTwoHandedItem?` true)
      (set `self.TwoHanedItem` `BP TwoHandedItem`)
      (`PrimitiveComponent.SetSimulatePhysics` _pickupmesh false)
      (`SceneComponent.K2_AttachToComponent` _pickupmesh (`Actor.RootComponent` `BP TwoHandedItem`) "None" "SnapToTarget" "SnapToTarget" "KeepWorld" true)
      (`self.K2_AttachToComponent` `BP TwoHandedItem` (`self.Mesh`) "twoHandedItemSocket" "SnapToTarget" "KeepRelative" "KeepWorld" true)
      (`self.K2_AddActorLocalOffset` `BP TwoHandedItem` (0.0 -10.0 10.0) false false)
      (return true))))

(fn `CameraTransformSmoothing`
  (bind _returnvalue (`SceneComponent.K2_GetComponentLocation` (`self.CameraFirstPerson`)))
  (bind _returnvalue_2 (`SceneComponent.K2_GetComponentLocation` (`self.ArrowCameraSmooth`)))
  (`SceneComponent.K2_SetWorldLocation` (`self.CameraFirstPerson`) (`KismetMathLibrary.VInterpTo` _returnvalue _returnvalue_2 (`GameplayStatics.GetWorldDeltaSeconds`) (`KismetMathLibrary.MapRangeClamped` (`KismetMathLibrary.Vector_Distance` _returnvalue _returnvalue_2) 10.0 18.0 5.0 150.0)) false false))

(fn `CanMove`
  (returns (Result :type Boolean))
  (return (and (not (`self.InteractObjectLockMovement?`)) true)))

(fn `DropTwoHandedItem`
  (params (`SimulatePhysics?` :type Boolean))
  (bind _twohaneditem (`self.TwoHanedItem`))
  (`/Engine/EditorBlueprintResources/StandardMacros.IsValid` _twohaneditem
    (:`Is Valid`
      (set `self.HaveTwoHandedItem?` false)
      (`self.K2_DetachFromActor` _twohaneditem "KeepWorld" "KeepRelative" "KeepWorld")
      (`/Game/LMiTW/Blueprints/GameplayActors/Pickup/BP_TwoHandedItem.E_DropTwoHandedItem` _twohaneditem `SimulatePhysics?`)
      (set `self.TwoHanedItem` null))))

(fn `GetAccessLevel`
  (returns (`Access level` :type "/Game/LMiTW/Blueprints/Enums/E_AcessLevels Enum"))
  (return (`self.GetPdaAccessLevel`)))

(fn `GetInteractObjectLockMovement`
  (returns (`LockMovement?` :type Boolean))
  (return (`self.InteractObjectLockMovement?`)))

(fn `GetPdaAccessLevel`
  (returns (AccessLevel :type "/Game/LMiTW/Blueprints/Enums/E_AcessLevels Enum"))
  (return (`self.PDA AccessLevel`)))

(fn `GetSoundStepInfo`
  (returns (Success :type Boolean) (FootStepsAudioComponent :type "AudioComponent Object Reference") (`FootStepsPlay?` :type Boolean) (`EquipmentPlay?` :type Boolean) (FootStepsVolume :type "Float (double-precision)") (EquipmentVolume :type "Float (double-precision)") (`IsMale?` :type Boolean))
  (return true (`self.FootSteps`) true true 1.0 1.0 true))

(fn `GetTwoHandedItem`
  (returns (`HaveItem?` :type Boolean) (ItemInfo :type "/Game/LMiTW/Blueprints/Structures/S_ItemInfo Structure") (Actor :type "/Game/LMiTW/Blueprints/GameplayActors/Pickup/BP_TwoHandedItem Object Reference"))
  (bind _twohaneditem (`self.TwoHanedItem`))
  (if (`self.HaveTwoHandedItem?`)
    (bind _iteminfo (`/Game/LMiTW/Blueprints/GameplayActors/Pickup/BP_TwoHandedItem.GetItemInfo` _twohaneditem))
    (return true _iteminfo _twohaneditem)
    (else
      (return false (struct) null))))

(fn `GetWelding`
  (returns (`HaveWelding?` :type Boolean) (WeldingActor :type "Actor Object Reference"))
  (return (`self.HaveWelding?`) (`self.Welding`)))

(fn `InitializeAnimationParametrs`
  (returns (LMBase_Chracter :type "LMBaseCharacter Object Reference") (BP_ControlMovementComponent :type "/Game/LMiTW/Blueprints/Components/BP_PlayerControlMovementComponent Object Reference"))
  (return self (`self.BP_PlayerControlMovementComponent`)))

(fn `InitializeMovementParametrs`
  (returns (InitParametrs :type "/Game/LMiTW/Blueprints/Structures/S_MovementInitInfo Structure"))
  (return (`self.sMovementAndStamina`)))

(fn `InitStartStoryWidget`
  (bind _returnvalue (`|CreateWidget` "/Game/LMiTW/HUD/GameOverlay/WBP_StartStoryGame.WBP_StartStoryGame_C"))
  (bind _output_get (set `self.WBP_StartStory` _returnvalue))
  (`UserWidget.AddToViewport` _output_get 1))

(fn `InitTemporaryOptionWidget`
  (bind _returnvalue (`|CreateWidget` "/Game/LMiTW/HUD/GameOverlay/WBP_TemporaryGraphicOption.WBP_TemporaryGraphicOption_C"))
  (bind _output_get (set `self.Temporary_WBP_Option` _returnvalue))
  (`UserWidget.AddToViewport` _output_get 0))

(fn `SetGraphicsLevel`
  (params (GraphicsLevel :type Integer))
  (locals (Optimization :type "/Game/LMiTW/Blueprints/Optimization/BP_Optimization Object Reference"))
  (bind _returnvalue (`GameplayStatics.GetActorOfClass` "/Game/LMiTW/Blueprints/Optimization/BP_Optimization.BP_Optimization_C"))
  (set `local.Optimization` _returnvalue)
  (switch `int` GraphicsLevel
    (:`1`
      (`/Game/LMiTW/Blueprints/Optimization/BP_Optimization.Set New Graphics Option Parametrs` (`local.Optimization`) (make `/Game/LMiTW/Blueprints/Structures/S_GraphicsLevel` 100)))
    (:`2`
      (`/Game/LMiTW/Blueprints/Optimization/BP_Optimization.Set New Graphics Option Parametrs` (`local.Optimization`) (make `/Game/LMiTW/Blueprints/Structures/S_GraphicsLevel` 75 0 0.0 2 250 0 1 0 0 0)))
    (:`3`
      (`/Game/LMiTW/Blueprints/Optimization/BP_Optimization.Set New Graphics Option Parametrs` (`local.Optimization`) (make `/Game/LMiTW/Blueprints/Structures/S_GraphicsLevel` 50 0 0.0 0 250 0 0 0 0 0)))))

(fn `SetInteractObjectLockMovement`
  (params (`LockMovement?` :type Boolean))
  (set `self.InteractObjectLockMovement?` `LockMovement?`))

(fn `SetPdaAccessLevel`
  (params (NewLevel :type "/Game/LMiTW/Blueprints/Enums/E_AcessLevels Enum" :default "NewEnumerator0"))
  (set `self.PDA AccessLevel` NewLevel))

(fn `SetWelding`
  (params (WeldingActor :type "Actor Object Reference"))
  (bind _output_get (set `self.Welding` WeldingActor))
  (`/Engine/EditorBlueprintResources/StandardMacros.IsValid` _output_get
    (:`Is Valid`
      (set `self.HaveWelding?` true))
    (:`Is Not Valid`
      (set `self.HaveWelding?` false))))

(fn `TransformTextOfNote`
  (params (MainText :type String))
  (returns (finishedText :type String) (OutCodes :type "Array of Text"))
  (locals (startIndex :type Integer) (localString :type String) (findedIndex :type Integer) (localCodes :type "Array of Text") (numberString :type String))
  (bind _returnvalue (`KismetStringLibrary.FindSubstring` (`local.localString`) "<pincode>" false false (`local.startIndex`)))
  (set `local.startIndex` 0)
  (set `local.localString` MainText)
  (for _ (range 21)
    ;[1 1 1] if don`t find string "<pincode>"
    (if (== _returnvalue -1)
      (return (`local.localString`) (`local.localCodes`))
      (else
        (set `local.findedIndex` _returnvalue)
        (set `local.numberString` (`KismetStringLibrary.Concat_StrStr` (`KismetStringLibrary.Conv_IntToString` (`KismetMathLibrary.RandomIntegerInRange` 0 9)) (`KismetStringLibrary.Conv_IntToString` (`KismetMathLibrary.RandomIntegerInRange` 0 9)) (`KismetStringLibrary.Conv_IntToString` (`KismetMathLibrary.RandomIntegerInRange` 0 9)) (`KismetStringLibrary.Conv_IntToString` (`KismetMathLibrary.RandomIntegerInRange` 0 9))))
        (set `local.localString` (`KismetStringLibrary.Concat_StrStr` (`KismetStringLibrary.GetSubstring` (`local.localString`) 0 (`local.findedIndex`)) (`local.numberString`) (`KismetStringLibrary.GetSubstring` (`local.localString`) (+ (`local.findedIndex`) 9) (`KismetStringLibrary.Len` (`local.localString`)))))
        (`KismetArrayLibrary.Array_Add` (`local.localCodes`) (`KismetTextLibrary.Conv_StringToText` (`local.numberString`)))
        (set `local.startIndex` (+ (`local.findedIndex`) 4))))))

(fn `UserConstructionScript`)