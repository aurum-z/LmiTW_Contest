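; Ability logic Blueprint for a single-target spherecast attack that damages one actor in front of the attacker.
; StartAbility sets a one-shot timer from the attack info's start delay, which then runs the spherecast.
; The attacker's SphereTraceForTarget sweeps along its forward vector using the configured distance and radius, ignoring itself.
; A blocking hit applies damage and ends the ability; a miss does neither.
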(event `self.StartAbility`
  (`KismetSystemLibrary.K2_SetTimerDelegate` (delegate `ProcessSpherecast`) (`.StartDelay_3_534C48C24C4D882392C702A5FD9C604F` (break `/Game/LMiTW/Blueprints/Structures/S_AbilityAttackParams` (`/Game/LMiTW/Data/Abilities/Base/BP_Ability.GetAttackInfo` (`self.Ability`))))))

(event `ProcessSpherecast`
  (bind _attacker (`self.Attacker`))
  (bind _attacker_2 (`self.Attacker`)
    (:`then`
      (bind _outhit (`LMBaseCharacter.SphereTraceForTarget` _attacker_2 (`Actor.K2_GetActorLocation` _attacker_2) (+ (`Actor.K2_GetActorLocation` _attacker_2) (* (`Actor.GetActorForwardVector` _attacker_2) (`.SpherecastDistance_9_03401D3644990DBE445D30B1B25A46D2` (break `/Game/LMiTW/Blueprints/Structures/S_AbilityAttackParams` (`/Game/LMiTW/Data/Abilities/Base/BP_Ability.GetAttackInfo` (`self.Ability`)))))) (`.SpherecastRadius_8_D3B064EE44D5E86EAEA1EC90D6B37913` (break `/Game/LMiTW/Blueprints/Structures/S_AbilityAttackParams` (`/Game/LMiTW/Data/Abilities/Base/BP_Ability.GetAttackInfo` (`self.Ability`)))) (`|MakeArray` _attacker_2 :!type "Actor Object Reference")))
      (bind (_bblockinghit _binitialoverlap _time _distance _location _impactpoint _normal _impactnormal _physmat _hitactor) (`GameplayStatics.BreakHitResult` _outhit))
      (if _bblockinghit
        (`GameplayStatics.ApplyDamage` _hitactor 0.0 (`Pawn.GetController` _attacker) _attacker)
        (`self.EndAbility`)))
    (:`else`)))