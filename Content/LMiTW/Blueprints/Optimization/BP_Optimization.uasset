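; BP_Optimization applies a set of graphics and performance options on BeginPlay and during construction.
; SetNewGraphicsOptionParametrs turns a graphics-level struct into console commands for resolution, quality and frame cap, plus a GameUserSettings view-distance call and optional unlit mode.
; Both callers supply only default values, and command names are appended to values without a separating space.
; An older variable-driven copy in the EventGraph never runs.
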(event `self.ReceiveBeginPlay`
  (`self.Set New Graphics Option Parametrs` (make `/Game/LMiTW/Blueprints/Structures/S_GraphicsLevel` 100)))

(fn `Set New Graphics Option Parametrs`
  (params (GraphicLevel :type "/Game/LMiTW/Blueprints/Structures/S_GraphicsLevel Structure"))
  (bind (_screenpercentage _viewdistancequality _viewdistancescale _postprocessanti_aliasing _maxfps _motionblurquality _shadowquality _texturequality _effectsquality _detailquality) (break `/Game/LMiTW/Blueprints/Structures/S_GraphicsLevel` GraphicLevel))
  (`|ExecutionSequence`
    (:`then_0`
      (if (`self.UnlitMode?`)
        (`KismetSystemLibrary.ExecuteConsoleCommand` "viewmode unlit" null)))
    (:`then_1`
      ;[1 1 1] 0 to 100
      (`KismetSystemLibrary.ExecuteConsoleCommand` (`KismetStringLibrary.Concat_StrStr` "r.ScreenPercentage " (`KismetStringLibrary.Conv_IntToString` _screenpercentage)) null))
    (:`then_2`
      ;[1 1 1] View distance scale: 0 to 1
      (bind _returnvalue (`GameUserSettings.GetGameUserSettings`))
      (`GameUserSettings.SetViewDistanceQuality` _returnvalue _viewdistancequality))
    (:`then_3`
      (`|ExecutionSequence`
        (:`then_0`
          ;[1 1 1] 0 to 1
          (`KismetSystemLibrary.ExecuteConsoleCommand` (`KismetStringLibrary.Concat_StrStr` "r.ViewDistanceScale " (`KismetStringLibrary.Conv_DoubleToString` _viewdistancescale)) null))
        (:`then_1`
          ;[1 1 1] PostProcess Anti-aliasing: 0 to 1
          (`KismetSystemLibrary.ExecuteConsoleCommand` (`KismetStringLibrary.Concat_StrStr` "r.PostProcessAAQuality " (`KismetStringLibrary.Conv_IntToString` _postprocessanti_aliasing)) null))
        (:`then_2`
          ;[1 1 1] Max fps
          (`KismetSystemLibrary.ExecuteConsoleCommand` (`KismetStringLibrary.Concat_StrStr` "t.MaxFPS " (`KismetStringLibrary.Conv_IntToString` _maxfps)) null))
        (:`then_3`
          (`|ExecutionSequence`
            (:`then_0`
              ;[1 1 1] Motion blur quality 0 3
              (`KismetSystemLibrary.ExecuteConsoleCommand` (`KismetStringLibrary.Concat_StrStr` "sg.PostProcessQuality " (`KismetStringLibrary.Conv_IntToString` _motionblurquality)) null))
            (:`then_1`
              ;[1 1 1] Shadow quality 0 3
              (`KismetSystemLibrary.ExecuteConsoleCommand` (`KismetStringLibrary.Concat_StrStr` "sg.ShadowQuality " (`KismetStringLibrary.Conv_IntToString` _shadowquality)) null))
            (:`then_2`
              ;[1 1 1] Texture quality 0 3
              (`KismetSystemLibrary.ExecuteConsoleCommand` (`KismetStringLibrary.Concat_StrStr` "sg.TextureQuality " (`KismetStringLibrary.Conv_IntToString` _texturequality)) null))
            (:`then_3`
              (`|ExecutionSequence`
                (:`then_0`
                  ;[1 1 1] EffectsQuality 0 3
                  (`KismetSystemLibrary.ExecuteConsoleCommand` (`KismetStringLibrary.Concat_StrStr` "sg.EffectsQuality " (`KismetStringLibrary.Conv_IntToString` _effectsquality)) null))
                (:`then_1`
                  ;[1 1 1] DetailQuality 0 2
                  (`KismetSystemLibrary.ExecuteConsoleCommand` (`KismetStringLibrary.Concat_StrStr` "r.DetailMode " (`KismetStringLibrary.Conv_IntToString` _detailquality)) null))))))))))

(fn `UserConstructionScript`
  (`self.Set New Graphics Option Parametrs` (struct)))