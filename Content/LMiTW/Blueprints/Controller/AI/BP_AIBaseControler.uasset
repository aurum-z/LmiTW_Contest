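; Base AI controller that drives an enemy's staged behavior, patrolling, player detection and attacks.
; The pawn supplies the starting stage and mode; stages start the behavior tree or enable custom patrol, while modes sync to Blackboard and pawn.
; Perceiving the player raises a timer-driven alertness bar; losing them sets an inspect location and decays it.
; Patrol points are random reachable spots around the player or follow a ping-pong custom path.
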(event `self.ReceiveBeginPlay`
  ;[1 1 1] Begin play
  (`self.Init`))

(event `self.Perception.OnTargetPerceptionInfoUpdated`
  (params (UpdateInfo :type "ActorPerceptionUpdateInfo Structure (by ref)"))
  ;[1 1 1] Perception update
  (`self.UpdatePerception` UpdateInfo))

(event `InspectingEnded`
  ;[1 1 1] Inspecting end
  (`self.SetMode` "NewEnumerator1"))

(event `/Game/LMiTW/Blueprints/Interface/BPI_AIController.IncrementInspectingIteration`
  ;[1 1 1] Inspect iterations
  (`self.IncrementInspectingIterations`))

(event `SuspectingBarFull`
  ;[1 1 1] Suspecting bar full
  (`self.SetMode` "NewEnumerator2"))

(fn `Attack`
  (returns (Success :type Boolean))
  (set `self.IsAttacking` true)
  (bind _success (message `/Game/LMiTW/Blueprints/Interface/BPI_AICharacter.ProcessAttack` (`self.K2_GetPawn`)))
  (return _success))

(fn `GetAcceptablePatrolPoint`
  (returns (Success :type Boolean) (Point :type "Vector Structure"))
  (bind _distance (message `/Game/LMiTW/Blueprints/Interface/BPI_AICharacter.GetAcceptableDistance` (`self.K2_GetPawn`)))
  (bind (_randomlocation _returnvalue) (`NavigationSystemV1.K2_GetRandomReachablePointInRadius` (`self.K2_GetActorLocation` (`GameplayStatics.GetPlayerCharacter` 0)) _distance null null))
  (return _returnvalue _randomlocation))

(fn `GetAIMode`
  (returns (Mode :type "/Game/LMiTW/Blueprints/Enums/E_AIMode Enum"))
  (return (`self.GetMode`)))

(fn `GetMode`
  (returns (Mode :type "/Game/LMiTW/Blueprints/Enums/E_AIMode Enum"))
  (return (`self.CurrentMode`)))

(fn `GetNewPatrolPoint`
  (returns (Point :type "Vector Structure"))
  (return (`self.GetNextPatrolPoint`)))

(fn `GetNextCustomPatrolPoint`
  (returns (Point :type "Vector Structure"))
  (if (`self.IsReversePatrolPath`)
    (bind _result (`/Engine/EditorBlueprintResources/StandardMacros.DecrementInt` (`self.CurrentPatrolPoint`))
      (:`  `
        (if (>= _result 0)
          (return (`|GetArrayItem` (`self.CustomPathPoints`) (`self.CurrentPatrolPoint`)))
          (else
            (set `self.IsReversePatrolPath` false)
            (return (`self.GetNextCustomPatrolPoint`))))))
    (else
      (bind _result_2 (`/Engine/EditorBlueprintResources/StandardMacros.IncrementInt` (`self.CurrentPatrolPoint`))
        (:`  `
          (if (== _result_2 (`KismetArrayLibrary.Array_Length` (`self.CustomPathPoints`)))
            (set `self.IsReversePatrolPath` true)
            (return (`self.GetNextCustomPatrolPoint`))
            (else
              (return (`|GetArrayItem` (`self.CustomPathPoints`) (`self.CurrentPatrolPoint`))))))))))

(fn `GetNextPatrolPoint`
  (returns (Point :type "Vector Structure"))
  (locals (Local_SearchFails :type Integer) (Local_MaxSearchFails :type Integer :default 100))
  (bind (_success _point) (`self.GetAcceptablePatrolPoint`))
  (if (not (`self.InCustomPatrolMode`))
    (if (< (`local.Local_SearchFails`) (`local.Local_MaxSearchFails`)) :!label _label
      (if _success
        (return _point)
        (else
          (`/Engine/EditorBlueprintResources/StandardMacros.IncrementInt` (`local.Local_SearchFails`) ; Infinity loop protecting
            (:`  `
              (goto _label)))))
      (else
        (return (0.0 0.0 0.0)) ; Fail - returns zero location. TODO Add fail handling
      ))
    (else
      (return (`self.GetNextCustomPatrolPoint`)))))

(fn `GetStartMode`
  (returns (Mode :type "/Game/LMiTW/Blueprints/Enums/E_AIMode Enum"))
  (`/Engine/EditorBlueprintResources/StandardMacros.IsValid` (`self.K2_GetPawn`)
    (:`Is Valid`
      (bind _mode (message `/Game/LMiTW/Blueprints/Interface/BPI_AICharacter.GetStartMode` (`self.K2_GetPawn`)))
      (return _mode))
    (:`Is Not Valid`
      (return "NewEnumerator0"))))

(fn `GetStartStage`
  (returns (Stage :type "/Game/LMiTW/Blueprints/Enums/E_AIStages Enum"))
  (bind _returnvalue (`self.K2_GetPawn`))
  (`/Engine/EditorBlueprintResources/StandardMacros.IsValid` _returnvalue
    (:`Is Valid`
      (bind _stage (message `/Game/LMiTW/Blueprints/Interface/BPI_AICharacter.GetStartStage` _returnvalue))
      (return _stage))
    (:`Is Not Valid`
      (return "NewEnumerator0"))))

(fn `IncrementInspectingIterations`
  (if (< (`self.CurrentInspectingIterations`) (`self.MaxInspectingIterations`))
    (`/Engine/EditorBlueprintResources/StandardMacros.IncrementInt` (`self.CurrentInspectingIterations`))
    (else
      (set `self.CurrentInspectingIterations` 0)
      (`self.InspectingEnded`))))

(fn `InCustomPatrolMode`
  (returns (Result :type Boolean))
  (return (`self.IsCustomPatrolMode`)))

(fn `Init`
  (`self.SetStage` (`self.GetStartStage`))
  (`self.SetMode` (`self.GetStartMode`))
  (`self.UseBlackboard` (`self.DefaultBlackboard`))
  (`BlackboardComponent.SetValueAsObject` (`self.Blackboard`) "Controller" self))

(fn `NewCustomPatrolPath`
  (params (PathPoints :type "Array of Vector Structure (by ref)"))
  (returns (Success :type Boolean))
  (`self.SetCustomPatrolPath` PathPoints)
  (return true))

(fn `ProcessSences`
  (params (Targets :type "Array of Actor Object Reference"))
  (for _array_element Targets
    (if (`self.ActorHasTag` _array_element "Player")
      (`self.SetTargetPlayer` _array_element)
      (`self.SetMode` "NewEnumerator5"))))

(fn `ProgressSuspecting`
  (`/Engine/EditorBlueprintResources/StandardMacros.IncrementInt` (`self.AlertnessCurrent`)
    (:`  `
      (if (not (< (`self.AlertnessCurrent`) (`self.AlertnessMax`)))
        (`self.SuspectingBarFull`)
        (`KismetSystemLibrary.K2_ClearAndInvalidateTimerHandle` (`self.SuspectingProgressTimer`))))))

(fn `RegressSuspecting`
  (bind _result (`/Engine/EditorBlueprintResources/StandardMacros.DecrementInt` (`self.AlertnessCurrent`))
    (:`  `
      (if (== _result 0)
        (`KismetSystemLibrary.K2_ClearAndInvalidateTimerHandle` (`self.SuspectingRegressTimer`))))))

(fn `SetAIStage`
  (params (Stage :type "/Game/LMiTW/Blueprints/Enums/E_AIStages Enum" :default "NewEnumerator0"))
  (returns (Success :type Boolean))
  (bind _success (`self.SetStage` Stage))
  (return _success))

(fn `SetCustomPatrolPath`
  (params (CustomPathPoints :type "Array of Vector Structure"))
  (set `self.CustomPathPoints` CustomPathPoints))

(fn `SetInspectingLocation`
  (params (Location :type "Vector Structure"))
  (bind _output_get (set `self.InspectLocation` Location))
  (`BlackboardComponent.SetValueAsVector` (`self.Blackboard`) "InspectingLocation" _output_get))

(fn `SetMode`
  (params (Mode :type "/Game/LMiTW/Blueprints/Enums/E_AIMode Enum" :default "NewEnumerator0"))
  (bind _output_get (set `self.CurrentMode` Mode))
  (`BlackboardComponent.SetValueAsEnum` (`self.Blackboard`) "CurrentMode" _output_get)
  (message `/Game/LMiTW/Blueprints/Interface/BPI_AICharacter.SetMode` (`self.K2_GetPawn`) (`self.GetMode`)))

(fn `SetSensesSetup`
  (params (NewSetup :type "/Game/LMiTW/Blueprints/Structures/S_AISensesSetup Structure")))

(fn `SetStage`
  (params (Stage :type "/Game/LMiTW/Blueprints/Enums/E_AIStages Enum" :default "NewEnumerator0"))
  (returns (Success :type Boolean))
  (bind _output_get (set `self.CurrentStage` Stage))
  (switch `/Game/LMiTW/Blueprints/Enums/E_AIStages` _output_get
    (:`NewEnumerator0`
      (`KismetSystemLibrary.PrintString` "AI - Setted a not valid stage!" true true (struct :`R` 1.0 :`B` 0.008603 :`A` 1.0) 5.0)
      (`self.RunBehaviorTree` null)
      (return false))
    (:`NewEnumerator1`
      (bind _returnvalue (`self.RunBehaviorTree` (`self.BehaviorTreeStageFirst`)))
      (return _returnvalue))
    (:`NewEnumerator2`
      (return true))
    (:`NewEnumerator3`
      (set `self.IsCustomPatrolMode` true)
      (return true))))

(fn `SetTargetPlayer`
  (params (Target :type "Actor Object Reference"))
  (bind _output_get (set `self.TargetPlayer` Target))
  (`BlackboardComponent.SetValueAsObject` (`self.Blackboard`) "TargetPlayer" _output_get))

(fn `StartPatrol`
  (`self.SetMode` "NewEnumerator1"))

(fn `StartRegressSuspecting`
  (`KismetSystemLibrary.K2_ClearAndInvalidateTimerHandle` (`self.SuspectingProgressTimer`))
  (bind _returnvalue (`KismetSystemLibrary.K2_SetTimer` null "RegressSuspecting" (`self.SuspectingTickInterval`) true))
  (set `self.SuspectingRegressTimer` _returnvalue))

(fn `StartSuspecting`
  (`KismetSystemLibrary.K2_ClearAndInvalidateTimerHandle` (`self.SuspectingRegressTimer`))
  (bind _returnvalue (`KismetSystemLibrary.K2_SetTimer` null "ProgressSuspecting" (`self.SuspectingTickInterval`) true))
  (set `self.SuspectingProgressTimer` _returnvalue)
  (`self.SetMode` "NewEnumerator5"))

(fn `UpdatePerception`
  (params (ActorPerceptionUpdateInfo :type "ActorPerceptionUpdateInfo Structure (by ref)"))
  (locals (Local_Target :type "Actor Object Reference"))
  (bind (_targetid _target _stimulus) (break `ActorPerceptionUpdateInfo` ActorPerceptionUpdateInfo))
  (bind ((`StimulusLocation` _stimuluslocation) (`bSuccessfullySensed` _bsuccessfullysensed)) (break `AIStimulus` _stimulus))
  (bind _output_get (set `local.Local_Target` _target))
  (`/Engine/EditorBlueprintResources/StandardMacros.IsValid` _output_get
    (:`Is Valid`
      (if (`self.ActorHasTag` _output_get "Player")
        (if _bsuccessfullysensed
          (`self.SetTargetPlayer` (`local.Local_Target`))
          (if (== (`self.AlertnessCurrent`) (`self.AlertnessMax`))
            (`self.SuspectingBarFull`)
            (else
              (`self.StartSuspecting`)))
          (else
            (`self.SetInspectingLocation` _stimuluslocation)
            (`self.SetMode` "NewEnumerator6")
            (`self.SetTargetPlayer` null)
            (if (not (== (`self.AlertnessCurrent`) (`self.AlertnessMax`)))
              (`self.StartRegressSuspecting`))))))))

(fn `UserConstructionScript`)