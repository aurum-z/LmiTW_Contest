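; In-game player controller that creates the game overlay widget and saves the default camera angle limits on BeginPlay.
; Switches between Free Move and PDA input modes, toggling the cursor and the pawn's interaction tracing.
; RedirectInput moves input between actors, for cases like welding that need the mouse.
; Camera yaw and pitch limits can be overridden or restored to defaults, though comments flag this path as broken and slated for removal.
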(event `self.ReceiveBeginPlay`
  (`self.GameOverlayInit`)
  (`self.CameraManagerInit`))

(event `/Game/LMiTW/Blueprints/Interface/BPI_PlayerController.SetPlayerInputMode`
  (params (NewMode :type "/Game/LMiTW/Blueprints/Enums/E_InputMode Enum" :default "NewEnumerator0"))
  (`self.SetPlayerInputOnInputMode` NewMode))

(event `/Game/LMiTW/Blueprints/Interface/BPI_PlayerController.RedirectInput`
  (params (actorWhatInputDisable :type "Actor Object Reference") (actorWhatInputEnable :type "Actor Object Reference"))
  ;[1 1 1] Work for welt, when we need use mouse, and not keyboard
  (`self.FRedirectInput` actorWhatInputDisable actorWhatInputEnable))

(event `/Game/LMiTW/Blueprints/Interface/BPI_PlayerController.SetCameraViewAmglesConstraints`
  (params (NewYawMin :type "Float (single-precision)") (NewYawMax :type "Float (single-precision)") (`SetNewYaw?` :type Boolean) (NewPitchMin :type "Float (single-precision)") (NewPitchMax :type "Float (single-precision)") (`SetNewPitch?` :type Boolean))
  ;[1 1 1] Delete this function in future. This function dont work
  (`self.FSetCameraViewAgnlesConstraint` (`self.PlayerCameraManager`) NewYawMin NewYawMax `SetNewYaw?` NewPitchMin NewPitchMax `SetNewPitch?`))

(event `NewCamera`
  (params (ActorWithCamera :type "Actor Object Reference")))

(fn `CameraManagerInit`
  (bind _playercameramanager (`self.PlayerCameraManager`))
  (bind _playercameramanager_2 (`self.PlayerCameraManager`))
  ;[1 1 1] Delete this in future
  (`|ExecutionSequence`
    (:`then_0`
      ;;[1 1 1] Save camera default rotation constraints
      (set `self.viewYawMinDefault` (`PlayerCameraManager.ViewYawMin` _playercameramanager_2))
      (set `self.viewYawMaxDefault` (`PlayerCameraManager.ViewYawMax` _playercameramanager_2))
      (set `self.viewPitchMinDefault` (`PlayerCameraManager.ViewPitchMin` _playercameramanager))
      (set `self.viewPitchMaxDefault` (`PlayerCameraManager.ViewPitchMax` _playercameramanager)))))

(fn `DisableCharacterInteraction`
  (`/Game/LMiTW/Blueprints/Components/BP_PlayerInteractionComponent.StopTracing` (`self.GetComponentByClass` (`GameplayStatics.GetPlayerPawn` 0) "/Game/LMiTW/Blueprints/Components/BP_PlayerInteractionComponent.BP_PlayerInteractionComponent_C")))

(fn `EnableCharacterInteraction`
  (`/Game/LMiTW/Blueprints/Components/BP_PlayerInteractionComponent.StartTracing` (`self.GetComponentByClass` (`GameplayStatics.GetPlayerPawn` 0) "/Game/LMiTW/Blueprints/Components/BP_PlayerInteractionComponent.BP_PlayerInteractionComponent_C")))

(fn `FRedirectInput`
  (params (ActorWhatInputDisabled :type "Actor Object Reference") (ActorWhatInputEnabled :type "Actor Object Reference"))
  (`|ExecutionSequence`
    (:`then_0`
      (`/Engine/EditorBlueprintResources/StandardMacros.IsValid` ActorWhatInputDisabled
        (:`Is Valid`
          (`self.DisableInput` ActorWhatInputDisabled self))))
    (:`then_1`
      (`/Engine/EditorBlueprintResources/StandardMacros.IsValid` ActorWhatInputEnabled
        (:`Is Valid`
          (`self.EnableInput` ActorWhatInputEnabled self))))))

(fn `FSetCameraViewAgnlesConstraint`
  (params (CameraManager :type "PlayerCameraManager Object Reference") (NewYawMin :type "Float (double-precision)") (NewYawMax :type "Float (double-precision)") (`SetNewYaw?` :type Boolean) (NewPitchMin :type "Float (double-precision)") (NewPitchMax :type "Float (double-precision)") (`SetNewPitch?` :type Boolean))
  (`|ExecutionSequence`
    (:`then_0`
      (if `SetNewYaw?`
        (set `PlayerCameraManager.ViewYawMin` NewYawMin CameraManager)
        (set `PlayerCameraManager.ViewYawMax` NewYawMax CameraManager)
        (else
          ;[1 1 1] Set default Yaw
          (set `PlayerCameraManager.ViewYawMin` (`self.viewYawMinDefault`) CameraManager)
          (set `PlayerCameraManager.ViewYawMax` (`self.viewYawMaxDefault`) CameraManager))))
    (:`then_1`
      (if `SetNewPitch?`
        (set `PlayerCameraManager.ViewPitchMin` NewPitchMin CameraManager)
        (set `PlayerCameraManager.ViewPitchMax` NewPitchMax CameraManager)
        (else
          ;[1 1 1] Set default Pitch
          (set `PlayerCameraManager.ViewPitchMin` (`self.viewPitchMinDefault`) CameraManager)
          (set `PlayerCameraManager.ViewPitchMax` (`self.viewPitchMaxDefault`) CameraManager))))))

(fn `GameOverlayInit`
  (bind _returnvalue (`|CreateWidget` "/Game/LMiTW/HUD/GameOverlay/WBP_GameOverlay.WBP_GameOverlay_C" self))
  (bind _output_get (set `self.GameOverlayWidget` _returnvalue))
  (`UserWidget.AddToViewport` _output_get 0))

(fn `GetGameOverlay`
  (returns (GameOverlayWidget :type "/Game/LMiTW/HUD/GameOverlay/WBP_GameOverlay Object Reference"))
  (bind _gameoverlaywidget (`self.GameOverlayWidget`)
    (:`then`
      (return _gameoverlaywidget))
    (:`else`)))

(fn `SetPlayerInputOnInputMode`
  (params (Mode :type "/Game/LMiTW/Blueprints/Enums/E_InputMode Enum" :default "NewEnumerator0"))
  (set `self.PlayerInputMode` Mode)
  (switch `/Game/LMiTW/Blueprints/Enums/E_InputMode` (`self.PlayerInputMode`)
    (:`NewEnumerator2`
      (`WidgetBlueprintLibrary.SetInputMode_GameOnly` self)
      (set `self.bShowMouseCursor` false)
      (`self.EnableCharacterInteraction`))
    (:`NewEnumerator1`
      (cast `/Game/LMiTW/Blueprints/Character/BP_LMPlayerCharacter` (`GameplayStatics.GetPlayerCharacter` 0))
      ;[1 1 1] PDA
      (`WidgetBlueprintLibrary.SetInputMode_GameAndUIEx` self null)
      (set `self.bShowMouseCursor` true)
      (`self.DisableCharacterInteraction`))))

(fn `UserConstructionScript`)