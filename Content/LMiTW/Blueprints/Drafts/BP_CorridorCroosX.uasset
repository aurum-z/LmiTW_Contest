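; BP_CorridorCroosX is a draft corridor actor, apparently a cross-junction piece, assembled from static mesh components such as floor panels and ceilings.
; Its construction script enlarges the bounds scale of two groups of those meshes, one by a larger factor than the other.
; Some meshes appear in both groups, so the second, smaller value overrides the first for them.
; The event graph holds only disabled placeholder events, so it has no runtime logic.
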(fn `UserConstructionScript`
  (`PrimitiveComponent.SetBoundsScale` (`self.StaticMesh6`) 7.0)
  (`PrimitiveComponent.SetBoundsScale` (`self.StaticMesh7`) 7.0)
  (`PrimitiveComponent.SetBoundsScale` (`self.StaticMesh5`) 7.0)
  (`PrimitiveComponent.SetBoundsScale` (`self.StaticMesh6`) 7.0)
  (`PrimitiveComponent.SetBoundsScale` (`self.SM_FloorPanel_D`) 2.5)
  (`PrimitiveComponent.SetBoundsScale` (`self.SM_Ceiling_Main_B1`) 2.5)
  (`PrimitiveComponent.SetBoundsScale` (`self.SM_Ceiling_Main_B`) 2.5)
  (`PrimitiveComponent.SetBoundsScale` (`self.StaticMesh7`) 2.5)
  (`PrimitiveComponent.SetBoundsScale` (`self.StaticMesh4`) 2.5)
  (`PrimitiveComponent.SetBoundsScale` (`self.StaticMesh5`) 2.5))