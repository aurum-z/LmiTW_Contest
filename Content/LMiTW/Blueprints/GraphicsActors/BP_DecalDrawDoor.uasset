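; A placeable decal actor that can ride on a sliding door or its frame.
; The construction script applies the assigned decal material, or falls back to a default material instance when none is set.
; On BeginPlay, if a door slider is referenced, it attaches to that actor's Door or DoorFrame component according to the AttachTo choice, keeping its world transform.
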(event `self.ReceiveBeginPlay`
  (`/Engine/EditorBlueprintResources/StandardMacros.IsValid` (`self.AttachToDoorSlider`)
    (:`Is Valid`
      (switch `/Game/LMiTW/Blueprints/Enums/E_DecalAttachDoor` (`self.AttachTo`)
        (:`NewEnumerator0`
          (`self.K2_AttachToComponent` (`/Game/LMiTW/Blueprints/GameplayActors/Door/BP_MasterDoor.Door` (`self.AttachToDoorSlider`)) "None" "KeepWorld" "KeepWorld" "KeepWorld"))
        (:`NewEnumerator1`
          (`self.K2_AttachToComponent` (`/Game/LMiTW/Blueprints/GameplayActors/Door/BP_MasterDoor.DoorFrame` (`self.AttachToDoorSlider`)) "None" "KeepWorld" "KeepWorld" "KeepWorld"))))))

(fn `UserConstructionScript`
  (bind _decalmaterial (`self.DecalMaterial`))
  (`/Engine/EditorBlueprintResources/StandardMacros.IsValid` _decalmaterial
    (:`Is Valid`
      (`DecalComponent.SetDecalMaterial` (`self.Decal`) _decalmaterial))
    (:`Is Not Valid`
      (`DecalComponent.SetDecalMaterial` (`self.Decal`) (`self.DecalMI`)))))